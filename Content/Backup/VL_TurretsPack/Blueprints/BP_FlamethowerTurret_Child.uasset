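; Flamethrower turret child Blueprint that shows power and attack effects and burns enemies in front of its muzzle.
; Tick uses paired DoOnce gates to update lights and materials on power changes, and flame particles and looping sound on attack changes.
; While attacking, it sphere-traces forward every frame and applies radial damage at hits on EnemyList classes, unscaled by delta time.
; SkinFunction applies normal or damaged material sets, and E_SkinSelector cycles skins.
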(event Custom|E_SkinSelector
  (if (select (Variables|Default|GetIsDamage) (< (Variables|Default|GetSkinType) (Utilities|Array|LastIndex (Variables|Default|GetSkinArray2))) (< (Variables|Default|GetSkinType) (Utilities|Array|LastIndex (Variables|Default|GetSkinArray1))))
    (Math|Integer|IncrementInt (Variables|Default|GetSkinType)
      (:%20%20
        _))
    (else
      (Variables|Default|SetSkinType 0)))
  (CallFunction|SkinFunction))

(event EventBeginPlay
  (|CallParentFunction)
  (CallFunction|SkinFunction))

(event EventTick
  (params (DeltaSeconds :type Float%20%28single-precision%29))
  (bind _turret_flamethower_loop (Variables|Default|GetTurret_Flamethower_Loop))
  (bind _p_muzle01 (Variables|Default|GetP_Muzle01))
  (bind _returnvalue (Transformation|GetWorldLocation _p_muzle01))
  (|CallParentFunction DeltaSeconds)
  (Utilities|FlowControl|Sequence
    (:then_0
      (if (Variables|Default|GetIsPower)
        (Utilities|FlowControl|Sequence
          (:then_0
            (Utilities|FlowControl|DoOnce true :!label _label
              (:Completed
                _)))
          (:then_1
            (goto _label_2 Reset)))
        (else
          (Utilities|FlowControl|Sequence
            (:then_0
              (Utilities|FlowControl|DoOnce false :!label _label_2
                (:Completed
                  _)))
            (:then_1
              (goto _label Reset)))))
      (Rendering|Material|SetMaterial (Variables|Default|GetStaticMesh2) 5 (select (Variables|Default|GetIsPower) "/Game/Backup/VL_TurretsPack/Materials/MI_LightMain.MI_LightMain" "/Game/Backup/VL_TurretsPack/Materials/MI_Glass.MI_Glass"))
      (Rendering|Material|SetMaterial (Variables|Default|GetStaticMesh2) 4 (select (Variables|Default|GetIsPower) "/Game/Backup/VL_TurretsPack/Materials/MI_Fire.MI_Fire" "/Game/Backup/VL_TurretsPack/EpicContent/Materials/M_Burst.M_Burst"))
      (Rendering|SetVisibility (Variables|Default|GetSpotLight) (Variables|Default|GetIsPower) false))
    (:then_1
      (if (Variables|Default|GetIsAttack)
        (Utilities|FlowControl|Sequence
          (:then_0
            (Utilities|FlowControl|DoOnce true :!label _label_3
              (:Completed
                _)))
          (:then_1
            (goto _label_4 Reset)))
        (else
          (Utilities|FlowControl|Sequence
            (:then_0
              (Utilities|FlowControl|DoOnce false :!label _label_4
                (:Completed
                  _)))
            (:then_1
              (goto _label_3 Reset)))))
      (Components|Activation|SetActive (Variables|Default|GetP_Muzle01) (Variables|Default|GetIsAttack) false)
      (if (Variables|Default|GetIsAttack) ; SOUND LOOP
        (Audio|Components|Audio|Play _turret_flamethower_loop 0.0)
        (else
          (Audio|Components|Audio|Stop _turret_flamethower_loop))))
    (:then_2
      (if (Variables|Default|GetIsAttack) ; DAMAGE
        (bind _outhit (Collision|SphereTraceForObjects _returnvalue (+ _returnvalue (* (Math|Vector|GetForwardVector (Transformation|GetWorldRotation _p_muzle01)) (Variables|Default|GetScanRadius))) 2e+01 (Variables|Default|GetTraceType) false 0 "None"))
        (if (!= (Utilities|Array|FindItem (Variables|Default|GetEnemyList) (Utilities|GetClass (.hitactor _outhit))) -1)
          (Game|Damage|ApplyRadialDamage (Variables|Default|GetDamage) (.location _outhit) (Variables|Default|GetDamageRadius) 0 0 0 0 false "ECC_Visibility"))))))

(fn ConstructionScript
  (|CallParentFunction)
  (Rendering|Material|SetMaterial (Variables|Default|GetStaticMesh2) 5 (select (Variables|Default|GetIsPower) "/Game/Backup/VL_TurretsPack/Materials/MI_LightMain.MI_LightMain" "/Game/Backup/VL_TurretsPack/Materials/MI_Glass.MI_Glass"))
  (Rendering|Material|SetMaterial (Variables|Default|GetStaticMesh2) 4 (select (Variables|Default|GetIsPower) "/Game/Backup/VL_TurretsPack/Materials/MI_Fire.MI_Fire" "/Game/Backup/VL_TurretsPack/EpicContent/Materials/M_Burst.M_Burst"))
  (CallFunction|SkinFunction))

(fn SkinFunction
  (bind _skintype (Variables|Default|GetSkinType))
  (bind _skinarray1 (Variables|Default|GetSkinArray1))
  (bind _materialsmain (Variables|Default|GetMaterialsMain))
  (bind _materialsdamage (Variables|Default|GetMaterialsDamage))
  (bind _skintype_2 (Variables|Default|GetSkinType))
  (bind _skinarray2 (Variables|Default|GetSkinArray2))
  (bind _output (Utilities|Array|Get(acopy) _skinarray2 _skintype_2))
  (bind _output_2 (Utilities|Array|Get(acopy) _materialsdamage 4))
  (bind _output_3 (Utilities|Array|Get(acopy) _skinarray1 _skintype))
  (bind _output_4 (Utilities|Array|Get(acopy) _materialsmain 4))
  (bind _output_5 (Utilities|Array|Get(acopy) _materialsmain 3))
  (bind _output_6 (Utilities|Array|Get(acopy) _materialsmain 1))
  (bind _output_7 (Utilities|Array|Get(acopy) _materialsdamage 3))
  (bind _output_8 (Utilities|Array|Get(acopy) _materialsdamage 1))
  (if (Variables|Default|GetIsDamage)
    (Rendering|Material|SetMaterial (Variables|Default|GetStaticMesh) 0 _output)
    (Rendering|Material|SetMaterial (Variables|Default|GetStaticMesh1) 1 _output)
    (Rendering|Material|SetMaterial (Variables|Default|GetStaticMesh2) 0 _output)
    (Rendering|Material|SetMaterial (Variables|Default|GetStaticMesh) 1 _output_7) ; Chrome
    (Rendering|Material|SetMaterial (Variables|Default|GetStaticMesh1) 0 _output_7)
    (Rendering|Material|SetMaterial (Variables|Default|GetStaticMesh2) 3 _output_7)
    (Rendering|Material|SetMaterial (Variables|Default|GetStaticMesh) 2 _output_8) ; Plastic
    (Rendering|Material|SetMaterial (Variables|Default|GetStaticMesh1) 2 _output_8)
    (Rendering|Material|SetMaterial (Variables|Default|GetStaticMesh2) 1 _output_8)
    (Rendering|Material|SetMaterial (Variables|Default|GetStaticMesh) 4 _output_2) ; Decal
    (Rendering|Material|SetMaterial (Variables|Default|GetStaticMesh1) 5 _output_2)
    (Rendering|Material|SetMaterial (Variables|Default|GetStaticMesh2) 6 _output_2)
    (else
      (Rendering|Material|SetMaterial (Variables|Default|GetStaticMesh) 0 _output_3)
      (Rendering|Material|SetMaterial (Variables|Default|GetStaticMesh1) 1 _output_3)
      (Rendering|Material|SetMaterial (Variables|Default|GetStaticMesh2) 0 _output_3)
      (Rendering|Material|SetMaterial (Variables|Default|GetStaticMesh) 1 _output_5) ; Chrome
      (Rendering|Material|SetMaterial (Variables|Default|GetStaticMesh1) 0 _output_5)
      (Rendering|Material|SetMaterial (Variables|Default|GetStaticMesh2) 3 _output_5)
      (Rendering|Material|SetMaterial (Variables|Default|GetStaticMesh) 2 _output_6) ; Plastic
      (Rendering|Material|SetMaterial (Variables|Default|GetStaticMesh1) 2 _output_6)
      (Rendering|Material|SetMaterial (Variables|Default|GetStaticMesh2) 1 _output_6)
      (Rendering|Material|SetMaterial (Variables|Default|GetStaticMesh) 4 _output_4) ; Decal
      (Rendering|Material|SetMaterial (Variables|Default|GetStaticMesh1) 5 _output_4)
      (Rendering|Material|SetMaterial (Variables|Default|GetStaticMesh2) 6 _output_4))))