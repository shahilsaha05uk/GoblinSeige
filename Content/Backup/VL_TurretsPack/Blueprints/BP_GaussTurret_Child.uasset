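; Gauss turret child Blueprint that fires gauss bullets while attacking, adding laser sight, rail-heat and lamp effects to its parent turret.
; Each Tick pulses IsFire from a sine of game time scaled by ReloadTime, with a DoOnce spawning one bullet, sound and muzzle effect per pulse.
; While powered, a line trace drives the laser beam, and rail glow interpolates toward hot during firing.
; SkinFunction applies normal or damaged material sets, and E_SkinSelector cycles skins.
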(event Custom|E_SkinSelector
  (if (select (Variables|Default|GetIsDamage) (< (Variables|Default|GetSkinType) (Utilities|Array|LastIndex (Variables|Default|GetSkinArray2))) (< (Variables|Default|GetSkinType) (Utilities|Array|LastIndex (Variables|Default|GetSkinArray1))))
    (Math|Integer|IncrementInt (Variables|Default|GetSkinType)
      (:%20%20
        _))
    (else
      (Variables|Default|SetSkinType 0)))
  (CallFunction|SkinFunction))

(event EventBeginPlay
  (|CallParentFunction))

(event EventTick
  (params (DeltaSeconds :type Float%20%28single-precision%29))
  (bind _spawnarrow (Variables|Default|GetSpawnArrow))
  (bind _returnvalue (Transformation|GetWorldTransform _spawnarrow))
  (|CallParentFunction DeltaSeconds)
  (CallFunction|LaserFunction)
  (CallFunction|HotMetal)
  (Utilities|FlowControl|Sequence
    (:then_0
      (if (Variables|Default|GetIsAttack)
        (Variables|Default|SetIsFire (<= (Math|Float|Absolute(Float) (Math|Trig|Sin(Radians) (* (Utilities|Time|GetGameTimeinSeconds) (Variables|Default|GetReloadTime)))) 0.1))
        (else
          (Variables|Default|SetIsFire false))))
    (:then_1
      (if (Variables|Default|GetIsFire)
        (Utilities|FlowControl|DoOnce false :!label _label
          (:Completed
            (Components|Activation|SetActive (Variables|Default|GetFireParticleSystem) true false)
            (Game|SpawnActorfromClass "/Game/Backup/VL_TurretsPack/Blueprints/BP_Gauss_Bullet.BP_Gauss_Bullet_C" (Math|Transform|MakeTransform (.location _returnvalue) (.rotation _returnvalue) "1.000000,1.000000,1.000000") "AlwaysSpawn" "OverrideRootScale" 0 0)
            (Audio|PlaySoundatLocation "/Game/Backup/VL_TurretsPack/Sounds/Turret_Gauss_Fire_Cue.Turret_Gauss_Fire_Cue" (Transformation|GetActorLocation) "0, 0, 0" 1.0 1.0 0.0 0 0 0 0)
            (Utilities|FlowControl|Delay 0.4)
            (Components|Activation|SetActive (Variables|Default|GetFireParticleSystem) false false)))
        (else
          (goto _label Reset))))
    (:then_2
      (if (Variables|Default|GetIsPower)
        (Utilities|FlowControl|Sequence
          (:then_0
            (Utilities|FlowControl|DoOnce true :!label _label_2
              (:Completed
                _)))
          (:then_1
            (goto _label_3 Reset)))
        (else
          (Utilities|FlowControl|Sequence
            (:then_0
              (Utilities|FlowControl|DoOnce false :!label _label_3
                (:Completed
                  _)))
            (:then_1
              (goto _label_2 Reset)))))
      (Rendering|Material|SetMaterial (Variables|Default|GetStaticMesh2) 4 (select (Variables|Default|GetIsPower) "/Game/Backup/VL_TurretsPack/Materials/MI_LightMain.MI_LightMain" "/Game/Backup/VL_TurretsPack/Materials/MI_Glass.MI_Glass")) ; Lamp Set State
      (Rendering|SetVisibility (Variables|Default|GetSpotLight1) (Variables|Default|GetIsPower) false))))

(fn ConstructionScript
  (|CallParentFunction)
  (Rendering|Material|SetScalarParameterValueonMaterials (Variables|Default|GetHotRail) "Intensity" 0.0)
  (CallFunction|SkinFunction))

(fn LaserFunction
  (bind _trace (Variables|Default|GetTrace))
  (bind _laser_particlesystem (Variables|Default|GetLaser_ParticleSystem))
  (bind _laser_particlesystem_2 (Variables|Default|GetLaser_ParticleSystem))
  (bind _returnvalue (Transformation|GetWorldLocation _trace))
  (if (Variables|Default|GetIsPower)
    (bind (_outhit _returnvalue_2) (Collision|LineTraceForObjects _returnvalue (+ _returnvalue (* (Math|Vector|GetForwardVector (Transformation|GetWorldRotation _trace)) (* (Variables|Default|GetScanRadius) 2.0))) (Variables|Default|GetTraceType) false 0 "None"))
    (Rendering|SetVisibility _laser_particlesystem true false)
    (Class|ParticleSystemComponent|SetBeamSourcePoint _laser_particlesystem_2 0 (.TraceStart (Collision|BreakHitResult _outhit)))
    (Class|ParticleSystemComponent|SetBeamTargetPoint _laser_particlesystem_2 0 (Math|Vector|SelectVector (.Location (Collision|BreakHitResult _outhit)) (.TraceEnd (Collision|BreakHitResult _outhit)) _returnvalue_2))
    (Transformation|SetWorldLocation (Variables|Default|GetLaserEndSphere) (- (Math|Vector|SelectVector (.Location (Collision|BreakHitResult _outhit)) (.TraceEnd (Collision|BreakHitResult _outhit)) _returnvalue_2) (Math|Vector|GetForwardVector _trace)) false false)
    (else
      (Rendering|SetVisibility _laser_particlesystem false false))))

(fn HotMetal
  (bind _hotrail (Variables|Default|GetHotRail))
  (if (Variables|Default|GetIsPower)
    (bind _output_get (Variables|Default|SetHotMetal_Inter (Math|Interpolation|FInterpTo (Variables|Default|GetHotMetal_Inter) (Math|Float|SelectFloat 6.0 0.0 (Variables|Default|GetIsFire)) (Utilities|Time|GetWorldDeltaSeconds) 2.0)))
    (Rendering|Material|SetScalarParameterValueonMaterials _hotrail "Intensity" _output_get)
    (else
      (Rendering|Material|SetScalarParameterValueonMaterials _hotrail "Intensity" 0.0)
      (Variables|Default|SetHotMetal_Inter 0.0))))

(fn SkinFunction
  (bind _skintype (Variables|Default|GetSkinType))
  (bind _skinarray1 (Variables|Default|GetSkinArray1))
  (bind _materialsmain (Variables|Default|GetMaterialsMain))
  (bind _materialsdamage (Variables|Default|GetMaterialsDamage))
  (bind _skintype_2 (Variables|Default|GetSkinType))
  (bind _skinarray2 (Variables|Default|GetSkinArray2))
  (bind _output (Utilities|Array|Get(acopy) _skinarray2 _skintype_2))
  (bind _output_2 (Utilities|Array|Get(acopy) _materialsdamage 4))
  (bind _output_3 (Utilities|Array|Get(acopy) _skinarray1 _skintype))
  (bind _output_4 (Utilities|Array|Get(acopy) _materialsmain 4))
  (bind _output_5 (Utilities|Array|Get(acopy) _materialsmain 3))
  (bind _output_6 (Utilities|Array|Get(acopy) _materialsmain 1))
  (bind _output_7 (Utilities|Array|Get(acopy) _materialsdamage 3))
  (bind _output_8 (Utilities|Array|Get(acopy) _materialsdamage 1))
  (if (Variables|Default|GetIsDamage)
    (Rendering|Material|SetMaterial (Variables|Default|GetStaticMesh) 0 _output)
    (Rendering|Material|SetMaterial (Variables|Default|GetStaticMesh1) 1 _output)
    (Rendering|Material|SetMaterial (Variables|Default|GetStaticMesh2) 0 _output)
    (Rendering|Material|SetMaterial (Variables|Default|GetStaticMesh) 1 _output_7) ; Chrome
    (Rendering|Material|SetMaterial (Variables|Default|GetStaticMesh1) 0 _output_7)
    (Rendering|Material|SetMaterial (Variables|Default|GetStaticMesh2) 3 _output_7)
    (Rendering|Material|SetMaterial (Variables|Default|GetStaticMesh) 2 _output_8) ; Plastic
    (Rendering|Material|SetMaterial (Variables|Default|GetStaticMesh1) 2 _output_8)
    (Rendering|Material|SetMaterial (Variables|Default|GetStaticMesh2) 1 _output_8)
    (Rendering|Material|SetMaterial (Variables|Default|GetStaticMesh) 4 _output_2) ; Decal
    (Rendering|Material|SetMaterial (Variables|Default|GetStaticMesh1) 5 _output_2)
    (Rendering|Material|SetMaterial (Variables|Default|GetStaticMesh2) 6 _output_2)
    (else
      (Rendering|Material|SetMaterial (Variables|Default|GetStaticMesh) 0 _output_3)
      (Rendering|Material|SetMaterial (Variables|Default|GetStaticMesh1) 1 _output_3)
      (Rendering|Material|SetMaterial (Variables|Default|GetStaticMesh2) 0 _output_3)
      (Rendering|Material|SetMaterial (Variables|Default|GetStaticMesh) 1 _output_5) ; Chrome
      (Rendering|Material|SetMaterial (Variables|Default|GetStaticMesh1) 0 _output_5)
      (Rendering|Material|SetMaterial (Variables|Default|GetStaticMesh2) 3 _output_5)
      (Rendering|Material|SetMaterial (Variables|Default|GetStaticMesh) 2 _output_6) ; Plastic
      (Rendering|Material|SetMaterial (Variables|Default|GetStaticMesh1) 2 _output_6)
      (Rendering|Material|SetMaterial (Variables|Default|GetStaticMesh2) 1 _output_6)
      (Rendering|Material|SetMaterial (Variables|Default|GetStaticMesh) 4 _output_4) ; Decal
      (Rendering|Material|SetMaterial (Variables|Default|GetStaticMesh1) 5 _output_4)
      (Rendering|Material|SetMaterial (Variables|Default|GetStaticMesh2) 6 _output_4))))