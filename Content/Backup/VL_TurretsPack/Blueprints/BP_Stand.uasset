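; BP_Stand is a stand actor from the turrets pack with a text label and configurable lighting, apparently for display.
; Its construction script sets the label and applies shared intensity, color, shadow, radius and cone settings to four spotlights, with inner cone at half the outer.
; It also spawns a configurable number of point lights, spaced by yaw in a ring around the Center component.
; BeginPlay and Tick are empty.
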(event EventBeginPlay)

(event EventTick
  (params (DeltaSeconds :type Float%20%28single-precision%29)))

(fn ConstructionScript
  (bind _center (Variables|Default|GetCenter))
  (bind _pointlight_number (Variables|PointLight|GetPointLight_Number))
  (bind _spotlight1 (Variables|Default|GetSpotLight1))
  (bind _spotlight_outercone (Variables|SpotLight|GetSpotLight_OuterCone))
  (bind _relativelocation (Variables|/Script/Engine.SceneComponent|GetRelativeLocation _center))
  (bind (_x _y _z) (Math|Vector|BreakVector _relativelocation))
  (Rendering|Components|TextRender|SetText (Variables|Default|GetTextRender) (Variables|Default|GetText))
  (Rendering|Components|Light|SetIntensity _spotlight1 (Variables|SpotLight|GetSpotLight_Intensity))
  (Rendering|Components|Light|SetLightColor _spotlight1 (Variables|SpotLight|GetSpotLight_Color) true)
  (Rendering|Components|Light|SetCastShadows _spotlight1 (Variables|SpotLight|GetSpotLight_Shadow))
  (Rendering|Lighting|SetAttenuationRadius _spotlight1 (Variables|SpotLight|GetSpotLight_Radius))
  (Rendering|Lighting|SetInnerConeAngle _spotlight1 (/ _spotlight_outercone 2.0))
  (Rendering|Lighting|SetOuterConeAngle _spotlight1 _spotlight_outercone)
  (for _index (range 1 _pointlight_number)
    (bind _returnvalue (AddComponent|AddPointLightComponent false (Math|Transform|MakeTransform (- _relativelocation (* (Math|Vector|GetForwardVector (Math|Rotator|MakeRotator _x _y (+ _z (* _index (Math|Conversions|ToFloat(Integer) (/ 360 _pointlight_number)))))) (Variables|PointLight|GetPointLight_Distance))) (Variables|/Script/Engine.SceneComponent|GetRelativeRotation (Variables|Default|GetCenter)))))
    (Transformation|AttachComponentToComponent _returnvalue (Variables|Default|GetCenter) "None" "KeepWorld" "KeepWorld" "KeepWorld" true)
    (Rendering|Components|Light|SetIntensity _returnvalue (Variables|PointLight|GetPointLight_Intensity))
    (Rendering|Components|Light|SetLightColor _returnvalue (Variables|PointLight|GetPointLight_Color) true)
    (Rendering|Components|Light|SetCastShadows _returnvalue (Variables|PointLight|GetPointLight_Shadow))
    (Rendering|Lighting|SetAttenuationRadius _returnvalue (Variables|PointLight|GetPointLight_Radius))))