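; Drying rack prop with fifteen hanging fish and ham mesh components, randomized for visual variety.
; The construction script runs fifteen passes, each setting a randomly picked component to a random mesh from the HangingSM array, using the RandomHangingMeat stream.
; Picks can repeat, so some components keep their default mesh.
; The event graph holds no active logic.
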(event EventBeginPlay)

(event Collision|EventActorBeginOverlap
  (params (OtherActor :type Actor%20Object%20Reference)))

(event EventTick
  (params (DeltaSeconds :type Float%20%28single-precision%29)))

(fn ConstructionScript
  (for _index (range 0 14)
    (Components|StaticMesh|SetStaticMesh (Utilities|Array|Get(acopy) (Utilities|Array|MakeArray (Variables|Default|GetCAMP_fish_hanging_C_SM3) (Variables|Default|GetCAMP_fish_hanging_A_SM3) (Variables|Default|GetCAMP_fish_hanging_B_SM3) (Variables|Default|GetCAMP_fish_hanging_C_SM2) (Variables|Default|GetCAMP_fish_hanging_B_SM2) (Variables|Default|GetCAMP_fish_hanging_A_SM2) (Variables|Default|GetCAMP_fish_hanging_A_SM) (Variables|Default|GetCAMP_fish_hanging_C_SM1) (Variables|Default|GetCAMP_fish_hanging_B_SM1) (Variables|Default|GetCAMP_ham_hanging_SM2) (Variables|Default|GetCAMP_ham_hanging_SM1) (Variables|Default|GetCAMP_ham_hanging_SM) (Variables|Default|GetCAMP_fish_hanging_C_SM) (Variables|Default|GetCAMP_fish_hanging_B_SM) (Variables|Default|GetCAMP_fish_hanging_A_SM1)) (Class|KismetMathLibrary|RandomIntegerfromStream (Variables|RandomHangingMeat|GetRandom%20Hanging%20Meat) 14)) (Utilities|Array|Get(acopy) (Variables|Default|GetHanging%20SM) (Class|KismetMathLibrary|RandomIntegerfromStream (Variables|RandomHangingMeat|GetRandom%20Hanging%20Meat) 4)))))