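; A camp hand cart prop Blueprint with a configurable broken state and surface look, both set in the construction script.
; When Broken is set, it clears the wheels mesh, swaps the cart body to the broken mesh and resets that body's relative location.
; CleanMossMud indexes MaterialArray to pick one material for both body and wheels.
; The event graph has no active logic.
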(event EventBeginPlay)

(event Collision|EventActorBeginOverlap
  (params (OtherActor :type Actor%20Object%20Reference)))

(event EventTick
  (params (DeltaSeconds :type Float%20%28single-precision%29)))

(fn ConstructionScript
  (if (Variables|MeshVariation|GetBroken)
    (Components|StaticMesh|SetStaticMesh (Variables|Default|GetCAMP_handCart_wheels_SM) 0)
    (Components|StaticMesh|SetStaticMesh (Variables|Default|GetCAMP_handCart_SM) "/Game/Assets/CAMP_GameProps/Meshes/CAMP_handCart_broken_SM.CAMP_handCart_broken_SM")
    (Transformation|SetRelativeLocation (Variables|Default|GetCAMP_handCart_SM) "0, 0, 0" false false))
  (Rendering|Material|SetMaterial (Variables|Default|GetCAMP_handCart_SM) 0 (Utilities|Array|Get(acopy) (Variables|MeshVariation|GetMaterial%20-%20Array) (Variables|MeshVariation|GetClean/Moss/Mud))))