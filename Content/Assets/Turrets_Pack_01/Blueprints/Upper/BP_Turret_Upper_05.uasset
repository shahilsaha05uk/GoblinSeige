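; BP_Turret_Upper_05 is an upper turret Blueprint with left and right fire point groups that it alternates between on each shot.
; Fire flips the active side, picks that side's shoot montage and fires its points on a timer with the main projectile class.
; Reload chooses a side-matched montage when partial reload is allowed, then defers to the parent.
; Each projectile also spawns a pooled back-blast effect behind its fire point.
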(event EventReload
  (if (and (Variables|Default|GetAllowPartialReload) (not (Variables|Default|GetReloading)))
    (if (== (Variables|Default|GetActiveFirePointTag) "FirePointR")
      (Variables|Default|SetReloadMontage "/Game/Turrets_Pack_01/Animations/Upper/Upper_05/AM_Turret_Upper_05_Reload_R.AM_Turret_Upper_05_Reload_R")
      (else
        (Variables|Default|SetReloadMontage "/Game/Turrets_Pack_01/Animations/Upper/Upper_05/AM_Turret_Upper_05_Reload_L.AM_Turret_Upper_05_Reload_L")))
    (|CallParentFunction)
    (else
      (|CallParentFunction))))

(event EventOnSingleProjectileFired
  (params (FirePoint :type Scene%20Component%20Object%20Reference))
  (bind _returnvalue (Transformation|GetWorldRotation FirePoint))
  (|CallParentFunction FirePoint)
  (Niagara|SpawnSystematLocation (Variables|Turret|RocketLauncher|GetBackFireFX) (+ (Transformation|GetWorldLocation FirePoint) (* (Math|Vector|GetForwardVector _returnvalue) -2.5e+02)) _returnvalue "1.000000,1.000000,1.000000" true true "AutoRelease"))

(event EventFire
  (if (and (not (CallFunction|IsFiring)) (or (not (Variables|Default|GetReloading)) (Variables|Default|GetAllowPartialReload)))
    (if (== (Variables|Default|GetActiveFirePointTag) "FirePointR")
      (Variables|Default|SetActiveFirePointTag "FirePointL")
      (Variables|Default|SetPostFireMontage "/Game/Turrets_Pack_01/Animations/Upper/Upper_05/AM_Turret_Upper_05_Shoot_L.AM_Turret_Upper_05_Shoot_L")
      (else
        (Variables|Default|SetActiveFirePointTag "FirePointR")
        (Variables|Default|SetPostFireMontage "/Game/Turrets_Pack_01/Animations/Upper/Upper_05/AM_Turret_Upper_05_Shoot_R.AM_Turret_Upper_05_Shoot_R")))
    (Variables|Default|SetFiring true)
    (CallFunction|FireMultiplewithTimer (CallFunction|GetFirePoints (Variables|Default|GetActiveFirePointTag)) (Variables|Default|GetMainProjectileClass) (Variables|Default|GetMainFireTimerRate))))