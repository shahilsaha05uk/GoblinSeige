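; Upper turret variant 02, a child Blueprint that adds secondary small guns alongside its twin main gun.
; Main fire alternates two barrels when the target is reachable, running a trace that sets beam FX length, with left/right montages whose completion clears the firing lock.
; Small guns run on their own looping timer, cycling four tagged fire points to spawn projectiles, sound and FX until StopFire clears it.
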(event Custom|FireSmallGun
  ;[0.05 0.05 0.05] Setup small guns
  (if (and (Variables|Default|GetTargetIsSet) (CallFunction|IsTargetReachable 1e+04 "SG_FirePoint"))
    (if (== (Variables|Turret|SmallGun|GetSmallGunFirePointIndex) 3)
      (Variables|Turret|SmallGun|SetSmallGunFirePointIndex 0)
      (else
        (Math|Integer|IncrementInt (Variables|Turret|SmallGun|GetSmallGunFirePointIndex)
          (:%20%20
            _))))
    (Game|SpawnActorfromClass (Variables|Turret|SmallGun|GetSmallGunProjectile) (Transformation|GetWorldTransform (Utilities|Array|Get(acopy) (CallFunction|GetFirePoints "SG_FirePoint") (Variables|Turret|SmallGun|GetSmallGunFirePointIndex))) "AlwaysSpawn" "SelectDefaultAtRuntime" 0 (CallFunction|GetOwnerTurret))
    (Audio|PlaySoundatLocation (Variables|Turret|SmallGun|GetSmallGunFireSound) (.Location (Math|Transform|BreakTransform (Transformation|GetWorldTransform (Utilities|Array|Get(acopy) (CallFunction|GetFirePoints "SG_FirePoint") (Variables|Turret|SmallGun|GetSmallGunFirePointIndex))))) "0, 0, 0" 1.0 1.0 0.0 0 0 0 0)
    (Niagara|SpawnSystematLocation (Variables|Turret|SmallGun|GetSmallGunFireFX) (.Location (Math|Transform|BreakTransform (Transformation|GetWorldTransform (Utilities|Array|Get(acopy) (CallFunction|GetFirePoints "SG_FirePoint") (Variables|Turret|SmallGun|GetSmallGunFirePointIndex))))) (.Rotation (Math|Transform|BreakTransform (Transformation|GetWorldTransform (Utilities|Array|Get(acopy) (CallFunction|GetFirePoints "SG_FirePoint") (Variables|Turret|SmallGun|GetSmallGunFirePointIndex))))) "1.000000,1.000000,1.000000" true true "AutoRelease")))

(event EventSetupAutoFireTimer
  ;[0.05 0.05 0.05] Setup small guns
  (|CallParentFunction)
  (bind _returnvalue (Utilities|Time|SetTimerbyEvent (delegate Custom|FireSmallGun) (Variables|Turret|SmallGun|GetSmallGunsFireTimeRate) true (Variables|Turret|SmallGun|GetSmallGunsFireInitialDelay)))
  (Variables|Turret|SmallGun|SetSmallGunFireTimerHandle _returnvalue))

(event EventFire
  ;[0.05 0.05 0.05] Fire
  (if (and (not (CallFunction|IsFiring)) (CallFunction|IsTargetReachable 1e+04 "FirePoint"))
    (if (== (Variables|Default|GetActiveFirePointIndex) 0)
      (Variables|Default|SetActiveFirePointIndex 1)
      (else
        (Variables|Default|SetActiveFirePointIndex 0)))
    (Variables|Default|SetFiring true)
    (bind _fxcomponent (CallFunction|FireSingleFX (Utilities|Array|Get(acopy) (CallFunction|GetFirePoints "FirePoint") (Variables|Default|GetActiveFirePointIndex)) (Variables|Default|GetFireProjectilesFX)))
    (Utilities|IsValid _fxcomponent
      (:Is%20Valid
        (bind _outhit (CallFunction|FireSingleTrace (Utilities|Array|Get(acopy) (CallFunction|GetFirePoints "FirePoint") (Variables|Default|GetActiveFirePointIndex)) (Variables|Turret|MainGun|GetFireTraceLength) (Variables|Turret|MainGun|GetOnImpactFX) (Variables|Turret|MainGun|GetOnImpactSound) (Variables|Turret|MainGun|GetOnImpactDecal) (Variables|Turret|MainGun|GetOnImpactDecalLifetime) (Variables|Turret|MainGun|GetOnImpactDecalFadeOutDuration)))
        (if (.bBlockingHit (Collision|BreakHitResult _outhit))
          (Niagara|SetNiagaraVariable(Float) _fxcomponent "BeamLength" (.Distance (Collision|BreakHitResult _outhit)))
          (else
            (Niagara|SetNiagaraVariable(Float) _fxcomponent "BeamLength" (Variables|Turret|MainGun|GetFireTraceLength))))
        (Animation|Montage|PlayMontage (Variables|/Game/Turrets_Pack_01/Blueprints/BP_Turret.BP_Turret_C|GetUpper (CallFunction|GetOwnerTurret)) (Utilities|Array|Get(acopy) (Utilities|Array|MakeArray "/Game/Turrets_Pack_01/Animations/Upper/Upper_02/AM_Turret_Upper_02_Shoot_L.AM_Turret_Upper_02_Shoot_L" "/Game/Turrets_Pack_01/Animations/Upper/Upper_02/AM_Turret_Upper_02_Shoot_R.AM_Turret_Upper_02_Shoot_R") (Variables|Default|GetActiveFirePointIndex))
          (:OnCompleted
            (Variables|Default|SetFiring false)))))))

(event EventStopFire
  ;[0.05 0.05 0.05] Setup small guns
  (Utilities|Time|ClearandInvalidateTimerbyHandle (Variables|Turret|SmallGun|GetSmallGunFireTimerHandle))
  (|CallParentFunction))