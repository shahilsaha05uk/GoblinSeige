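; Base upper-turret logic for an owning BP_Turret, handling activation, targeting, firing, ammo and montage-driven reload.
; Timed sphere traces pick the nearest target by interface or tag, which can activate the turret and feed the auto-fire timer.
; Subclasses override Fire; helpers provide timed or multiple projectiles with homing, line-trace impacts, and Niagara stream fire that drains ammo by timer.
; Owner components are found by tag for the mesh, muzzles and flash lights.
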(event Custom|SetTargetActor
  (params (NewTarget :type Actor%20Object%20Reference))
  ;[0.05 0.05 0.05] Target
  (Variables|Turret|Target|SetPreviousTarget (Variables|Turret|Target|GetCurrentTarget))
  (bind _output_get (Variables|Turret|Target|SetCurrentTarget NewTarget))
  (Utilities|IsValid _output_get
    (:Is%20Valid
      (Variables|Turret|Target|SetCurrentTargetLocation (Transformation|GetActorLocation _output_get))
      (CallFunction|OnTargetFound))
    (:Is%20Not%20Valid
      (Variables|Turret|Target|SetCurrentTargetLocation "0, 0, 0")
      (CallFunction|OnTargetLost))))

(event Custom|Fire
  ;[0.05 0.05 0.05] Fire (should be overridden)
  (Development|PrintText (Utilities|Text|FormatText "Warning: Fire method is not overridden in {CurrentClass}" (Utilities|GetClassDisplayName (Utilities|GetClass self)))))

(event Custom|OnSingleProjectileFired
  (params (FirePoint :type Scene%20Component%20Object%20Reference))
  ;[0.05 0.05 0.05] On single projectile fired
  (CallFunction|ActivateFirePointLights true)
  (Utilities|FlowControl|Delay (Variables|Turret|Fire|Light|GetFirePointLightFlashDuration))
  (CallFunction|ActivateFirePointLights false))

(event Custom|StopFire
  (bind _turret (CallFunction|GetOwnerTurret))
  ;[0.05 0.05 0.05] Fire multiple with timer
  ;;[0.05 0.05 0.05] Stop fire
  (if (Variables|Turret|Fire|GetFiring)
    (Utilities|Time|ClearandInvalidateTimerbyHandle (Variables|Turret|Fire|GetFireTimerHandle))
    (Variables|Turret|Fire|SetActiveFirePointIndex 0)
    (Audio|PlaySoundatLocation (Variables|Turret|Fire|GetOnStopFireSound) (Transformation|GetActorLocation _turret) "0, 0, 0" 1.0 1.0 0.0 0 0 0 0)
    (CallFunction|StopFireFX)
    (if (not (Variables|Turret|Activation/Deactivation|GetDeactivating))
      (bind _onstopfiremontage (Variables|Turret|Fire|GetOnStopFireMontage)
        (:then
          (Animation|Montage|PlayMontage (Variables|/Game/Turrets_Pack_01/Blueprints/BP_Turret.BP_Turret_C|GetUpper _turret) _onstopfiremontage
            (:OnCompleted
              _)))
        (:else
          _))
      (Variables|Turret|Fire|SetFiring false)
      (if (and (Variables|Turret|Ammo/Reload|GetAutoReload) (or (not (CallFunction|HasAmmo 1)) (and (Variables|Turret|Ammo/Reload|GetAllowPartialReload) (CallFunction|HasAmmo (Variables|Turret|Ammo/Reload|GetPartialReloadMinAmmoNeeded)))))
        (CallFunction|Reload)))))

(event Custom|StartAmmoDecrementTimer
  ;[0.05 0.05 0.05] Ammo / Reload
  ;;[0.05 0.05 0.05] Ammo decrement
  (if (not (Variables|Turret|Ammo/Reload|GetInfiniteAmmo))
    (bind _returnvalue (Utilities|Time|SetTimerbyEvent (delegate Custom|TickDecrementAmmo) (Variables|Turret|Ammo/Reload|GetAmmoDecrementTimerRate) true))
    (Variables|Turret|Ammo/Reload|SetAmmoDecrementTimerHandle _returnvalue)))

(event Custom|TickDecrementAmmo
  ;[0.05 0.05 0.05] Ammo / Reload
  ;;[0.05 0.05 0.05] Ammo decrement
  (bind _output_get (Variables|Turret|Ammo/Reload|SetCurrentAmmo (Math|Integer|Clamp(Integer) (- (Variables|Turret|Ammo/Reload|GetCurrentAmmo) (Math|Float|Truncate (* (Variables|Turret|Projectiles|GetProjectilesPerSecond) (Variables|Turret|Ammo/Reload|GetAmmoDecrementTimerRate)))) 0 (Variables|Turret|Ammo/Reload|GetMaxAmmo))))
  (if (== _output_get 0)
    (Utilities|Time|ClearandInvalidateTimerbyHandle (Variables|Turret|Ammo/Reload|GetAmmoDecrementTimerHandle))
    (CallFunction|StopFire)))

(event Custom|SetupAutoFireTimer
  ;[0.05 0.05 0.05] Auto fire
  (if (and (Variables|Turret|Fire|Auto|GetAutoFire) (Variables|Turret|Activation/Deactivation|GetTurretActivated))
    (Utilities|Time|ClearandInvalidateTimerbyHandle (Variables|Turret|Fire|Auto|GetAutoFireTimerHandle))
    (bind _returnvalue (Utilities|Time|SetTimerbyEvent (delegate Custom|TickAutoFire) (Variables|Turret|Fire|Auto|GetAutoFireTimerRate) true (Variables|Turret|Fire|Auto|GetAutoFireTimerInitialDelay)))
    (Variables|Turret|Fire|Auto|SetAutoFireTimerHandle _returnvalue)))

(event Custom|OnTargetLost
  ;[0.05 0.05 0.05] Target
  ;;[0.05 0.05 0.05] On target lost
  (Variables|Turret|Target|SetTargetIsSet false)
  (if (Variables|Turret|Activation/Deactivation|GetDeactivateOnTargetLost)
    (CallFunction|DeactivateTurret)
    (else
      (CallFunction|StopFire))))

(event Custom|ActivateTurret
  (bind _mesh (CallFunction|GetUpperMeshComponent))
  ;[0.05 0.05 0.05] Activation / Deactivation
  (if (and (not (Variables|Turret|Activation/Deactivation|GetTurretActivated)) (not (Variables|Turret|Activation/Deactivation|GetActivating)))
    (Variables|Turret|Activation/Deactivation|SetActivating true)
    (Audio|PlaySoundatLocation (Variables|Turret|Activation/Deactivation|GetActivationSound) (Transformation|GetWorldLocation _mesh) "0, 0, 0" 1.0 1.0 0.0 0 0 0 0)
    (bind _activationmontage (Variables|Turret|Activation/Deactivation|GetActivationMontage)
      (:then
        (Animation|Montage|PlayMontage _mesh _activationmontage
          (:OnCompleted
            _)
          (:OnBlendOut
            _)
          (:OnInterrupted
            _)))
      (:else
        _))
    (Variables|Turret|Activation/Deactivation|SetTurretActivated true)
    (Variables|Turret|Activation/Deactivation|SetActivating false)
    (CallFunction|SetupAutoFireTimer)
    (Default|OnTurretActivated (CallFunction|GetOwnerTurret))))

(event Custom|OnTargetFound
  ;[0.05 0.05 0.05] Target
  ;;[0.05 0.05 0.05] On target lost
  (Variables|Turret|Target|SetTargetIsSet true)
  (if (!= (Variables|Turret|Target|GetPreviousTarget) (Variables|Turret|Target|GetCurrentTarget))
    (if (Variables|Turret|Activation/Deactivation|GetActivateOnTargetFound)
      (CallFunction|ActivateTurret)
      (else
        (CallFunction|SetupAutoFireTimer)))))

(event Custom|DeactivateTurret
  (bind _mesh (CallFunction|GetUpperMeshComponent))
  ;[0.05 0.05 0.05] Activation / Deactivation
  (if (and (Variables|Turret|Activation/Deactivation|GetTurretActivated) (not (Variables|Turret|Activation/Deactivation|GetDeactivating)))
    (Variables|Turret|Activation/Deactivation|SetDeactivating true)
    (Audio|PlaySoundatLocation (Variables|Turret|Activation/Deactivation|GetDeactivationSound) (Transformation|GetWorldLocation _mesh) "0, 0, 0" 1.0 1.0 0.0 0 0 0 0)
    (Utilities|Time|ClearandInvalidateTimerbyHandle (Variables|Turret|Fire|Auto|GetAutoFireTimerHandle))
    (CallFunction|StopFire)
    (bind _deactivationmontage (Variables|Turret|Activation/Deactivation|GetDeactivationMontage)
      (:then
        (Animation|Montage|PlayMontage _mesh _deactivationmontage 1.0 (Animation|GetPlayLength _deactivationmontage)
          (:OnCompleted
            _)))
      (:else
        _))
    (Variables|Turret|Activation/Deactivation|SetTurretActivated false)
    (Variables|Turret|Activation/Deactivation|SetDeactivating false)
    (Default|OnTurretDeactivated (CallFunction|GetOwnerTurret))))

(event Custom|Reload
  ;[0.05 0.05 0.05] Ammo / Reload
  (if (not (Variables|Turret|Ammo/Reload|GetReloading))
    (Variables|Turret|Ammo/Reload|SetReloading true)
    ;;[0.05 0.05 0.05] Stop auto fire timer
    (if (not (Variables|Turret|Ammo/Reload|GetAllowFireWhileReloading))
      (Utilities|Time|ClearandInvalidateTimerbyHandle (Variables|Turret|Fire|Auto|GetAutoFireTimerHandle)))
    ;;[0.05 0.05 0.05] Play start reload sound
    (Audio|PlaySoundatLocation (Variables|Turret|Ammo/Reload|GetReloadStartSound) (Transformation|GetActorLocation (Components|GetOwner)) "0, 0, 0" 1.0 1.0 0.0 0 0 0 0)
    ;;[0.05 0.05 0.05] Start reload animation
    (bind _reloadmontage (Variables|Turret|Ammo/Reload|GetReloadMontage)
      (:then
        (Animation|Montage|PlayMontage (CallFunction|GetUpperMeshComponent) _reloadmontage
          (:OnCompleted
            (Variables|Turret|Ammo/Reload|SetReloading false)
            ;;[0.05 0.05 0.05] Play reload completed sound
            (Audio|PlaySoundatLocation (Variables|Turret|Ammo/Reload|GetReloadEndSound) (Transformation|GetActorLocation (Components|GetOwner)) "0, 0, 0" 1.0 1.0 0.0 0 0 0 0))))
      (:else
        ;;[0.05 0.05 0.05] Reload delay
        (Utilities|FlowControl|Delay (Variables|Turret|Ammo/Reload|GetReloadDuration))
        (Variables|Turret|Ammo/Reload|SetReloading false)))
    ;;[0.05 0.05 0.05] Update current ammo value
    (Variables|Turret|Ammo/Reload|SetCurrentAmmo (Variables|Turret|Ammo/Reload|GetMaxAmmo))
    (CallFunction|SetupAutoFireTimer)))

(event Custom|ActivateFirePointLights
  (params (Enable :type Boolean))
  ;[0.05 0.05 0.05] Activate fire point lights
  (bind _newparam (CallFunction|GetActiveFirePointLights))
  (for _array_element _newparam
    (Rendering|SetVisibility _array_element Enable false)))

(event Custom|StartFirePointLightsActivationTimer
  ;[0.05 0.05 0.05] Activate fire point lights
  (bind _returnvalue (Utilities|Time|SetTimerbyEvent (delegate Custom|TickLights) (Variables|Turret|Fire|Light|GetFirePointLightActivationTimerRate) true))
  (Variables|Turret|Fire|Light|SetFirePointLightActivationTimerHandle _returnvalue))

(event Custom|StopFirePointLightsActivationTimer
  ;[0.05 0.05 0.05] Activate fire point lights
  (Utilities|Time|ClearandInvalidateTimerbyHandle (Variables|Turret|Fire|Light|GetFirePointLightActivationTimerHandle))
  (CallFunction|ActivateFirePointLights false))

(event Custom|TickLights
  ;[0.05 0.05 0.05] Activate fire point lights
  (CallFunction|ActivateFirePointLights true)
  (Utilities|FlowControl|Delay (Variables|Turret|Fire|Light|GetFirePointLightFlashDuration))
  (CallFunction|ActivateFirePointLights false))

(event Custom|SetTargetLocation
  (params (NewTarget :type Vector))
  ;[0.05 0.05 0.05] Target
  (Variables|Turret|Target|SetCurrentTargetLocation NewTarget)
  (CallFunction|OnTargetFound))

(event Custom|OnNeedAmmo
  ;[0.05 0.05 0.05] Ammo / Reload
  ;;[0.05 0.05 0.05] Need ammo
  (Audio|PlaySoundatLocation (Variables|Turret|Ammo/Reload|GetNeedAmmoSound) (Transformation|GetWorldLocation (CallFunction|GetUpperMeshComponent)) "0, 0, 0" 1.0 1.0 0.0 0 0 0 0)
  (CallFunction|StopFire))

(event Custom|ResetTarget
  ;[0.05 0.05 0.05] Target
  (Variables|Turret|Target|SetCurrentTarget 0)
  (Variables|Turret|Target|SetCurrentTargetLocation "0, 0, 0")
  (CallFunction|OnTargetLost))

(event Custom|TickAutoDetectNearestEnemy
  ;[0.05 0.05 0.05] Auto detect nearest enemy
  (if (Variables|Turret|Target|AutoDetect|GetAutoDetectByInterface)
    (bind _actor (CallFunction|FindNearestActorwithInterface (Variables|Turret|Target|AutoDetect|GetTurretTargetInterface)))
    (CallFunction|SetTargetActor _actor)
    (else
      (bind _actor_2 (CallFunction|FindNearestActorwithTag (Variables|Turret|Target|AutoDetect|GetTurretTargetTag)))
      (CallFunction|SetTargetActor _actor_2))))

(event Custom|TickAutoFire
  ;[0.05 0.05 0.05] Auto fire
  (if (Variables|Turret|Target|GetTargetIsSet)
    (CallFunction|Fire)
    (else
      (CallFunction|StopFire))))

(event Custom|FireMultipleWithTimer
  (params (FirePoints :type Array%20of%20Scene%20Component%20Object%20References) (ProjectileClass :type Actor%20Class%20Reference) (Time :type Float%20%28single-precision%29))
  ;[0.05 0.05 0.05] Fire multiple with timer
  (Utilities|Time|ClearandInvalidateTimerbyHandle (Variables|Turret|Fire|GetFireTimerHandle))
  (Variables|Turret|Fire|SetActiveFirePoints FirePoints)
  (Variables|Turret|Fire|SetActiveFirePointIndex 0)
  (bind _returnvalue (Utilities|Time|SetTimerbyEvent (delegate Custom|TickFireMultipleWithTimer) Time true))
  (Variables|Turret|Fire|SetFireTimerHandle _returnvalue)
  (Variables|Turret|Fire|SetFiring true))

(event Custom|TickFireMultipleWithTimer
  ;[0.05 0.05 0.05] Fire multiple with timer
  (if (and (Variables|Turret|Target|GetTargetIsSet) (Utilities|Array|IsValidIndex (Variables|Turret|Fire|GetActiveFirePoints) (Variables|Turret|Fire|GetActiveFirePointIndex)))
    (bind _projectile (CallFunction|FireSingle (Utilities|Array|Get(acopy) (Variables|Turret|Fire|GetActiveFirePoints) (Variables|Turret|Fire|GetActiveFirePointIndex)) (stale Custom|FireMultipleWithTimer ProjectileClass)))
    (Utilities|IsValid _projectile
      (:Is%20Valid
        (bind _postfiremontage (Variables|Turret|Fire|GetPostFireMontage)
          (:then
            (Animation|Montage|PlayMontage (Variables|/Game/Turrets_Pack_01/Blueprints/BP_Turret.BP_Turret_C|GetUpper (CallFunction|GetOwnerTurret)) _postfiremontage
              (:then
                _)))
          (:else
            _))
        (Math|Integer|IncrementInt (Variables|Turret|Fire|GetActiveFirePointIndex)))
      (:Is%20Not%20Valid
        (CallFunction|StopFire)))
    (else
      (CallFunction|StopFire))))

(event EventBeginPlay
  ;[0.05 0.05 0.05] Begin play
  (if (Variables|Turret|Activation/Deactivation|GetActivateOnBeginPlay)
    (CallFunction|ActivateTurret))
  (if (Variables|Turret|Target|AutoDetect|GetAutoDetectNearestTarget)
    (Utilities|Time|SetTimerbyEvent (delegate Custom|TickAutoDetectNearestEnemy) (Variables|Turret|Target|AutoDetect|GetAutoDetectNearestTargetTimerRate) true))
  (if (not (Variables|Turret|Activation/Deactivation|GetActivateOnBeginPlay))
    (CallFunction|SetupAutoFireTimer)))

(fn GetUpperMeshComponent
  (return (Utilities|Array|Get(acopy) (Actor|GetComponentsbyTag (Components|GetOwner) "/Script/Engine.SkeletalMeshComponent" "Upper"))))

(fn GetFirePoints
  (params (Tag :type Name :default "FirePoint"))
  (for _array_element (Actor|GetComponentsbyTag (Components|GetOwner) "/Script/Engine.SceneComponent" Tag)
    (if (not (Components|ComponentHasTag _array_element "FPL"))
      (Utilities|Array|Add (LocalVariables|GetOutFirePoints) _array_element)))
  (return (LocalVariables|GetOutFirePoints)))

(fn FireSingle
  (params (FirePoint :type Scene%20Component%20Object%20Reference) (ProjectileClass :type Actor%20Class%20Reference))
  (bind _returnvalue (Transformation|GetWorldTransform FirePoint))
  (bind _returnvalue_2 (Transformation|GetWorldTransform FirePoint))
  (if (CallFunction|HasAmmo 1)
    ;[0.05 0.05 0.05] Spend ammo
    (CallFunction|ConsumeAmmo)
    ;[0.05 0.05 0.05] Spawn
    (bind _returnvalue_3 (Game|SpawnActorfromClass ProjectileClass (Math|Transform|MakeTransform (.location _returnvalue) (.rotation _returnvalue) "1.000000,1.000000,1.000000") "AlwaysSpawn" "SelectDefaultAtRuntime" 0 (CallFunction|GetOwnerTurret)))
    (CallFunction|OnSingleProjectileFired FirePoint)
    ;[0.05 0.05 0.05] Play fire sound
    (Audio|PlaySoundatLocation (Variables|Turret|Fire|GetFireSound) (.location _returnvalue_2) "0, 0, 0" 1.0 1.0 0.0 0 0 0 0)
    ;[0.05 0.05 0.05] Spawn fire FX
    (bind _firefx (Variables|Turret|Fire|GetFireFX)
      (:then
        (Niagara|SpawnSystematLocation _firefx (.location _returnvalue_2) (.rotation _returnvalue_2) "1.000000,1.000000,1.000000" true true "AutoRelease"))
      (:else
        _))
    ;[0.05 0.05 0.05] Set homing projectile target
    (if (Math|Boolean|ANDBoolean (Variables|/Script/Engine.ProjectileMovementComponent|GetbIsHomingProjectile (Actor|GetComponentbyClass _returnvalue_3 "/Script/Engine.ProjectileMovementComponent")) (Variables|Turret|Target|GetTargetIsSet) (Utilities|IsValid (Variables|Turret|Target|GetCurrentTarget)))
      (Variables|/Script/Engine.ProjectileMovementComponent|SetHomingTargetComponent (Actor|GetComponentbyClass _returnvalue_3 "/Script/Engine.ProjectileMovementComponent") (Variables|/Script/Engine.Actor|GetRootComponent (Variables|Turret|Target|GetCurrentTarget))))
    (return _returnvalue_3)
    (else
      (CallFunction|OnNeedAmmo)
      (return 0))))

(fn FireMultiple
  (params (FirePoints :type Array%20of%20Scene%20Component%20Object%20References) (ProjectileClass :type Actor%20Class%20Reference))
  (for _array_element FirePoints
    (bind _projectile (CallFunction|FireSingle _array_element ProjectileClass))
    (Utilities|IsValid _projectile
      (:Is%20Valid
        (Utilities|Array|Add (LocalVariables|GetOutProjectiles) _projectile))
      (:Is%20Not%20Valid
        (return (LocalVariables|GetOutProjectiles)))))
  (return (LocalVariables|GetOutProjectiles)))

(fn GetOwnerTurret
  (return (.AsBP%20Turret (Utilities|Casting|CastToBP_Turret (Components|GetOwner)))))

(fn HasAmmo
  (params (Capacity :type Integer))
  (bind _currentammo (Variables|Turret|Ammo/Reload|GetCurrentAmmo))
  (return (or (and (> _currentammo 0) (<= Capacity _currentammo)) (Variables|Turret|Ammo/Reload|GetInfiniteAmmo))))

(fn FindNearestActorwithInterface
  (params (Interface :type Interface%20Class%20Reference))
  (bind _returnvalue (Components|GetOwner))
  (bind _autodetectnearesttargetradius (Variables|Turret|Target|AutoDetect|GetAutoDetectNearestTargetRadius))
  (bind _returnvalue_2 (Transformation|GetActorLocation _returnvalue))
  (LocalVariables|SetOutDistance _autodetectnearesttargetradius)
  (bind _outhits (Collision|MultiSphereTraceForObjects _returnvalue_2 _returnvalue_2 _autodetectnearesttargetradius (Variables|Turret|Target|AutoDetect|GetAutoDetectNearestTargetObjectTypes) false 0 (Variables|Turret|Target|AutoDetect|GetAutoDetectRadiusDrawDebugType)))
  (for _array_element _outhits
    (if (and (Utilities|DoesObjectImplementInterface (.HitActor (Collision|BreakHitResult _array_element)) Interface) (< (Math|Vector|Distance(Vector) (Transformation|GetActorLocation (Components|GetOwner)) (Transformation|GetActorLocation (.HitActor (Collision|BreakHitResult _array_element)))) (LocalVariables|GetOutDistance)))
      (LocalVariables|SetOutDistance (Math|Vector|Distance(Vector) (Transformation|GetActorLocation (Components|GetOwner)) (Transformation|GetActorLocation (.HitActor (Collision|BreakHitResult _array_element)))))
      (LocalVariables|SetOutActor (.HitActor (Collision|BreakHitResult _array_element)))))
  (return (LocalVariables|GetOutActor) (LocalVariables|GetOutDistance)))

(fn FindNearestActorwithTag
  (params (Tag :type Name))
  (bind _returnvalue (Components|GetOwner))
  (bind _autodetectnearesttargetradius (Variables|Turret|Target|AutoDetect|GetAutoDetectNearestTargetRadius))
  (bind _returnvalue_2 (Transformation|GetActorLocation _returnvalue))
  (LocalVariables|SetOutDistance _autodetectnearesttargetradius)
  (bind _outhits (Collision|MultiSphereTraceForObjects _returnvalue_2 _returnvalue_2 _autodetectnearesttargetradius (Variables|Turret|Target|AutoDetect|GetAutoDetectNearestTargetObjectTypes) false 0 (Variables|Turret|Target|AutoDetect|GetAutoDetectRadiusDrawDebugType)))
  (for _array_element _outhits
    (if (and (Actor|ActorHasTag (.HitActor (Collision|BreakHitResult _array_element)) Tag) (< (Math|Vector|Distance(Vector) (Transformation|GetActorLocation (Components|GetOwner)) (Transformation|GetActorLocation (.HitActor (Collision|BreakHitResult _array_element)))) (LocalVariables|GetOutDistance)))
      (LocalVariables|SetOutDistance (Math|Vector|Distance(Vector) (Transformation|GetActorLocation (Components|GetOwner)) (Transformation|GetActorLocation (.HitActor (Collision|BreakHitResult _array_element)))))
      (LocalVariables|SetOutActor (.HitActor (Collision|BreakHitResult _array_element)))))
  (return (LocalVariables|GetOutActor) (LocalVariables|GetOutDistance)))

(fn GetTargetLocation
  (bind _currenttarget (Variables|Turret|Target|GetCurrentTarget)
    (:then
      (return (+ (Variables|Turret|Target|GetCurrentTargetLocationOffset) (Transformation|GetActorLocation _currenttarget)) (Variables|Turret|Target|GetTargetIsSet)))
    (:else
      (return (+ (Variables|Turret|Target|GetCurrentTargetLocationOffset) (Variables|Turret|Target|GetCurrentTargetLocation)) (Variables|Turret|Target|GetTargetIsSet)))))

(fn IsFiring
  (return (or (Utilities|Time|IsTimerActivebyHandle (Variables|Turret|Fire|GetFireTimerHandle)) (Variables|Turret|Fire|GetFiring))))

(fn StartFireFX
  (if (CallFunction|HasAmmo (Math|Float|Truncate (* (Variables|Turret|Projectiles|GetProjectilesPerSecond) (Variables|Turret|Ammo/Reload|GetAmmoDecrementTimerRate))))
    (Variables|Turret|Projectiles|GetFireProjectilesFXComponent
      (:then
        _)
      (:else
        (bind _returnvalue (Niagara|SpawnSystemAttached (Variables|Turret|Projectiles|GetFireProjectilesFX) (Utilities|Array|Get(acopy) (CallFunction|GetFirePoints "FirePoint")) "None" "0, 0, 0" "0, 0, 0" "SnapToTarget" false))
        (bind _output_get (Variables|Turret|Projectiles|SetFireProjectilesFXComponent _returnvalue))))
    (Niagara|SetNiagaraVariable(Float) _output_get "ProjectilesPerSecond" (Variables|Turret|Projectiles|GetProjectilesPerSecond))
    (Variables|Turret|Fire|SetFiring true)
    (CallFunction|StartAmmoDecrementTimer)
    (CallFunction|StartFirePointLightsActivationTimer)))

(fn StopFireFX
  (bind _fireprojectilesfxcomponent (Variables|Turret|Projectiles|GetFireProjectilesFXComponent)
    (:then
      (Niagara|SetNiagaraVariable(Float) _fireprojectilesfxcomponent "ProjectilesPerSecond" 0.0))
    (:else
      _))
  (Variables|Turret|Fire|SetFiring false)
  (CallFunction|StopFirePointLightsActivationTimer))

(fn FindLookatTargetRotation
  (bind _returnvalue (Components|GetOwner))
  (bind (_location _targetisset) (CallFunction|GetTargetLocation))
  (bind _returnvalue_2 (Transformation|GetActorRotation _returnvalue))
  (bind _returnvalue_3 (Transformation|GetActorLocation _returnvalue))
  (bind _returnvalue_4 (Math|Rotator|FindLookatRotation _returnvalue_3 _location))
  (return (Math|Rotator|MakeRotator (- (.roll _returnvalue_4) (.roll _returnvalue_2)) (* (- (.pitch _returnvalue_4) (.pitch _returnvalue_2)) -1.0) (- (.yaw _returnvalue_4) (.yaw _returnvalue_2))) _targetisset))

(fn ConsumeAmmo
  (Variables|Turret|Ammo/Reload|SetCurrentAmmo (Math|Integer|Clamp(Integer) (- (Variables|Turret|Ammo/Reload|GetCurrentAmmo) 1) 0 (Variables|Turret|Ammo/Reload|GetMaxAmmo))))

(fn FireSingleFX
  (params (FirePoint :type Scene%20Component%20Object%20Reference) (FX :type Niagara%20System%20Object%20Reference))
  (bind _returnvalue (Transformation|GetWorldTransform FirePoint))
  (if (CallFunction|HasAmmo 1)
    ;[0.05 0.05 0.05] Spend ammo
    (CallFunction|ConsumeAmmo)
    (bind _returnvalue_2 (Niagara|SpawnSystematLocation FX (.location _returnvalue) (.rotation _returnvalue)))
    (CallFunction|OnSingleProjectileFired FirePoint)
    ;[0.05 0.05 0.05] Play fire sound
    (Audio|PlaySoundatLocation (Variables|Turret|Fire|GetFireSound) (Transformation|GetWorldLocation (CallFunction|GetUpperMeshComponent)) "0, 0, 0" 1.0 1.0 0.0 0 0 0 0)
    (return _returnvalue_2)
    (else
      (CallFunction|OnNeedAmmo)
      (return 0))))

(fn FireSingleTrace
  (params (FirePoint :type Scene%20Component%20Object%20Reference) (TraceLength :type Float%20%28double-precision%29) (OnImpactFX :type Niagara%20System%20Object%20Reference) (OnImpactSound :type Sound%20Base%20Object%20Reference) (OnImpactDecal :type Material%20Interface%20Object%20Reference) (ImpactDecalLifetime :type Float%20%28double-precision%29) (ImpactDecalFadeOutDuration :type Float%20%28double-precision%29))
  (bind _returnvalue (Transformation|GetWorldLocation FirePoint))
  (bind _outhit (Collision|LineTraceByChannel _returnvalue (+ _returnvalue (* (Math|Vector|GetForwardVector FirePoint) TraceLength)) "TraceTypeQuery1" false 0 "None"))
  (if (.bBlockingHit (Collision|BreakHitResult _outhit))
    (bind _onimpactfx (LocalVariables|GetOnImpactFX)
      (:then
        (Niagara|SpawnSystematLocation _onimpactfx (.ImpactPoint (Collision|BreakHitResult _outhit)) (Math|Conversions|RotationFromXVector (.ImpactNormal (Collision|BreakHitResult _outhit))) "1.000000,1.000000,1.000000" true true "AutoRelease"))
      (:else
        _))
    (Audio|PlaySoundatLocation OnImpactSound (.ImpactPoint (Collision|BreakHitResult _outhit)) "0, 0, 0" 1.0 1.0 0.0 0 0 0 0)
    (bind _onimpactdecal (LocalVariables|GetOnImpactDecal)
      (:then
        (bind _returnvalue_2 (Class|GameplayStatics|SpawnDecalAttached _onimpactdecal "64.000000,64.000000,64.000000" (.HitComponent (Collision|BreakHitResult _outhit)) "None" (.ImpactPoint (Collision|BreakHitResult _outhit)) (Math|Conversions|RotationFromXVector (.ImpactNormal (Collision|BreakHitResult _outhit))) "KeepWorldPosition" ImpactDecalLifetime))
        (Rendering|Components|Decal|SetFadeOut _returnvalue_2 (- ImpactDecalLifetime ImpactDecalFadeOutDuration) ImpactDecalFadeOutDuration false))
      (:else
        _))
    (return _outhit)
    (else
      (return _outhit))))

(fn IsTargetReachable
  (params (Range :type Float%20%28double-precision%29) (FirePointTag :type Name :default "FirePoint"))
  (if (Variables|Turret|Target|GetTargetIsSet)
    (if (Variables|Turret|Fire|GetDisableFireWhileTargetIsUnreachable)
      (return (Math|Float|InRange(Float) (.pitch (.ReturnValue (CallFunction|FindLookatTargetRotation))) (Variables|Turret|Aim|GetMinAimPitch) (Variables|Turret|Aim|GetMaxAimPitch)))
      (else
        (return true)))
    (else
      (return false))))

(fn GetActiveFirePointLights
  (bind _returnvalue (Components|GetOwner))
  (bind _activefirepointtag (Variables|Turret|Fire|GetActiveFirePointTag))
  (bind _returnvalue_2 (Actor|GetComponentsByClass _returnvalue "/Script/Engine.LightComponent"))
  (if (> (Utilities|Array|Length _returnvalue_2) 1)
    (for _array_element _returnvalue_2
      (if (and (Components|ComponentHasTag _array_element "FPL") (or (and (!= _activefirepointtag "") (Components|ComponentHasTag _array_element _activefirepointtag)) (== _activefirepointtag "")))
        (Utilities|Array|Add (LocalVariables|GetOutLights) _array_element)))
    (return (LocalVariables|GetOutLights))
    (elif (Components|ComponentHasTag (Utilities|Array|Get(acopy) _returnvalue_2) "FPL")
      (return _returnvalue_2)
      (else
        (return 0)))))