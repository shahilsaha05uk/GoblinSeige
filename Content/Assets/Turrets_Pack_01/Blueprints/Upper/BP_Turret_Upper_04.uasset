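; Upper turret weapon Blueprint that fires continuous hitscan shots while a target is reachable.
; Fire checks range and ammo, reloading when short, then plays a pre-fire sound and optional montage before starting the attached fire sound and FX.
; A looping timer, paced by projectiles per second, performs single traces from the first fire point with impact effects.
; StopFire ends the sound and timer, then calls the parent.
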(event Custom|TraceProjectile
  (if (CallFunction|IsFiring)
    (CallFunction|FireSingleTrace (Utilities|Array|Get(acopy) (CallFunction|GetFirePoints "FirePoint")) (Variables|Turret|Minigun|GetFireTraceLength) (Variables|Turret|Minigun||GetOnImpactFX) (Variables|Turret|Minigun|GetOnImpactSound) (Variables|Turret|Minigun|GetOnImpactDecal) (Variables|Turret|Minigun|GetOnImpactDecalLifetime) (Variables|Turret|Minigun|GetOnImpactDecalFadeOutDuration))
    (else
      (Utilities|Time|ClearandInvalidateTimerbyHandle (Variables|Turret|Minigun|GetTraceProjectileTimerHandle)))))

(event EventStopFire
  (bind _firesoundreference (Variables|Turret|Minigun|GetFireSoundReference)
    (:then
      (Audio|Components|Audio|Stop _firesoundreference)
      (Components|DestroyComponent _firesoundreference)
      (Utilities|Time|ClearandInvalidateTimerbyHandle (Variables|Turret|Minigun|GetTraceProjectileTimerHandle)))
    (:else
      _))
  (|CallParentFunction))

(event EventFire
  (bind _turret (CallFunction|GetOwnerTurret))
  (bind _upper (Variables|/Game/Turrets_Pack_01/Blueprints/BP_Turret.BP_Turret_C|GetUpper _turret))
  (bind _returnvalue (Transformation|GetWorldTransform _upper))
  (if (CallFunction|IsTargetReachable 1e+04 "FirePoint")
    (if (and (not (CallFunction|IsFiring)) (not (Variables|Turret|Minigun|GetIsPlayingMontage)))
      (if (CallFunction|HasAmmo (Math|Float|Truncate (* (Variables|Default|GetProjectilesPerSecond) (Variables|Default|GetAmmoDecrementTimerRate))))
        (Audio|PlaySoundatLocation (Variables|Default|GetPreFireSound) (Transformation|GetActorLocation (Components|GetOwner)) "0, 0, 0" 1.0 1.0 0.0 0 0 0 0)
        (bind _prefiremontage (Variables|Default|GetPreFireMontage)
          (:then
            (Animation|Montage|PlayMontage _upper _prefiremontage
              (:then
                (Variables|Turret|Minigun|SetIsPlayingMontage true))
              (:OnCompleted
                (Variables|Turret|Minigun|SetIsPlayingMontage false :!label _label)
                (Variables|Default|SetFiring true)
                (bind _returnvalue_2 (Audio|SpawnSoundAttached (Variables|Default|GetFireSound) _upper "None" (.location _returnvalue) (.rotation _returnvalue) "SnapToTargetIncludingScale" false 1.0 1.0 0.0 0 0))
                (Variables|Turret|Minigun|SetFireSoundReference _returnvalue_2)
                (CallFunction|StartFireFX)
                (bind _returnvalue_3 (Utilities|Time|SetTimerbyEvent (delegate Custom|TraceProjectile) (/ 1.0 (Variables|Default|GetProjectilesPerSecond)) true))
                (Variables|Turret|Minigun|SetTraceProjectileTimerHandle _returnvalue_3))))
          (:else
            (goto _label)))
        (else
          (CallFunction|Reload))))
    (else
      (CallFunction|StopFire))))