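; BP_Tower is an automatic weapon tower that detects and selects enemy targets within range.
; Range-collision overlaps track actors implementing BI_EnemyInterface and recompute the nearest one as targets enter or leave.
; IdentifyTheTarget keeps the current target locked until it leaves the list, then switches to the closest, signaling through empty FindTarget and NOTarget events.
; OnIncreaseRange grows the attack radius, but its looping timer is disconnected.
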(event OnComponentBeginOverlap(RangeCollisionComp)
  (params (OverlappedComponent :type Primitive%20Component%20Object%20Reference) (OtherActor :type Actor%20Object%20Reference) (OtherComp :type Primitive%20Component%20Object%20Reference) (OtherBodyIndex :type Integer) (bFromSweep :type Boolean) (SweepResult :type Hit%20Result%20Structure%20%28by%20ref%29))
  (bind _targets (Variables|Default|GetTargets))
  ;[1 0 0.2339] Find Target(得加个锁定目标
  (if (Utilities|DoesObjectImplementInterface OtherActor "/Game/BP/AI/BI_EnemyInterface.BI_EnemyInterface_C")
    (Utilities|Array|AddUnique _targets OtherActor)
    (Variables|Default|SetClosestTarget (.ReturnValue (Actor|FindNearestActor (Transformation|GetActorLocation) _targets)))
    (CallFunction|IdentifytheTarget)
    (CallFunction|FindTarget)))

(event OnComponentEndOverlap(RangeCollisionComp)
  (params (OverlappedComponent :type Primitive%20Component%20Object%20Reference) (OtherActor :type Actor%20Object%20Reference) (OtherComp :type Primitive%20Component%20Object%20Reference) (OtherBodyIndex :type Integer))
  (bind _targets (Variables|Default|GetTargets))
  ;[1 0 0.2339] Find Target(得加个锁定目标
  (if (Utilities|DoesObjectImplementInterface OtherActor "/Game/BP/AI/BI_EnemyInterface.BI_EnemyInterface_C")
    (Utilities|Array|RemoveItem _targets OtherActor)
    (if (Utilities|Array|IsNotEmpty _targets)
      (Variables|Default|SetClosestTarget (.ReturnValue (Actor|FindNearestActor (Transformation|GetActorLocation) (Variables|Default|GetTargets))))
      (CallFunction|IdentifytheTarget)
      (CallFunction|FindTarget)
      (else
        (Variables|Default|SetClosestTarget 0)
        (Variables|Default|SetCurrentTarget 0)
        (CallFunction|NOTarget)))))

(event Custom|OnIncreaseRange
  (Variables|Default|SetmAttackRadius (+ (Variables|Default|GetmAttackRadius) 1e+02))
  (CallFunction|IncreaseRange)
  (Development|PrintString "range should increase"))

(event Custom|NOTarget
  ;[1 1 1] 注释
)

(event Custom|FindTarget
  ;[1 1 1] 注释
)

(event EventBeginPlay)

(fn ConstructionScript
  (|CallParentFunction))

(fn IdentifytheTarget
  (if (Utilities|Array|ContainsItem (Variables|Default|GetTargets) (Variables|Default|GetCurrentTarget))
    _
    (else
      (Variables|Default|SetCurrentTarget (Variables|Default|GetClosestTarget))))
  (return))