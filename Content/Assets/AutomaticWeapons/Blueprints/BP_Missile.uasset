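; BP_Missile is a homing missile projectile that launches at LaunchSpeed and explodes on hit.
; After a short delay it enables Tick, which interpolates velocity toward ClosestTarget and raises speed every frame, making acceleration frame-rate dependent.
; ClosestTarget is not assigned within these graphs.
; On hit it spawns an explosion effect, applies full radial damage that obstacles on the Pawn channel block, then destroys itself.
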(event EventBeginPlay
  (Utilities|FlowControl|Delay 0.5)
  (Actor|Tick|SetActorTickEnabled true))

(event EventTick
  (params (DeltaSeconds :type Float%20%28single-precision%29))
  (bind _closesttarget (Variables|Default|GetClosestTarget))
  (Utilities|IsValid _closesttarget
    (:Is%20Valid
      (Variables|Default|SetTaygetLocation (Transformation|GetActorLocation _closesttarget))
      (Variables|/Script/Engine.MovementComponent|SetVelocity (Variables|Default|GetProjectileMovement) (Math|Interpolation|VInterpTo (Variables|/Script/Engine.MovementComponent|GetVelocity (Variables|Default|GetProjectileMovement)) (* (Math|Vector|GetUnitDirection(Vector) (Transformation|GetActorLocation) (Variables|Default|GetTaygetLocation)) (Variables|Default|GetLaunch%20speed)) (Utilities|Time|GetWorldDeltaSeconds) 3.0))
      (Variables|Default|SetLaunch%20speed (+ (Variables|Default|GetLaunch%20speed) 5e+02)))))

(event Collision|EventHit
  (params (MyComp :type Primitive%20Component%20Object%20Reference) (Other :type Actor%20Object%20Reference) (OtherComp :type Primitive%20Component%20Object%20Reference) (bSelfMoved :type Boolean) (HitLocation :type Vector :default "0, 0, 0") (HitNormal :type Vector :default "0, 0, 0") (NormalImpulse :type Vector :default "0, 0, 0") (Hit :type Hit%20Result%20Structure%20%28by%20ref%29))
  (Niagara|SpawnSystematLocation "/Game/Assets/AutomaticWeapons/Particles/FX_Explode.FX_Explode" HitLocation "0, 0, 0" "5.000000,5.000000,5.000000")
  (Game|Damage|ApplyRadialDamage (Variables|Default|GetBase%20Damage) (Transformation|GetActorLocation) 5e+02 0 0 self 0 true "ECC_Pawn") ; 可视性遮挡则无伤害
  (Actor|DestroyActor))

(fn ConstructionScript
  (Variables|/Script/Engine.ProjectileMovementComponent|SetInitialSpeed (Variables|Default|GetProjectileMovement) (Variables|Default|GetLaunch%20speed)))