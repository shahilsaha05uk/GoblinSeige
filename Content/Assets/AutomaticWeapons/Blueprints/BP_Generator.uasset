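; BP_Generator is an area spawner that creates a set quantity of BP_Enemy actors when play begins.
; Each enemy spawns at a random point in a box around the generator, raised vertically, receiving the generator reference and configured HP.
; A custom Spwan event shares the same spawn node, allowing a single enemy to be spawned on demand.
; The construction script sizes the Box and Plane components from Scale3D to match the spawn area.
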(event Custom|Spwan
  (Game|SpawnActorfromClass "/Game/BP/AI/BP_Enemy.BP_Enemy_C" (Math|Transform|MakeTransform (+ (Math|Random|RandomPointinBoundingBox (Transformation|GetActorLocation) (Variables|Default|GetScale3D)) "0.000000,0.000000,88.000000") (Transformation|GetActorRotation) "1.000000,1.000000,1.000000") "AdjustIfPossibleButAlwaysSpawn" "MultiplyWithRoot" 0 self (Variables|Default|GetHP) 0))

(event EventBeginPlay
  (for _index (range 1 (Variables|Default|GetQuantity))
    (Game|SpawnActorfromClass "/Game/BP/AI/BP_Enemy.BP_Enemy_C" (Math|Transform|MakeTransform (+ (Math|Random|RandomPointinBoundingBox (Transformation|GetActorLocation) (Variables|Default|GetScale3D)) "0.000000,0.000000,88.000000") (Transformation|GetActorRotation) "1.000000,1.000000,1.000000") "AdjustIfPossibleButAlwaysSpawn" "MultiplyWithRoot" 0 self (Variables|Default|GetHP) 0)))

(event Collision|EventActorBeginOverlap
  (params (OtherActor :type Actor%20Object%20Reference)))

(event EventTick
  (params (DeltaSeconds :type Float%20%28single-precision%29)))

(fn ConstructionScript
  (bind _scale3d (Variables|Default|GetScale3D))
  (Components|Box|SetBoxExtent (Variables|Default|GetBox) _scale3d true)
  (Transformation|SetWorldScale3D (Variables|Default|GetPlane) (/ _scale3d 5e+01)))