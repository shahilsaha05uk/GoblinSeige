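; Arrow tower automatic weapon that shoots projectiles at its current target.
; On Fire, it aims the Arrow component at a living target and spawns the projectile class from that component's transform.
; If the target is invalid or reports dead through IsDeadMessage, it calls FindTarget and only aims at the new target, without shooting in that call.
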(event EventLookatTarget
  (bind _arrow (Variables|Default|GetArrow))
  (bind _currenttarget (Variables|Default|GetCurrentTarget))
  (Utilities|IsValid _currenttarget
    (:Is%20Valid
      (Transformation|SetWorldRotation _arrow (Math|Rotator|FindLookatRotation (Transformation|GetWorldLocation _arrow) (Transformation|GetActorLocation _currenttarget)) false false))))

(event EventFire
  (bind _arrow (Variables|Default|GetArrow))
  (bind _returnvalue (Transformation|GetWorldTransform _arrow))
  (bind _currenttarget (Variables|Default|GetCurrentTarget)
    (:then
      (bind _returnvalue_2 (Class|EnemyInterface|IsDead(Message) _currenttarget))
      (if _returnvalue_2
        (bind _returnvalue_3 (Class|Turret|FindTarget :!label _label))
        (bind _output_get (Variables|Default|SetCurrentTarget _returnvalue_3))
        (Utilities|IsValid _output_get
          (:Is%20Valid
            (Class|Turret|LookatTarget)))
        (else
          (Class|Turret|LookatTarget)
          (Class|Turret|SpawnProjectile (Variables|Default|GetmProjectileClass) (.location _returnvalue) (.rotation _returnvalue) 0))))
    (:else
      (goto _label))))

(fn ConstructionScript
  (|CallParentFunction))