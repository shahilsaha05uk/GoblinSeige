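; Cannon tower that automatically lobs BP_Bomb projectiles at its current target while attacking, driven by find and lose target events.
; Each tick until yaw locks on, it smoothly yaws one mesh toward the target and pitches another along a suggested ballistic arc to the target's ground position.
; Firing waits an aim delay estimated from the yaw gap, spawns the bomb at the arrow, then reloads and re-aims for the next shot.
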(event Custom|Fire
  (bind _arrow (Variables|Default|GetArrow))
  (bind _returnvalue (Transformation|GetWorldTransform _arrow))
  ;[1 1 1] Fire
  (Variables|Default|SetAimingTime (CallFunction|CalculatetheAimingTime))
  (Utilities|FlowControl|Delay (Variables|Default|GetAimingTime))
  (if (Variables|Default|GetReady)
    (Game|SpawnActorfromClass "/Game/Assets/AutomaticWeapons/Blueprints/BP_Bomb.BP_Bomb_C" (Math|Transform|MakeTransform (.location _returnvalue) (.rotation _returnvalue) "1.000000,1.000000,1.000000") "Undefined" "OverrideRootScale" 0 (Variables|Default|GetLaunch%20Speed) (Variables|Default|GetBase%20Damage) 0)
    ;;[1 1 1] Simulate reload time
    (Variables|Default|SetReady false)
    (Utilities|FlowControl|Delay (Variables|Default|GetInterval))
    (Variables|Default|SetReady true)
    (if (Variables|Default|GetAttacking)
      (Variables|Default|SetTargeted false)
      (CallFunction|Fire))))

(event EventBeginPlay
  (|CallParentFunction) ; 此节点被禁用，将不会被调用。\n从引脚连出引线来编译功能。
)

(event Collision|EventActorBeginOverlap
  (params (OtherActor :type Actor%20Object%20Reference))
  (|CallParentFunction OtherActor) ; 此节点被禁用，将不会被调用。\n从引脚连出引线来编译功能。
)

(event EventTick
  (params (DeltaSeconds :type Float%20%28single-precision%29))
  (|CallParentFunction DeltaSeconds)
  (CallFunction|FacingTarget))

(event EventFindTarget
  (if (not (Variables|Default|GetAttacking))
    (Variables|Default|SetAttacking true)
    (CallFunction|Fire)))

(event EventNOTarget
  (Variables|Default|SetAttacking false))

(fn ConstructionScript
  (|CallParentFunction))

(fn FacingTarget
  (bind _currenttarget (Variables|Default|GetCurrentTarget))
  (bind _m_fort3 (Variables|Default|GetM_Fort3))
  (bind _m_fort3_2 (Variables|Default|GetM_Fort3))
  (bind _m_fort2 (Variables|Default|GetM_Fort2))
  (bind _returnvalue (Transformation|GetWorldLocation _m_fort3_2))
  (bind _returnvalue_2 (Transformation|GetWorldRotation _m_fort3))
  (bind _returnvalue_3 (Transformation|GetWorldRotation _m_fort2))
  (bind _returnvalue_4 (Transformation|GetActorLocation _currenttarget))
  (bind _returnvalue_5 (Math|Rotator|FindLookatRotation _returnvalue _returnvalue_4))
  (if (not (Variables|Default|GetTargeted))
    (Variables|Default|GetCurrentTarget
      (:then
        (Utilities|FlowControl|Sequence
          (:then_0
            (bind _tossvelocity (Class|GameplayStatics|BlueprintSuggestProjectileVelocity (Transformation|GetWorldLocation (Variables|Default|GetArrow)) (- (Transformation|GetActorLocation (Variables|Default|GetCurrentTarget)) "0.000000,0.000000,80.000000") (Variables|Default|GetLaunch%20Speed) 0.0 "DoNotTrace" 1.0 false false))
            (Transformation|SetWorldRotation _m_fort3 (Math|Rotator|MakeRotator (.roll _returnvalue_2) (.pitch (Math|Interpolation|RInterpTo (Transformation|GetWorldRotation _m_fort3) (Math|Conversions|RotationFromXVector _tossvelocity) (Utilities|Time|GetWorldDeltaSeconds) 5.0)) (.yaw _returnvalue_2)) false false))
          (:then_1
            (Transformation|SetWorldRotation _m_fort2 (Math|Rotator|MakeRotator (.roll _returnvalue_3) (.pitch _returnvalue_3) (.yaw (Math|Interpolation|RInterpTo (Transformation|GetWorldRotation _m_fort2) _returnvalue_5 (Utilities|Time|GetWorldDeltaSeconds) 5.0))) false false)
            (Variables|Default|SetTargeted (<= (Math|Float|Absolute(Float) (.yaw (Math|Rotator|Delta(Rotator) _returnvalue_5 (Transformation|GetWorldRotation (Variables|Default|GetM_Fort2))))) 0.2)))))
      (:else))))

(fn CalculatetheAimingTime
  (return (/ (Math|Float|Absolute(Float) (.yaw (Math|Rotator|Delta(Rotator) (Math|Rotator|FindLookatRotation (Transformation|GetWorldLocation (Variables|Default|GetM_Fort3)) (Transformation|GetActorLocation (Variables|Default|GetCurrentTarget))) (Transformation|GetWorldRotation (Variables|Default|GetM_Fort2))))) 1.5e+02)))