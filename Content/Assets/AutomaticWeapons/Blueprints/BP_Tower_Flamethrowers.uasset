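; Flamethrower tower that turns toward its current target and burns enemies inside a forward box.
; Each tick it smoothly interpolates yaw on one turret mesh and pitch on another toward the target.
; FindTarget starts the flame effect and a looping timer that damages every BP_Enemy overlapping the box; NOTarget stops both.
; The construction script sizes and offsets the box along X from the attack radius.
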(event Custom|Fire
  (for _array_element (Collision|GetOverlappingActors (Variables|Default|GetBox) "/Game/BP/AI/BP_Enemy.BP_Enemy_C" :!class /Script/Engine.PrimitiveComponent)
    (Game|Damage|ApplyDamage _array_element (Variables|Default|GetBase%20Damage) 0 0)))

(event EventBeginPlay
  (|CallParentFunction) ; 此节点被禁用，将不会被调用。\n从引脚连出引线来编译功能。
)

(event Collision|EventActorBeginOverlap
  (params (OtherActor :type Actor%20Object%20Reference))
  (|CallParentFunction OtherActor) ; 此节点被禁用，将不会被调用。\n从引脚连出引线来编译功能。
)

(event EventTick
  (params (DeltaSeconds :type Float%20%28single-precision%29))
  ;[1 1 1] Fire
  (|CallParentFunction DeltaSeconds)
  (CallFunction|FacingTarget))

(event EventFindTarget
  ;[1 1 1] Fire
  (if (not (Variables|Default|GetAttacking))
    (Variables|Default|SetAttacking true)
    (Components|Activation|Activate (Variables|Default|GetFX_Flame) true)
    (bind _returnvalue (Utilities|Time|SetTimerbyFunctionName 0 "Fire" (Variables|Default|GetInterval) true))
    (Variables|Default|SetFiredTimer _returnvalue)))

(event EventNOTarget
  ;[1 1 1] Fire
  (Variables|Default|SetAttacking false)
  (Utilities|Time|ClearandInvalidateTimerbyHandle (Variables|Default|GetFiredTimer))
  (Components|Activation|SetActive (Variables|Default|GetFX_Flame) false false))

(fn ConstructionScript
  (bind _box (Variables|Default|GetBox))
  (bind _mattackradius (Variables|Default|GetmAttackRadius))
  (bind _returnvalue (* _mattackradius 0.5))
  (|CallParentFunction)
  (Components|Box|SetBoxExtent _box (Math|Vector|MakeVector _returnvalue 1e+02 1e+02) true)
  (Transformation|SetRelativeLocation _box (Math|Vector|MakeVector (- _returnvalue 1e+02) 0.0 0.0) false false))

(fn FacingTarget
  (bind _m_fort2 (Variables|Default|GetM_Fort2))
  (bind _m_fort3 (Variables|Default|GetM_Fort3))
  (bind _returnvalue (Transformation|GetWorldRotation _m_fort3))
  (bind _returnvalue_2 (Transformation|GetWorldRotation _m_fort2))
  (bind _currenttarget (Variables|Default|GetCurrentTarget)
    (:then
      (Utilities|FlowControl|Sequence
        (:then_0
          (Transformation|SetWorldRotation _m_fort3 (Math|Rotator|MakeRotator (.roll _returnvalue) (.pitch (Math|Interpolation|RInterpTo (Transformation|GetWorldRotation _m_fort3) (Math|Rotator|FindLookatRotation (Transformation|GetWorldLocation (Variables|Default|GetM_Fort3)) (Transformation|GetActorLocation _currenttarget)) (Utilities|Time|GetWorldDeltaSeconds) 5.0)) (.yaw _returnvalue)) false false))
        (:then_1
          (Transformation|SetWorldRotation _m_fort2 (Math|Rotator|MakeRotator (.roll _returnvalue_2) (.pitch _returnvalue_2) (.yaw (Math|Interpolation|RInterpTo (Transformation|GetWorldRotation _m_fort2) (Math|Rotator|FindLookatRotation (Transformation|GetWorldLocation (Variables|Default|GetM_Fort3)) (Transformation|GetActorLocation _currenttarget)) (Utilities|Time|GetWorldDeltaSeconds) 5.0))) false false))))
    (:else)))