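; Electric auto-weapon tower that, on each Fire event, launches a BP_Lightning projectile at several of the nearest targets at once.
; Fire calls ClosestTargets with MaxNum, then spawns one projectile per selected target from the Arrow's location.
; ClosestTargets copies Targets into a working list, then repeatedly takes the actor nearest the tower and removes it, yielding distinct targets in nearest-first order.
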(event EventFire
  ;[1 1 1] Fire
  (CallFunction|ClosestTargets (Variables|Default|GetMaxNum))
  (for _array_element (Variables|Default|GetRecenttargets)
    (Class|Turret|SpawnProjectile "/Game/Assets/AutomaticWeapons/Blueprints/BP_Lightning.BP_Lightning_C" (Transformation|GetWorldLocation (Variables|Default|GetArrow)) "0, 0, 0" _array_element)))

(fn ConstructionScript
  (|CallParentFunction))

(fn ClosestTargets
  (params (LastIndex :type Integer))
  (Utilities|Array|Clear (Variables|Default|GetRecenttargets))
  (LocalVariables|SetTargetDistance (Variables|Default|GetTargets))
  (for _index (range 1 LastIndex)
    (Utilities|IsValid (.ReturnValue (Actor|FindNearestActor (Transformation|GetActorLocation) (LocalVariables|GetTargetDistance)))
      (:Is%20Valid
        (Utilities|Array|Add (Variables|Default|GetRecenttargets) (.ReturnValue (Actor|FindNearestActor (Transformation|GetActorLocation) (LocalVariables|GetTargetDistance))))
        (Utilities|Array|RemoveItem (LocalVariables|GetTargetDistance) (.ReturnValue (Actor|FindNearestActor (Transformation|GetActorLocation) (LocalVariables|GetTargetDistance))))))))