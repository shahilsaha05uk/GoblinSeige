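; Parent cannon building that fires on a target, with empty start/stop projectile events.
; Fire keeps a valid target or stops the projectile and calls FindTarget, then aims, starts the projectile and applies full radial damage around the Arrow using the building's AttackDamage.
; Aiming interpolates yaw on MFort2 and pitch on MFort3 separately.
; The construction script only calls its parent; range-box sizing is disconnected.
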(event Custom|StartCannonProjectile)

(event Custom|StopCannonProjectile)

(event EventLookatTarget
  (bind _m_fort2 (Variables|Default|GetM_Fort2))
  (bind _m_fort3 (Variables|Default|GetM_Fort3))
  (bind _returnvalue (Transformation|GetWorldRotation _m_fort3))
  (bind _returnvalue_2 (Transformation|GetWorldRotation _m_fort2))
  (bind _currenttarget (Variables|Default|GetCurrentTarget)
    (:then
      (Utilities|FlowControl|Sequence
        (:then_0
          (Transformation|SetWorldRotation _m_fort3 (Math|Rotator|MakeRotator (.roll _returnvalue) (.pitch (Math|Interpolation|RInterpTo (Transformation|GetWorldRotation _m_fort3) (Math|Rotator|FindLookatRotation (Transformation|GetWorldLocation (Variables|Default|GetM_Fort3)) (Transformation|GetActorLocation _currenttarget)) (Utilities|Time|GetWorldDeltaSeconds) 5.0)) (.yaw _returnvalue)) false false))
        (:then_1
          (Transformation|SetWorldRotation _m_fort2 (Math|Rotator|MakeRotator (.roll _returnvalue_2) (.pitch _returnvalue_2) (.yaw (Math|Interpolation|RInterpTo (Transformation|GetWorldRotation _m_fort2) (Math|Rotator|FindLookatRotation (Transformation|GetWorldLocation (Variables|Default|GetM_Fort3)) (Transformation|GetActorLocation _currenttarget)) (Utilities|Time|GetWorldDeltaSeconds) 5.0))) false false))))
    (:else)))

(event EventFire
  (Variables|Default|GetCurrentTarget
    (:then
      _)
    (:else
      (CallFunction|StopCannonProjectile)
      (bind _returnvalue (Class|Turret|FindTarget))
      (bind _output_get (Variables|Default|SetCurrentTarget _returnvalue))
      (Utilities|IsValid _output_get
        (:Is%20Valid
          _))))
  (Class|Turret|LookatTarget)
  (CallFunction|StartCannonProjectile)
  (Game|Damage|ApplyRadialDamage (.AttackDamage (Utilities|Struct|BreakBuildingStats (Utilities|Struct|BreakBuildingDetails (Variables|Default|GetBuildingDetails)))) (Transformation|GetWorldLocation (Variables|Default|GetArrow)) 2e+03 0 0 0 0 true "ECC_Visibility"))

(fn ConstructionScript
  (|CallParentFunction))