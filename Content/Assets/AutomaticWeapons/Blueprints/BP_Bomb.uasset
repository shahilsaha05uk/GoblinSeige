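; BP_Bomb is a projectile bomb that explodes on impact and damages actors within a radius.
; The construction script sets the projectile movement's initial speed from LaunchSpeed.
; On Hit, it spawns a scaled-up explosion effect at the impact point, applies radial damage around itself, then destroys itself.
; Damage has no distance falloff and is prevented by obstructions on the Pawn trace channel.
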(event EventBeginPlay)

(event Collision|EventActorBeginOverlap
  (params (OtherActor :type Actor%20Object%20Reference)))

(event EventTick
  (params (DeltaSeconds :type Float%20%28single-precision%29)))

(event Collision|EventHit
  (params (MyComp :type Primitive%20Component%20Object%20Reference) (Other :type Actor%20Object%20Reference) (OtherComp :type Primitive%20Component%20Object%20Reference) (bSelfMoved :type Boolean) (HitLocation :type Vector :default "0, 0, 0") (HitNormal :type Vector :default "0, 0, 0") (NormalImpulse :type Vector :default "0, 0, 0") (Hit :type Hit%20Result%20Structure%20%28by%20ref%29))
  (Niagara|SpawnSystematLocation "/Game/Assets/AutomaticWeapons/Particles/FX_Explode.FX_Explode" HitLocation "0, 0, 0" "5.000000,5.000000,5.000000")
  (Game|Damage|ApplyRadialDamage (Variables|Default|GetBase%20Damage) (Transformation|GetActorLocation) (Variables|Default|GetDamage%20Radius) 0 0 self 0 true "ECC_Pawn") ; 可视性遮挡则无伤害
  (Actor|DestroyActor))

(fn ConstructionScript
  (Variables|/Script/Engine.ProjectileMovementComponent|SetInitialSpeed (Variables|Default|GetProjectileMovement) (Variables|Default|GetLaunch%20speed)))