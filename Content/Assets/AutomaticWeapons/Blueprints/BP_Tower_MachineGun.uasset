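; Machine gun tower Blueprint that tracks the closest target and repeatedly fires bullets at it.
; Each tick, it smoothly rotates toward the target, splitting yaw and pitch between two mesh parts.
; FindTarget and NOTarget open and close a gate on Tick, where a Delay paces bullet spawns from the arrow component, passing along base damage.
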(event EventTick
  (params (DeltaSeconds :type Float%20%28single-precision%29))
  (bind _arrow (Variables|Default|GetArrow))
  (bind _returnvalue (Transformation|GetWorldTransform _arrow))
  ;[1 1 1] Fire
  (|CallParentFunction DeltaSeconds)
  (CallFunction|FacingTarget)
  (Utilities|FlowControl|Gate true
    (:Exit
      (Utilities|FlowControl|Delay (Variables|Default|GetInterval))
      (Game|SpawnActorfromClass "/Game/Assets/AutomaticWeapons/Blueprints/BP_Bullet.BP_Bullet_C" (Math|Transform|MakeTransform (.location _returnvalue) (.rotation _returnvalue) "1.000000,1.000000,1.000000") "Undefined" "OverrideRootScale" 0 (Variables|Default|GetBase%20Damage) 0))))

(event EventFindTarget
  (bind _arrow (Variables|Default|GetArrow))
  (bind _returnvalue (Transformation|GetWorldTransform _arrow))
  ;[1 1 1] Fire
  (if (not (Variables|Default|GetAttacking))
    (Variables|Default|SetAttacking true)
    (Utilities|FlowControl|Gate true) ; enters at Open
  ))

(event EventNOTarget
  (bind _arrow (Variables|Default|GetArrow))
  (bind _returnvalue (Transformation|GetWorldTransform _arrow))
  ;[1 1 1] Fire
  (Variables|Default|SetAttacking false)
  (Utilities|FlowControl|Gate true) ; enters at Close
)

(fn ConstructionScript
  (|CallParentFunction))

(fn FacingTarget
  (bind _m_fort2 (Variables|Default|GetM_Fort2))
  (bind _m_fort3 (Variables|Default|GetM_Fort3))
  (bind _returnvalue (Transformation|GetWorldRotation _m_fort3))
  (bind _returnvalue_2 (Transformation|GetWorldRotation _m_fort2))
  (bind _closesttarget (Variables|Default|GetClosestTarget)
    (:then
      (Utilities|FlowControl|Sequence
        (:then_0
          (Transformation|SetWorldRotation _m_fort3 (Math|Rotator|MakeRotator (.roll _returnvalue) (.pitch (Math|Interpolation|RInterpTo (Transformation|GetWorldRotation _m_fort3) (Math|Rotator|FindLookatRotation (Transformation|GetWorldLocation (Variables|Default|GetM_Fort3)) (Transformation|GetActorLocation _closesttarget)) (Utilities|Time|GetWorldDeltaSeconds) 1e+01)) (.yaw _returnvalue)) false false))
        (:then_1
          (Transformation|SetWorldRotation _m_fort2 (Math|Rotator|MakeRotator (.roll _returnvalue_2) (.pitch _returnvalue_2) (.yaw (Math|Interpolation|RInterpTo (Transformation|GetWorldRotation _m_fort2) (Math|Rotator|FindLookatRotation (Transformation|GetWorldLocation (Variables|Default|GetM_Fort3)) (Transformation|GetActorLocation _closesttarget)) (Utilities|Time|GetWorldDeltaSeconds) 1e+01))) false false))))
    (:else)))