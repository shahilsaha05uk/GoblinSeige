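; BP_Arrow is a homing arrow projectile that damages enemies and sticks into them.
; Each tick, while its target is a living EnemyInterface actor, it interpolates velocity toward a point slightly above the target's origin and raises its speed.
; Hitting a BP_Enemy applies damage, attaches the arrow to the closest physics-asset bone and stops it until the target becomes invalid.
; Other hits destroy it after a short delay.
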(event EventBeginPlay)

(event EventTick
  (params (DeltaSeconds :type Float%20%28single-precision%29))
  (bind _targetactor (Variables|Default|GetTargetActor))
  (if (and (Utilities|IsValid _targetactor) (Utilities|DoesObjectImplementInterface _targetactor "/Script/TowerDefenceGame.EnemyInterface"))
    (bind _value (Class|BIEnemyInterface|IsDead(Message) (Variables|Default|GetTargetActor)))
    (if (not _value)
      (Variables|/Script/Engine.MovementComponent|SetVelocity (Variables|Default|GetProjectileMovement) (CallFunction|TracktheTarget))
      (Variables|Default|SetLaunch%20speed (+ (Variables|Default|GetLaunch%20speed) 1e+02)))
    (elif (Variables|Default|GetHit)
      (Actor|DestroyActor))))

(event Collision|EventHit
  (params (MyComp :type Primitive%20Component%20Object%20Reference) (Other :type Actor%20Object%20Reference) (OtherComp :type Primitive%20Component%20Object%20Reference) (bSelfMoved :type Boolean) (HitLocation :type Vector :default "0, 0, 0") (HitNormal :type Vector :default "0, 0, 0") (NormalImpulse :type Vector :default "0, 0, 0") (Hit :type Hit%20Result%20Structure%20%28by%20ref%29))
  ;[1 1 1] Hit
  (bind _asbp_enemy (Utilities|Casting|CastToBP_Enemy Other)
    (:then
      (Variables|Default|SetHit true)
      (Transformation|AttachComponentToComponent (Variables|/Script/Engine.Character|GetMesh _asbp_enemy) (.BoneName (Class|SkeletalMeshComponent|GetClosestPointonPhysicsAsset (Variables|/Script/Engine.Character|GetMesh _asbp_enemy) HitLocation)) "KeepWorld" "KeepWorld" "KeepRelative" false)
      (Game|Damage|ApplyDamage _asbp_enemy (Variables|Default|GetBase%20Damage) 0 self)
      (Collision|SetCollisionEnabled (Variables|Default|GetSphere) "NoCollision")
      (Components|Activation|Deactivate (Variables|Default|GetProjectileMovement)))
    (:CastFailed
      (Utilities|FlowControl|Delay 1.0)
      (Actor|DestroyActor))))

(fn ConstructionScript
  (Variables|/Script/Engine.ProjectileMovementComponent|SetInitialSpeed (Variables|Default|GetProjectileMovement) (Variables|Default|GetLaunch%20speed)))

(fn TracktheTarget
  (return (Math|Interpolation|VInterpTo (Variables|/Script/Engine.MovementComponent|GetVelocity (Variables|Default|GetProjectileMovement)) (* (Math|Vector|GetUnitDirection(Vector) (Transformation|GetActorLocation) (+ (Transformation|GetActorLocation (Variables|Default|GetTargetActor)) "0.000000,0.000000,30.000000")) (Variables|Default|GetLaunch%20speed)) (Utilities|Time|GetWorldDeltaSeconds) 15.0)))