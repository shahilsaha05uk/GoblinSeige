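; Machine-gun tower Blueprint that aims at a target and fires BP_Bullet projectiles from its Arrow component.
; Power-on starts a looping AttackSpeed timer that validates CurrentTarget, calls FindTarget if it is dead, and spawns a bullet when a dot-product alignment check passes.
; FacingTarget interpolates yaw on MFort2 and pitch on MFort3 toward ClosestTarget (not CurrentTarget), stepping only on each timer fire.
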(event EventNOTarget
  (Variables|Default|SetAttacking false))

(event EventPoweron
  (bind _returnvalue (Utilities|Time|SetTimerbyEvent (delegate EventFire) (Variables|Default|GetAttackSpeed) true))
  (Variables|Default|SetFireHandler _returnvalue))

(event EventFire
  (bind _arrow (Variables|Default|GetArrow))
  (bind _returnvalue (Transformation|GetWorldTransform _arrow))
  (bind _currenttarget (Variables|Default|GetCurrentTarget)
    (:then
      (bind _value (Class|BIEnemyInterface|IsDead(Message) _currenttarget))
      (if _value
        (bind _returnvalue_2 (Class|Turret|FindTarget))
        (bind _output_get (Variables|Default|SetCurrentTarget _returnvalue_2))
        (Utilities|IsValid _output_get
          (:Is%20Valid
            (CallFunction|FacingTarget)
            (Variables|Default|SetAttacking true)))
        (else
          (CallFunction|FacingTarget)))
      (if (<= (Class|HelperMethods|GetDotProductBetweenComponentWorldLocationandActorLocation (Variables|Default|GetM_Fort3) (Variables|Default|GetCurrentTarget)) 0.1)
        (Class|Turret|SpawnProjectile "/Game/AutomaticWeapons/Blueprints/BP_Bullet.BP_Bullet_C" (.location _returnvalue) (.rotation _returnvalue) 0)))
    (:else)))

(fn ConstructionScript
  (|CallParentFunction))

(fn FacingTarget
  (bind _m_fort2 (Variables|Default|GetM_Fort2))
  (bind _m_fort3 (Variables|Default|GetM_Fort3))
  (bind _returnvalue (Transformation|GetWorldRotation _m_fort2))
  (bind _returnvalue_2 (Transformation|GetWorldRotation _m_fort3))
  (bind _closesttarget (Variables|Default|GetClosestTarget)
    (:then
      (Utilities|FlowControl|Sequence
        (:then_0
          (Transformation|SetWorldRotation _m_fort3 (Math|Rotator|MakeRotator (.roll _returnvalue_2) (.pitch (Math|Interpolation|RInterpTo (Transformation|GetWorldRotation _m_fort3) (Math|Rotator|FindLookatRotation (Transformation|GetWorldLocation (Variables|Default|GetM_Fort3)) (Transformation|GetActorLocation _closesttarget)) (Utilities|Time|GetWorldDeltaSeconds) 1e+01)) (.yaw _returnvalue_2)) false false))
        (:then_1
          (Transformation|SetWorldRotation _m_fort2 (Math|Rotator|MakeRotator (.roll _returnvalue) (.pitch _returnvalue) (.yaw (Math|Interpolation|RInterpTo (Transformation|GetWorldRotation _m_fort2) (Math|Rotator|FindLookatRotation (Transformation|GetWorldLocation (Variables|Default|GetM_Fort3)) (Transformation|GetActorLocation _closesttarget)) (Utilities|Time|GetWorldDeltaSeconds) 1e+01))) false false))))
    (:else)))