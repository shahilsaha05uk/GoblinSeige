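; BP_Tower is an automatic weapon tower that shows its attack range and fires projectiles at targets.
; IncreaseRange sizes the range collision sphere and scales a range decal to match AttackRange, and runs from the construction script.
; SpawnProjectile spawns the configured projectile class with damage, radius, launch speed and target, falling back to CurrentTarget when the given target is invalid.
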(event EventIncreaseRange
  (bind _attackrange (Variables|Default|GetAttackRange))
  (bind _returnvalue (/ _attackrange 1e+02))
  (Components|Sphere|SetSphereRadius (Variables|Default|GetRangeCollisionComp) _attackrange true)
  (Transformation|SetRelativeScale3D (Variables|Default|GetRangeDecalComp) (Math|Vector|MakeVector 1.0 _returnvalue _returnvalue)))

(event EventSpawnProjectile
  (params (ProjectileClass :type Projectile%20Class%20Reference) (Location :type Vector :default "0, 0, 0") (Rotation :type Rotator :default "0, 0, 0") (Target :type Actor%20Object%20Reference))
  (Utilities|IsValid Target
    (:Is%20Valid
      (Variables|Default|SettmpTarget Target))
    (:Is%20Not%20Valid
      (Variables|Default|SettmpTarget (Variables|Default|GetCurrentTarget))))
  (Game|SpawnActorfromClass (Variables|Default|GetmProjectileClass) (Math|Transform|MakeTransform Location Rotation "1.000000,1.000000,1.000000") "Undefined" "MultiplyWithRoot" self (Variables|Default|GetAttackDamage) (Variables|Default|GetDamageRadius) (Variables|Default|GetTargetLocation) (Variables|Default|GetLaunchSpeed) (Variables|Default|GettmpTarget) 0))

(fn ConstructionScript
  (Class|Turret|IncreaseRange))

(fn GetArrowWorldTransform
  (return ""))