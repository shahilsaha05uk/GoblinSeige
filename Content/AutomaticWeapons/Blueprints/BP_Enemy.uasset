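; BP_Enemy is a simple enemy character that walks continuously along its forward vector every tick and can be killed by damage.
; Any damage reduces HP; at zero or below it sets a death flag, switches the capsule to a "death" collision profile and ragdolls the mesh through physics simulation.
; It then calls Spwan on its Generator reference and destroys itself after a short delay.
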(event EventBeginPlay)

(event Collision|EventActorBeginOverlap
  (params (OtherActor :type Actor%20Object%20Reference)))

(event EventTick
  (params (DeltaSeconds :type Float%20%28single-precision%29))
  (Pawn|Input|AddMovementInput (Transformation|GetActorForwardVector) 1.0 false))

(event Game|Damage|EventAnyDamage
  (params (Damage :type Float%20%28single-precision%29) (DamageType :type Damage%20Type%20Object%20Reference) (InstigatedBy :type Controller%20Object%20Reference) (DamageCauser :type Actor%20Object%20Reference))
  ;[1 1 1] Damage&Death
  (bind _output_get (Variables|Default|SetHP (- (Variables|Default|GetHP) Damage)))
  (if (<= _output_get 0.0)
    (Variables|Default|SetDeath true)
    (Collision|SetCollisionProfileName (Variables|Collision|GetCapsuleComponent) "death" true :!class /Script/Engine.PrimitiveComponent)
    (Physics|SetSimulatePhysics (Variables|Character|GetMesh) true)
    (Default|Spwan (Variables|Default|GetGenerator))
    (Utilities|FlowControl|Delay 1.0)
    (Actor|DestroyActor)))

(fn ConstructionScript)