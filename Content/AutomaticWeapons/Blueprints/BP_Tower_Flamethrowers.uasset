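; Flamethrower tower Blueprint that burns enemies, building on a parent class's targeting and setup.
; Fire switches off the flame and retargets if the current target is dead, then aims, activates the flame and damages every BP_Enemy overlapping its box.
; LookatTarget smoothly interpolates yaw on MFort2 and pitch on MFort3 toward the target.
; Construction code sizing the damage box from AttackRange is disconnected and never runs.
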(event EventLookatTarget
  (bind _m_fort2 (Variables|Default|GetM_Fort2))
  (bind _m_fort3 (Variables|Default|GetM_Fort3))
  (bind _returnvalue (Transformation|GetWorldRotation _m_fort3))
  (bind _returnvalue_2 (Transformation|GetWorldRotation _m_fort2))
  (bind _currenttarget (Variables|Default|GetCurrentTarget)
    (:then
      (Utilities|FlowControl|Sequence
        (:then_0
          (Transformation|SetWorldRotation _m_fort3 (Math|Rotator|MakeRotator (.roll _returnvalue) (.pitch (Math|Interpolation|RInterpTo (Transformation|GetWorldRotation _m_fort3) (Math|Rotator|FindLookatRotation (Transformation|GetWorldLocation (Variables|Default|GetM_Fort3)) (Transformation|GetActorLocation _currenttarget)) (Utilities|Time|GetWorldDeltaSeconds) 5.0)) (.yaw _returnvalue)) false false))
        (:then_1
          (Transformation|SetWorldRotation _m_fort2 (Math|Rotator|MakeRotator (.roll _returnvalue_2) (.pitch _returnvalue_2) (.yaw (Math|Interpolation|RInterpTo (Transformation|GetWorldRotation _m_fort2) (Math|Rotator|FindLookatRotation (Transformation|GetWorldLocation (Variables|Default|GetM_Fort3)) (Transformation|GetActorLocation _currenttarget)) (Utilities|Time|GetWorldDeltaSeconds) 5.0))) false false))))
    (:else)))

(event EventFire
  (bind _currenttarget (Variables|Default|GetCurrentTarget)
    (:then
      (bind _value (Class|BIEnemyInterface|IsDead(Message) _currenttarget))
      (if _value
        (Components|Activation|SetActive (Variables|Default|GetFX_Flame) false false)
        (bind _returnvalue (Class|Turret|FindTarget))
        (bind _output_get (Variables|Default|SetCurrentTarget _returnvalue))
        (Utilities|IsValid _output_get
          (:Is%20Valid
            (Variables|Default|SetAttacking true))))
      (Class|Turret|LookatTarget)
      (Components|Activation|Activate (Variables|Default|GetFX_Flame) true)
      (for _array_element (Collision|GetOverlappingActors (Variables|Default|GetBox) "/Game/BP/AI/BP_Enemy.BP_Enemy_C" :!class /Script/Engine.PrimitiveComponent)
        (Game|Damage|ApplyDamage _array_element (Variables|Default|GetAttackDamage) 0 self)))
    (:else)))

(fn ConstructionScript
  (|CallParentFunction))