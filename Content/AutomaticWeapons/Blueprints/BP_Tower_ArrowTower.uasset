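; Arrow tower, an automatic weapon that fires BP_Arrow projectiles at its current target.
; Powering on starts a looping Fire timer at the AttackSpeed interval, which is cleared when no target is in range.
; Each tick of that timer rotates the Arrow component toward a living target and spawns a projectile from it.
; If the target is dead, it finds and aims at a new one without firing that cycle.
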(event EventPoweron
  (bind _returnvalue (Utilities|Time|SetTimerbyFunctionName 0 "Fire" (Variables|Default|GetAttackSpeed) true))
  (Variables|Default|SetFiredTimer _returnvalue))

(event EventFire
  (bind _arrow (Variables|Default|GetArrow))
  (bind _returnvalue (Transformation|GetWorldTransform _arrow))
  (bind _currenttarget (Variables|Default|GetCurrentTarget)
    (:then
      (bind _value (Class|BIEnemyInterface|IsDead(Message) _currenttarget))
      (if _value
        (bind _returnvalue_2 (Class|Turret|FindTarget))
        (bind _output_get (Variables|Default|SetCurrentTarget _returnvalue_2))
        (Utilities|IsValid _output_get
          (:Is%20Valid
            (CallFunction|AimedattheTarget)
            (Variables|Default|SetAttacking true)))
        (else
          (CallFunction|AimedattheTarget)
          (Class|Turret|SpawnProjectile "/Game/AutomaticWeapons/Blueprints/BP_Arrow.BP_Arrow_C" (.location _returnvalue) (.rotation _returnvalue) 0))))
    (:else)))

(event EventOnNoTargetinRange
  (Variables|Default|SetAttacking false)
  (Utilities|Time|ClearandInvalidateTimerbyHandle (Variables|Default|GetFiredTimer)))

(fn ConstructionScript
  (|CallParentFunction))

(fn AimedattheTarget
  (bind _arrow (Variables|Default|GetArrow))
  (bind _currenttarget (Variables|Default|GetCurrentTarget))
  (Utilities|IsValid _currenttarget
    (:Is%20Valid
      (Transformation|SetWorldRotation _arrow (Math|Rotator|FindLookatRotation (Transformation|GetWorldLocation _arrow) (Transformation|GetActorLocation _currenttarget)) false false))))