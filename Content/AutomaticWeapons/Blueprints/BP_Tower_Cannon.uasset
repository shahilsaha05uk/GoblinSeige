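; Cannon variant of an automatic tower that finds a living target, aims at it and fires projectiles.
; Fire replaces invalid or dead targets, waits an aim delay derived from the remaining yaw, then spawns a projectile at the arrow and starts a cooldown.
; LookatTarget smoothly yaws MFort2 and pitches MFort3 along a suggested ballistic arc toward the target's feet until yaw aligns.
; FacingTarget is empty here.
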(event EventLookatTarget
  (bind _currenttarget (Variables|Default|GetCurrentTarget))
  (bind _m_fort3 (Variables|Default|GetM_Fort3))
  (bind _m_fort3_2 (Variables|Default|GetM_Fort3))
  (bind _m_fort2 (Variables|Default|GetM_Fort2))
  (bind _returnvalue (Transformation|GetWorldLocation _m_fort3_2))
  (bind _returnvalue_2 (Transformation|GetWorldRotation _m_fort3))
  (bind _returnvalue_3 (Transformation|GetWorldRotation _m_fort2))
  (bind _returnvalue_4 (Transformation|GetActorLocation _currenttarget))
  (bind _returnvalue_5 (Math|Rotator|FindLookatRotation _returnvalue _returnvalue_4))
  (if (not (Variables|Default|GetbTargetSet))
    (Variables|Default|GetCurrentTarget
      (:then
        (Utilities|FlowControl|Sequence
          (:then_0
            (bind _tossvelocity (Class|GameplayStatics|BlueprintSuggestProjectileVelocity (Transformation|GetWorldLocation (Variables|Default|GetArrow)) (- (Transformation|GetActorLocation (Variables|Default|GetCurrentTarget)) "0.000000,0.000000,80.000000") (Variables|Default|GetLaunch%20Speed) 0.0 "DoNotTrace" 1.0 false false))
            (Transformation|SetWorldRotation _m_fort3 (Math|Rotator|MakeRotator (.roll _returnvalue_2) (.pitch (Math|Interpolation|RInterpTo (Transformation|GetWorldRotation _m_fort3) (Math|Conversions|RotationFromXVector _tossvelocity) (Utilities|Time|GetWorldDeltaSeconds) 5.0)) (.yaw _returnvalue_2)) false false))
          (:then_1
            (Transformation|SetWorldRotation _m_fort2 (Math|Rotator|MakeRotator (.roll _returnvalue_3) (.pitch _returnvalue_3) (.yaw (Math|Interpolation|RInterpTo (Transformation|GetWorldRotation _m_fort2) _returnvalue_5 (Utilities|Time|GetWorldDeltaSeconds) 5.0))) false false)
            (Variables|Default|SetbTargetSet (<= (Math|Float|Absolute(Float) (.yaw (Math|Rotator|Delta(Rotator) _returnvalue_5 (Transformation|GetWorldRotation (Variables|Default|GetM_Fort2))))) 0.2)))))
      (:else))))

(event EventFire
  (bind _arrow (Variables|Default|GetArrow))
  (bind _returnvalue (Transformation|GetWorldTransform _arrow))
  (bind _currenttarget (Variables|Default|GetCurrentTarget)
    (:then
      (bind _value (Class|BIEnemyInterface|IsDead(Message) _currenttarget))
      (if _value
        (bind _returnvalue_2 (Class|Turret|FindTarget :!label _label))
        (bind _output_get (Variables|Default|SetCurrentTarget _returnvalue_2))
        (Utilities|IsValid _output_get
          (:Is%20Valid
            (CallFunction|FacingTarget)
            (Variables|Default|SetAttacking true)))
        (else
          (CallFunction|FacingTarget))))
    (:else
      (goto _label)))
  (Variables|Default|SetAimingTime (CallFunction|CalculatetheAimingTime))
  (Utilities|FlowControl|Delay (Variables|Default|GetAimingTime))
  (if (Variables|Default|GetReady)
    (Class|Turret|SpawnProjectile 0 (.location _returnvalue) (.rotation _returnvalue) 0)
    (Variables|Default|SetReady false)
    (Utilities|FlowControl|Delay 1.0)
    (Variables|Default|SetReady true)
    (if (Variables|Default|GetAttacking)
      (Variables|Default|SetbTargetSet false))))

(fn ConstructionScript
  (|CallParentFunction))

(fn FacingTarget)

(fn CalculatetheAimingTime
  (bind _currenttarget (Variables|Default|GetCurrentTarget)
    (:then
      (return (/ (Math|Float|Absolute(Float) (.yaw (Math|Rotator|Delta(Rotator) (Math|Rotator|FindLookatRotation (Transformation|GetWorldLocation (Variables|Default|GetM_Fort3)) (Transformation|GetActorLocation _currenttarget)) (Transformation|GetWorldRotation (Variables|Default|GetM_Fort2))))) 1.5e+02)))
    (:else)))