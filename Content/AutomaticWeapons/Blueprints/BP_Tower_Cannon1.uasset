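; Cannon tower Blueprint that turns toward its current target and fires arcing projectiles from its Arrow component.
; LookatTarget smoothly yaws MFort2 toward the target and pitches MFort3 along a suggested projectile toss velocity aimed near the target's feet.
; Aiming stops once TargetSet is true, which depends only on yaw falling within a small tolerance.
; StartCannonProjectile spawns the configured projectile class at the Arrow transform, passing it the current target.
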(event EventStartCannonProjectile
  (bind _arrow (Variables|Default|GetArrow))
  (bind _returnvalue (Transformation|GetWorldTransform _arrow))
  (Class|Turret|SpawnProjectile (Variables|Default|GetmProjectileClass) (.location _returnvalue) (.rotation _returnvalue) (Variables|Default|GetCurrentTarget)))

(event EventLookatTarget
  (bind _currenttarget (Variables|Default|GetCurrentTarget))
  (bind _m_fort3 (Variables|Default|GetM_Fort3))
  (bind _m_fort2 (Variables|Default|GetM_Fort2))
  (bind _m_fort3_2 (Variables|Default|GetM_Fort3))
  (bind _returnvalue (Transformation|GetWorldLocation _m_fort3))
  (bind _returnvalue_2 (Transformation|GetWorldRotation _m_fort3_2))
  (bind _returnvalue_3 (Transformation|GetWorldRotation _m_fort2))
  (bind _returnvalue_4 (Transformation|GetActorLocation _currenttarget))
  (bind _returnvalue_5 (Math|Rotator|FindLookatRotation _returnvalue _returnvalue_4))
  (if (not (Variables|Default|GetbTargetSet))
    (Variables|Default|GetCurrentTarget
      (:then
        (Utilities|FlowControl|Sequence
          (:then_0
            (bind _tossvelocity (Class|GameplayStatics|BlueprintSuggestProjectileVelocity (Transformation|GetWorldLocation (Variables|Default|GetArrow)) (- (Transformation|GetActorLocation (Variables|Default|GetCurrentTarget)) "0.000000,0.000000,80.000000") (Variables|Default|GetLaunch%20Speed) 0.0 "DoNotTrace" 1.0 false false))
            (Transformation|SetWorldRotation _m_fort3_2 (Math|Rotator|MakeRotator (.roll _returnvalue_2) (.pitch (Math|Interpolation|RInterpTo (Transformation|GetWorldRotation _m_fort3_2) (Math|Conversions|RotationFromXVector _tossvelocity) (Utilities|Time|GetWorldDeltaSeconds) 5.0)) (.yaw _returnvalue_2)) false false))
          (:then_1
            (Transformation|SetWorldRotation _m_fort2 (Math|Rotator|MakeRotator (.roll _returnvalue_3) (.pitch _returnvalue_3) (.yaw (Math|Interpolation|RInterpTo (Transformation|GetWorldRotation _m_fort2) _returnvalue_5 (Utilities|Time|GetWorldDeltaSeconds) 5.0))) false false)
            (Variables|Default|SetbTargetSet (<= (Math|Float|Absolute(Float) (.yaw (Math|Rotator|Delta(Rotator) _returnvalue_5 (Transformation|GetWorldRotation (Variables|Default|GetM_Fort2))))) 0.2)))))
      (:else))))

(fn ConstructionScript
  (|CallParentFunction))