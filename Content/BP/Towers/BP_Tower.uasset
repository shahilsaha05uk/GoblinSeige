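; BP_Tower is a tower Blueprint that supplies projectile spawning, pooling reset and upgrade effects.
; SpawnProjectile spawns the configured projectile class at SpawnPoint when a target is valid, passing it the target and damage from the building stats.
; When a projectile finishes its job, it is moved back to SpawnPoint and hidden rather than destroyed.
; Upgrade calls the parent logic, then activates a Niagara effect.
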(event EventUpgrade
  (params (Details :type Upgrade%20Details%20Structure))
  (|CallParentFunction Details)
  (Components|Activation|Activate (Variables|Default|GetmNiagaraUpgradeComp) false))

(event EventOnProjectileJobComplete
  (params (Projectile :type Projectile%20Object%20Reference))
  (Transformation|SetActorLocation Projectile (Transformation|GetWorldLocation (Variables|Default|GetSpawnPoint)) false false)
  (Rendering|SetActorHiddenInGame Projectile true))

(fn ConstructionScript)

(fn SpawnProjectile
  (bind _mtarget (Variables|Default|GetmTarget))
  (Utilities|IsValid _mtarget
    (:Is%20Valid
      (bind _returnvalue (Game|SpawnActorfromClass (Variables|Default|GetProjectileClass) (Transformation|GetWorldTransform (Variables|Default|GetSpawnPoint)) "Undefined" "SelectDefaultAtRuntime" 0 (Utilities|Struct|BreakBuildingStats (Variables|Default|GetBuildingStats)) "0.000000,0.000000,0.000000" _mtarget 0))
      (return _returnvalue))))