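; Player controller that sets game-and-UI input mode on begin play and handles toggling the pause menu.
; Its PauseGame event flips an IsPaused flag and sets the game's paused state to match.
; The HUD supplies the MENU widget, which the controller adds to the viewport on pause and asks the HUD to destroy on unpause.
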(event EventBeginPlay
  (Input|SetInputModeGameandUI self 0 "DoNotLock" true false))

(event EventPauseGame
  (if (not (Variables|Default|GetbIsPaused))
    (bind _returnvalue (Class|HUDInterface|WidgetInitialiser(Message) (HUD|GetHUD) "PAUSE_MENU"))
    (UserInterface|Viewport|AddtoViewport _returnvalue 0)
    (Variables|Default|SetbIsPaused true)
    (Game|SetGamePaused true)
    (else
      (Class|HUDInterface|DestroyWidget(Message) (HUD|GetHUD) "PAUSE_MENU")
      (Variables|Default|SetbIsPaused false)
      (Game|SetGamePaused false))))

(fn ConstructionScript)