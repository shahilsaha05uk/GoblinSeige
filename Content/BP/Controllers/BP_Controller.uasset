(event Custom|Call_LoadNextPhase
  (bind _asbp_game_mode (Utilities|Casting|CastToBP_GameMode (Game|GetGameMode)))
  (Class|TowerDefenceGameGameModeBase|OnPhaseLoad _asbp_game_mode))

(event Custom|OnPlaybackComplete
  ;[0 0 0] When the media playback  completes, call the phase load
  (CallFunction|CallLoadNextPhase))

(event Custom|OnReadyToPlay
  (params (PhaseCount :type Integer))
  (bind _returnvalue (Pawn|GetControlledPawn))
  (bind (_target _location _rotation) (CallFunction|FindPlayerStart PhaseCount))
  ;[0 0 0] Rotate to set the view
  (bind _rate (Timeline|lerp Play)
    (:Update
      (Transformation|SetActorLocation _returnvalue (Math|Vector|Lerp(Vector) (Transformation|GetActorLocation _returnvalue) _location _rate) false false)
      (Pawn|SetControlRotation (Math|Rotator|Lerp(Rotator) (Pawn|GetControlRotation :!class /Script/Engine.Controller) _rotation _rate)))))

(event EventOnPhaseComplete
  (params (Phase :type Integer))
  ;[0 0 0] When the phase completes
  ;;[1 1 1] pause the game
  (|CallParentFunction Phase)
  ;;[1 1 1] Delay for the duration of the Feedback
  (Utilities|FlowControl|Delay (Variables|Default|GetfeedbackDuration))
  (if (!= Phase -1)
    ;[0 0 0] Once the feedback completes, create the Media Widget and add it to the screen
    (bind _returnvalue (UserInterface|CreateWidget "/Game/UI/WBP_MediaPlayer.WBP_MediaPlayer_C" 0 (Variables|Default|GetSource)))
    (bind _output_get (Variables|Default|SetmediaWidget _returnvalue))
    (EventDispatchers|AssignOnPlaybackComplete _output_get (EventDispatchers|CreateEvent :!event Custom|OnPlaybackComplete))
    (UserInterface|Viewport|AddtoViewport _output_get 0)))

(event EventBeginPlay
  (bind _returnvalue (Game|GetPlayerController 0))
  (bind _playercameramanager (Variables|/Script/Engine.PlayerController|GetPlayerCameraManager _returnvalue))
  (|CallParentFunction)
  (EventDispatchers|BindEventtoOnPhaseReadytoPlay (Subsystems|GetGameSubsystem) (EventDispatchers|CreateEvent :!event Custom|OnReadyToPlay))
  (CallFunction|CallLoadNextPhase)
  (Variables|/Script/Engine.PlayerCameraManager|SetViewPitchMin _playercameramanager -1.2e+02)
  (Variables|/Script/Engine.PlayerCameraManager|SetViewPitchMax _playercameramanager 2e+01))

(event Input|KeyboardEvents|SpaceBar
  (params (Key :type Key%20Structure :default "None"))
  (:Released
    (bind _returnvalue (Actor|GetActorOfClass "/Game/BP/Actors/bp_DOOR.bp_DOOR_C"))
    (Class|HealthComponent|DeductHealth (Variables|/Game/BP/Actors/bp_DOOR.bp_DOOR_C|GetHealthComponent _returnvalue) 2e+02)))

(fn ConstructionScript)

(fn FindPlayerStart
  (params (Phase :type Integer))
  (bind _returnvalue (Utilities|String|ToString(Integer) Phase))
  (bind _returnvalue_2 (Game|GetGameMode))
  (bind _self self)
  (bind _returnvalue_3 (Utilities|String|Append "Phase" _returnvalue))
  (bind _returnvalue_4 (Class|GameModeBase|FindPlayerStart _returnvalue_2 _self _returnvalue_3))
  (bind _returnvalue_5 (Transformation|GetActorTransform _returnvalue_4))
  (return _returnvalue_4 (.location _returnvalue_5) (.rotation _returnvalue_5) (.scale _returnvalue_5)))