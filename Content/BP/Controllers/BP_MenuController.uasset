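; BP_MenuController is the player controller for the game's menu.
; On BeginPlay it shows the mouse cursor, switches input to UI-only, and asks the HUD through a widget-initialiser message for the MENU widget, which it adds to the viewport.
; It then fires a trigger parameter on an audio component to start the menu sound.
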(event EventBeginPlay
  (Variables|Default|SetbShowMouseCursor true)
  (Input|SetInputModeUIOnly self 0 "DoNotLock" false)
  (bind _returnvalue (Class|HUDInterface|WidgetInitialiser(Message) (HUD|GetHUD) "MAIN_MENU"))
  (UserInterface|Viewport|AddtoViewport _returnvalue 0)
  (Class|BaseController|InitSound))

(event EventInitSound
  (Class|AudioParameterControllerInterface|SetTriggerParameter (Variables|Default|GetmAudioComp) (Variables|Sounds|GetMenuSoundTrigger)))

(fn ConstructionScript)