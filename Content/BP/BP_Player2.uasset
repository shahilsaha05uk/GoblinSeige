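; BP_Player2 is a player Blueprint that handles camera zoom by changing field of view.
; It stores the default FOV on BeginPlay, and the Zoom event restarts a timeline that sets the camera FOV from GetFOV on each update.
; GetFOV contains an interpolate-and-clamp calculation between min and max FOV, but that chain is marked unused, with no visible connection to the function's output.
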(event EventZoom
  (params (Value :type Float%20%28single-precision%29))
  ;[0 0 0] Zoom
  (bind _rate (Timeline|Timeline PlayFromStart)
    (:Update
      (Camera|SetFieldOfView (Variables|Default|GetCamera) (Utilities|GetFOV _rate Value)))))

(event EventBeginPlay
  (Variables|Default|SetdefaultFOV (Variables|/Script/Engine.CameraComponent|GetFieldOfView (Variables|Default|GetCamera))))

(fn ConstructionScript)