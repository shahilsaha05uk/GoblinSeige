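; BP_SpecPlayer is a player pawn, apparently for spectating, with movement, look and camera zoom input.
; Movement follows control yaw, with roll also feeding the right vector, while look changes only yaw because pitch input is zero.
; Zoom restarts a timeline that sets camera FOV from GetFOV, whose interpolate-and-clamp expression appears unconnected in its graph.
; BeginPlay stores the starting FOV, though nothing shown reads it.
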(event EventMove
  (params (InputActionValue :type Input%20Action%20Value%20Structure%20%28by%20ref%29))
  (bind _returnvalue (Pawn|GetControlRotation :!class /Script/Engine.Pawn))
  ;[0 0 0] Move
  (if true
    (Pawn|Input|AddMovementInput (Math|Vector|GetForwardVector (Math|Rotator|MakeRotator 0.0 0.0 (.yaw (Pawn|GetControlRotation :!class /Script/Engine.Pawn)))) (.x InputActionValue) false)
    (Pawn|Input|AddMovementInput (Math|Vector|GetRightVector (Math|Rotator|MakeRotator (.roll _returnvalue) 0.0 (.yaw _returnvalue))) (.y InputActionValue) false)))

(event EventLook
  (params (InputActionValue :type Input%20Action%20Value%20Structure%20%28by%20ref%29))
  ;[0 0 0] Look
  (Pawn|Input|AddControllerYawInput (.X (Class|EnhancedInputLibrary|BreakInputActionValue InputActionValue)))
  (Pawn|Input|AddControllerPitchInput 0.0))

(event EventZoom
  (params (Value :type Float%20%28single-precision%29))
  ;[0 0 0] Zoom
  (bind _rate (Timeline|ZoomTimeline PlayFromStart)
    (:Update
      (Camera|SetFieldOfView (Variables|Default|GetCamera) (Utilities|GetFOV _rate Value)))))

(event EventBeginPlay
  (Variables|Default|SetdefaultFOV (Variables|/Script/Engine.CameraComponent|GetFieldOfView (Variables|Default|GetCamera))))

(fn ConstructionScript)