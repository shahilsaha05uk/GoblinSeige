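; Player Blueprint with camera FOV zoom and mouse picking.
; Zoom restarts a timeline whose updates set the camera FOV from getFOV, where an interpolate-and-clamp expression appears marked unused.
; Releasing left mouse traces under the cursor through ControllerRef and prints the hit actor's name.
; BeginPlay caches the starting FOV in DefaultFOV, which is not read here.
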(event EventZoom
  (params (Value :type Float%20%28single-precision%29))
  ;[0 0 0] Zoom
  (bind _rate (Timeline|Timeline PlayFromStart)
    (:Update
      (Camera|SetFieldOfView (Variables|Default|GetCamera) (Utilities|GetFOV _rate Value)))))

(event EventBeginPlay
  (Variables|Default|SetdefaultFOV (Variables|/Script/Engine.CameraComponent|GetFieldOfView (Variables|Default|GetCamera))))

(event Input|MouseEvents|LeftMouseButton
  (params (Key :type Key%20Structure :default "None"))
  (bind _controllerref (Variables|Default|GetControllerRef))
  (bind _hitresult (Game|Player|GetHitResultUnderCursorbyChannel _controllerref "TraceTypeQuery5" true))
  (bind (_bblockinghit _binitialoverlap _time _distance _location _impactpoint _normal _impactnormal _physmat _hitactor) (Collision|BreakHitResult _hitresult))
  (:Released
    (if _bblockinghit
      (Development|PrintString (Utilities|GetDisplayName _hitactor)))))

(fn ConstructionScript)