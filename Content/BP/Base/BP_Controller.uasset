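; Base player controller that handles game pausing and switches level audio between background and wave music.
; On begin play it plays a sound and sets Game and UI input mode.
; PauseGame toggles the paused state, adding a menu widget obtained from the HUD or having the HUD destroy it.
; ManageAudio fades one audio component out and back in with the wave or background cue, delaying only the switch to wave music.
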(event EventBeginPlay
  (|CallParentFunction)
  (Class|SoundInterface|PlaySound)
  (Input|SetInputModeGameandUI self 0 "DoNotLock" true false))

(event EventPauseGame
  (if (not (Variables|Default|GetbIsPaused))
    (bind _returnvalue (Class|HUDInterface|WidgetInitialiser(Message) (HUD|GetHUD) "PAUSE_MENU"))
    (UserInterface|Viewport|AddtoViewport _returnvalue 0)
    (Variables|Default|SetbIsPaused true)
    (Game|SetGamePaused true)
    (else
      (Class|HUDInterface|DestroyWidget(Message) (HUD|GetHUD) "PAUSE_MENU")
      (Variables|Default|SetbIsPaused false)
      (Game|SetGamePaused false))))

(event EventManageAudio
  (params (hasWaveStarted :type Boolean))
  (bind _levelaudiocomp (Variables|Default|GetLevelAudioComp))
  (if hasWaveStarted
    (Audio|Components|Audio|FadeOut _levelaudiocomp 2.0 0.0 "Linear" :!class /Script/Engine.AudioComponent)
    (Utilities|FlowControl|Delay 1.0)
    (Audio|Components|Audio|SetSound _levelaudiocomp (Variables|Default|GetWaveCue))
    (Audio|Components|Audio|FadeIn (Variables|Default|GetLevelAudioComp) 1.0 1.0 0.0 "Linear" :!class /Script/Engine.AudioComponent)
    (else
      (Audio|Components|Audio|FadeOut (Variables|Default|GetLevelAudioComp) 2.0 0.0 "Linear" :!class /Script/Engine.AudioComponent)
      (Audio|Components|Audio|SetSound _levelaudiocomp (Variables|Default|GetBackgroundCue))
      (Audio|Components|Audio|FadeIn (Variables|Default|GetLevelAudioComp) 1.0 1.0 0.0 "Linear" :!class /Script/Engine.AudioComponent))))

(fn ConstructionScript)