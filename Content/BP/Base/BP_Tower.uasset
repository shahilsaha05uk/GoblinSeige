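; BP_Tower is a tower building Blueprint that manages its attack range and fires projectiles at targets.
; IncreaseRange, also run by the construction script, sizes the range collision sphere and scales the range decal from the AttackRange stat in BuildingDetails.
; SpawnProjectile spawns the tower's projectile class, passing damage, radius, launch speed, target location and target, falling back to CurrentTarget when the supplied target is invalid.
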(event EventSpawnProjectile
  (params (ProjectileClass :type Projectile%20Class%20Reference) (Location :type Vector :default "0, 0, 0") (Rotation :type Rotator :default "0, 0, 0") (Target :type Actor%20Object%20Reference))
  (bind _buildingdetails (Variables|Default|GetBuildingDetails))
  (bind _buildingstats (Utilities|Struct|BreakBuildingDetails _buildingdetails))
  (bind (_basedamage _basedamageradius _projectilelaunchspeed) (Utilities|Struct|BreakBuildingStats _buildingstats))
  ;[0 0 0] Spawning a projectile
  (Utilities|IsValid Target
    (:Is%20Valid
      (Variables|Default|SettmpTarget Target))
    (:Is%20Not%20Valid
      (Variables|Default|SettmpTarget (Variables|Default|GetCurrentTarget))))
  (Game|SpawnActorfromClass (Variables|Default|GetmProjectileClass) (Math|Transform|MakeTransform Location Rotation "1.000000,1.000000,1.000000") "Undefined" "MultiplyWithRoot" self _basedamage _basedamageradius (Variables|Default|GetTargetLocation) _projectilelaunchspeed (Variables|Default|GettmpTarget) 0))

(event EventIncreaseRange
  (bind _buildingdetails (Variables|Default|GetBuildingDetails))
  (bind _buildingstats (Utilities|Struct|BreakBuildingDetails _buildingdetails))
  (bind _attackrange (Utilities|Struct|BreakBuildingStats _buildingstats))
  (bind _returnvalue (/ _attackrange 1e+02))
  ;[0 0 0] Increasing the range
  (Components|Sphere|SetSphereRadius (Variables|Default|GetRangeCollisionComp) _attackrange false)
  (Transformation|SetRelativeScale3D (Variables|Default|GetRangeDecalComp) (Math|Vector|MakeVector 2.0 _returnvalue _returnvalue)))

(fn ConstructionScript
  (Class|BaseBuilding|IncreaseRange))