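; Enemy controller that spawns a goblin pawn and relays attack and move commands to the pawn it controls.
; SpawnPawn creates a BP_Goblin at a random XY point within the spawn box's bounds at a fixed height, stores it as EnemyRef, then calls the parent implementation.
; EnemyAttack and EnemyMove send BI_EnemyInterface messages to the controlled pawn, after checking it implements that interface.
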(event EventEnemyAttack
  (bind _returnvalue (Pawn|GetControlledPawn))
  (if (Utilities|DoesObjectImplementInterface _returnvalue "/Game/BP/AI/BI_EnemyInterface.BI_EnemyInterface_C")
    (Class|BIEnemyInterface|IAEnemyAttack(Message) _returnvalue)))

(event EventEnemyMove
  (bind _returnvalue (Pawn|GetControlledPawn))
  (if (Utilities|DoesObjectImplementInterface _returnvalue "/Game/BP/AI/BI_EnemyInterface.BI_EnemyInterface_C")
    (Class|BIEnemyInterface|IAEnemyMove(Message) _returnvalue)))

(event EventSpawnPawn
  (params (SpawnBox :type Enemy%20Spawn%20Point%20Object%20Reference))
  (bind _returnvalue (Game|SpawnActorfromClass "/Game/BP/AI/BP_Goblin.BP_Goblin_C" (Math|Transform|MakeTransform (Class|EnemySpawnPoint|GetRandomPointInsidetheSpawnArea SpawnBox) "0, 0, 0" "1.000000,1.000000,1.000000") "AlwaysSpawn" "MultiplyWithRoot" 0 0))
  (Variables|Default|SetEnemyRef _returnvalue)
  (|CallParentFunction SpawnBox))

(fn ConstructionScript)

(fn GetRandomPointInsidetheSpawnArea
  (params (SpawnPoint :type Box%20Component%20Object%20Reference))
  (bind (_origin _boxextent) (Collision|GetComponentBounds SpawnPoint))
  (bind _returnvalue (Math|Random|RandomPointinBoundingBox _origin _boxextent))
  (return (Math|Vector|MakeVector (.x _returnvalue) (.y _returnvalue) 1e+01)))