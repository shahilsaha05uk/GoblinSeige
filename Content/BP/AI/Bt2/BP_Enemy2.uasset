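; Goblin enemy Blueprint that walks a spline trail under AI control and has a montage-driven attack.
; FollowtheSpline stores the spline, then GoToNextPoint chains AI moves to random navigable locations around each successive point, advancing even when a move fails.
; Passing the last point sets a trail-completed Blackboard flag.
; Attack plays the montage and catches its notify, where door-breaking or looting is still a debug-print placeholder.
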(event Custom|GoToNextPoint
  (bind (_randomlocation _returnvalue) (CallFunction|GetNextLoc))
  (bind _currentpoint (Variables|Default|GetCurrentPoint))
  (if _returnvalue
    (AI|AIMoveTo (AI|GetAIController self) self _randomlocation 0 1e+02 false
      (:OnSuccess
        _)
      (:OnFail
        _))
    (Class|CompoundOperatorsBPLibrary|AddtoIntInt _currentpoint 1)
    (if (<= _currentpoint (Variables|Default|GetTotalSplines))
      (CallFunction|GotoNextPoint)
      (else
        (AI|Components|Blackboard|SetValueasBool (AI|GetBlackboard 0) (Variables|Default|Getblackboard_HasCompletedTrail) true)))))

(event Custom|OnAttackNotified
  ;[1 1 1] Break Door/ loot treasure
  (Development|PrintString "Attack!!"))

(event EventFollowtheSpline
  (params (Spline :type BP%20Spline%20Object%20Reference))
  (bind _output_get (Variables|Default|SetSpline (Variables|/Game/BP/AI/Bt2/BP_spline.BP_spline_C|GetSpline Spline)))
  (Utilities|IsValid _output_get
    (:Is%20Valid
      (Variables|Default|SetTotalSplines (Spline|GetNumberOfSplinePoints _output_get))
      (Variables|Default|SetCurrentPoint 0)
      (CallFunction|GotoNextPoint))))

(event EventAttack
  (bind _notifyname (Animation|Montage|PlayMontage (Variables|Character|GetMesh) "/Game/Animations/GoblinAttack.GoblinAttack")
    (:OnNotifyBegin
      (if (== _notifyname (Variables|Default|GetAttackNotif))
        (CallFunction|OnAttackNotified)))))

(event EventInit
  (|CallParentFunction)
  (Variables|/Script/Engine.CharacterMovementComponent|SetMaxWalkSpeed (Variables|Character|GetCharacterMovement) 1.8e+03))

(fn ConstructionScript)

(fn GetNextLoc
  (bind _spline (Variables|Default|GetSpline))
  (Utilities|IsValid _spline
    (:Is%20Valid
      (bind (_randomlocation _returnvalue) (Class|NavigationSystemV1|GetRandomLocationinNavigableRadius (Spline|GetLocationatSplinePoint _spline (Variables|Default|GetCurrentPoint) "World") 2e+03 0 0))
      (return _randomlocation _returnvalue))))