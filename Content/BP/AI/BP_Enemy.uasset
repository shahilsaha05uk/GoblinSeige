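; Enemy AI pawn Blueprint that walks along a given spline's points and plays a goblin attack montage.
; Movement chains AI move-to calls, aiming at a random navigable location around each spline point, offset along the spline component's forward vector.
; Capsule overlap with a target-interface actor sets a reached-target blackboard flag.
; The attack montage's notify is forwarded to the parent class's attack handler.
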(event OnComponentBeginOverlap(CapsuleComponent)
  (params (OverlappedComponent :type Primitive%20Component%20Object%20Reference) (OtherActor :type Actor%20Object%20Reference) (OtherComp :type Primitive%20Component%20Object%20Reference) (OtherBodyIndex :type Integer) (bFromSweep :type Boolean) (SweepResult :type Hit%20Result%20Structure%20%28by%20ref%29))
  ;[1 1 1] Notifies the blackboard when they reach within the target
  (if (Utilities|DoesObjectImplementInterface OtherActor "/Script/TowerDefenceGame.TargetInterface")
    (AI|Components|Blackboard|SetValueasBool (AI|GetBlackboard 0) (Variables|Blackboard|Getblackboard_HasReachedNearTarget) true)
    (Development|PrintString "Reached Target")))

(event Custom|Follow
  (bind _movementresult (AI|AIMoveTo self (CallFunction|GetNextPoint (Variables|Spline|GetCurrentPoint)) 0 8e+02 false)
    (:then
      (Development|PrintString (Utilities|String|EnumtoString _movementresult)))
    (:OnSuccess
      (if (< (Variables|Spline|GetCurrentPoint) (Variables|Spline|GetTotalSplinePoints))
        (Math|Integer|IncrementInt (Variables|Spline|GetCurrentPoint)
          (:%20%20
            (CallFunction|Follow)))))))

(event EventIAFollowtheSpline
  (params (Spline :type Spline%20Object%20Reference))
  (bind _output_get (Variables|Spline|SetTargetSpline (Variables|/Script/TowerDefenceGame.Spline|GetmSpline Spline)))
  (Variables|Spline|SetTotalSplinePoints (Spline|GetNumberOfSplinePoints _output_get))
  (Variables|Spline|SetCurrentPoint 0)
  (CallFunction|Follow))

(event EventOnAttackNotified
  (|CallParentFunction))

(event EventIAEnemyAttack
  ;[0 0 0] When the enemy attacks
  (bind _notifyname (Animation|Montage|PlayMontage (Variables|Character|GetMesh) "/Game/Animations/GoblinAttack.GoblinAttack")
    (:OnNotifyBegin
      (if (== _notifyname (Variables|Private|GetAttackNotif))
        (Class|BaseEnemy|OnAttackNotified)))))

(fn ConstructionScript)

(fn GetNextPoint
  (params (PointIndex :type Integer))
  (bind _targetspline (Variables|Spline|GetTargetSpline))
  (bind _randomlocation (Class|NavigationSystemV1|GetRandomLocationinNavigableRadius (+ (Spline|GetLocationatSplinePoint _targetspline PointIndex "World") (* (Math|Vector|GetForwardVector _targetspline) 1e+03)) 1e+03 0 0))
  (return _randomlocation))