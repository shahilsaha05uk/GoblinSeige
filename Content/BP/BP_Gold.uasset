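; BP_Gold is a lootable gold Blueprint that tracks how much gold remains and ends the game once it is depleted.
; On BeginPlay it caches its widget component's WBP_GoldLootBar and fills the current gold to the total.
; Each LootGold event removes one gold, updates the loot bar, and at zero or below triggers the game-over signature on BP_GameMode.
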(event EventBeginPlay
  (|CallParentFunction)
  (bind _aswbp_gold_loot_bar (Utilities|Casting|CastToWBP_GoldLootBar (UserInterface|GetWidget (Variables|Default|GetWidgetComp))))
  (Variables|Default|SetGoldLootBar _aswbp_gold_loot_bar)
  (Variables|Default|SetmCurrentGold (Variables|Default|GetmTotalGold)))

(event EventLootGold
  (bind _output_get (Variables|Default|SetmCurrentGold (- (Variables|Default|GetmCurrentGold) 1)))
  (Class|GoldLootBar|LootGold (Variables|Default|GetGoldLootBar) _output_get (Variables|Default|GetmTotalGold))
  (if (<= (Variables|Default|GetmCurrentGold) 0)
    (bind _asbp_game_mode (Utilities|Casting|CastToBP_GameMode (Game|GetGameMode)))
    (Default|CallOnGameOverSignature _asbp_game_mode)))

(fn ConstructionScript)