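; Zombie enemy character that walks at reduced speed and attacks the level's Castle actor, which it caches on BeginPlay.
; Attack plays a montage and damages the castle when its attack notify begins.
; Incoming damage feeds a health component, which updates the health widget while health stays above zero.
; A looping timer also makes the zombie periodically damage itself, and FindCastle is an empty stub.
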(event Custom|Attack
  (bind _castleref (Variables|Default|GetCastleRef))
  (Utilities|IsValid _castleref
    (:Is%20Valid
      (bind _notifyname (Animation|Montage|PlayMontage (Variables|Character|GetMesh) "/Game/Animations/zombie_attack_Montage.zombie_attack_Montage")
        (:OnNotifyBegin
          (if (== _notifyname "OnAttackNotify")
            (Game|Damage|ApplyDamage _castleref 2e+01 (Game|GetInstigatorController) self)))))))

(event Custom|TakeDamage
  (bind _self self)
  (Game|Damage|ApplyDamage _self 5.0 (Game|GetInstigatorController _self) _self))

(event Custom|OnDamageTaken
  (params (DamagedActor :type Actor%20Object%20Reference) (Damage :type Float%20%28single-precision%29) (DamageType :type Damage%20Type%20Object%20Reference) (InstigatedBy :type Controller%20Object%20Reference) (DamageCauser :type Actor%20Object%20Reference))
  (bind _mhealthcomponent (Variables|Default|GetmHealthComponent))
  (bind _returnvalue (Class|HealthComponent|GetHealth _mhealthcomponent))
  (Class|HealthComponent|OnDamageTaken _mhealthcomponent Damage)
  (if (not (<= _returnvalue 0.0))
    (Class|HealthBarWidget|Updater (Variables|Default|GetmHealthWidget) _returnvalue)))

(event EventBeginPlay
  (Variables|/Script/Engine.CharacterMovementComponent|SetMaxWalkSpeed (Variables|Character|GetCharacterMovement) 2e+02)
  (EventDispatchers|AssignOnTakeAnyDamage (delegate Custom|OnDamageTaken))
  (bind _returnvalue (Actor|GetActorOfClass "/Game/BP/Castle.Castle_C"))
  (Variables|Default|SetCastleRef _returnvalue)
  (Utilities|Time|SetTimerbyEvent (delegate Custom|TakeDamage) 3.0 true))

(fn ConstructionScript)

(fn FindCastle)

(fn IsCastleValid
  (return (Utilities|IsValid (Variables|Default|GetCastleRef))))