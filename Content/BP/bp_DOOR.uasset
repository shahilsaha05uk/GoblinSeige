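; Door actor with a health component that takes damage and displays its health through a widget.
; On BeginPlay it initializes the WBP_ObjectHealth widget with that component and binds a handler to its any-damage event.
; The handler deducts health only if the damaged actor, rather than the damage causer, implements BI_EnemyInterface2.
; The graph contains no opening or destruction logic.
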(event Custom|OnTakeDamage
  (params (DamagedActor :type Actor%20Object%20Reference) (Damage :type Float%20%28single-precision%29) (DamageType :type Damage%20Type%20Object%20Reference) (InstigatedBy :type Controller%20Object%20Reference) (DamageCauser :type Actor%20Object%20Reference))
  (if (Utilities|DoesObjectImplementInterface DamagedActor "/Game/BP/AI/Bt2/BI_EnemyInterface2.BI_EnemyInterface2_C")
    (Class|HealthComponent|DeductHealth (Variables|Default|GetHealthComponent) Damage)))

(event Custom|HealthCompInitialised
  (bind _aswbp_object_health (Utilities|Casting|CastToWBP_ObjectHealth (UserInterface|GetWidget (Variables|Default|GetWidget))))
  (Default|Init _aswbp_object_health (Variables|Default|GetHealthComponent)))

(event EventBeginPlay
  (CallFunction|HealthCompInitialised)
  (EventDispatchers|AssignOnTakeAnyDamage (delegate Custom|OnTakeDamage)))

(fn ConstructionScript)