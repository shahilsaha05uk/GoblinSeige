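; BP_Tower is a placeable, upgradeable tower building that fires projectiles at its target.
; SpawnProjectile spawns the projectile class at SpawnPoint when the target is valid, passing in the target and damage from BuildingStats.
; For pooling, finished projectiles are moved back to SpawnPoint and hidden.
; Upgrades play a Niagara effect, while Interact and Disassociate extend parent behavior to toggle the placement's radius sphere.
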(event EventUpgrade
  (params (Details :type Upgrade%20Details%20Structure))
  ;[1 1 1] Play the niagara when the player upgrades
  (|CallParentFunction Details)
  (Components|Activation|Activate (Variables|Default|GetmNiagaraUpgradeComp) false))

(event EventInteract
  ;[1 1 1] When the player interacts
  (|CallParentFunction)
  (bind _asbp_placement (Utilities|Casting|CastToBP_Placement (Variables|Default|GetmPlacement)))
  (Rendering|SetVisibility (Variables|/Game/BP/Actors/BP_Placement.BP_Placement_C|GetradSphere _asbp_placement) true false))

(event EventDisassociate
  ;[1 1 1] When the player loses focus
  (|CallParentFunction)
  (bind _asbp_placement (Utilities|Casting|CastToBP_Placement (Variables|Default|GetmPlacement)))
  (Rendering|SetVisibility (Variables|/Game/BP/Actors/BP_Placement.BP_Placement_C|GetradSphere _asbp_placement) false false))

(event EventOnProjectileJobComplete
  (params (Projectile :type Projectile%20Object%20Reference))
  ;[1 1 1] When pooling a projectile completes
  (Transformation|SetActorLocation Projectile (Transformation|GetWorldLocation (Variables|Default|GetSpawnPoint)) false false)
  (Rendering|SetActorHiddenInGame Projectile true))

(fn ConstructionScript)

(fn SpawnProjectile
  (bind _mtarget (Variables|Default|GetmTarget))
  (Utilities|IsValid _mtarget
    (:Is%20Valid
      (bind _returnvalue (Game|SpawnActorfromClass (Variables|Default|GetProjectileClass) (Transformation|GetWorldTransform (Variables|Default|GetSpawnPoint)) "AlwaysSpawn" "MultiplyWithRoot" 0 (Utilities|Struct|BreakBuildingStats (Variables|Default|GetBuildingStats)) "0.000000,0.000000,0.000000" _mtarget 0))
      (return _returnvalue))))