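; BP_Placers is an actor that switches its static mesh between a default material and an interaction material.
; BeginPlay runs the parent logic, then caches the mesh's slot 0 material as the default.
; The ToggleMaterial event takes a boolean and either applies the interact material to that slot or restores the cached default.
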(event EventBeginPlay
  (|CallParentFunction)
  (Variables|Default|SetmDefaultMaterial (Rendering|Material|GetMaterial (Variables|Default|GetmStaticMesh) 0)))

(event EventToggleMaterial
  (params (Value :type Boolean))
  (bind _mstaticmesh (Variables|Default|GetmStaticMesh))
  (if Value
    (Rendering|Material|SetMaterial _mstaticmesh 0 (Variables|Default|GetmInteractMaterial))
    (else
      (Rendering|Material|SetMaterial _mstaticmesh 0 (Variables|Default|GetmDefaultMaterial)))))

(fn ConstructionScript)