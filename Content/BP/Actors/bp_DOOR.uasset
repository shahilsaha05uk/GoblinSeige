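; Destructible door actor that enemies attack as a target, with a health component and a widget displaying its health.
; On BeginPlay it initialises the widget and binds to damage, health update and game subsystem phase-complete events.
; Only damage from causers implementing EnemyInterface deducts health, and reaching zero notifies the subsystem that the target is destroyed.
; A phase-complete handler hides the door, while phase-change and failure-feedback calls are left unconnected.
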(event Custom|OnTakeDamage
  (params (DamagedActor :type Actor%20Object%20Reference) (Damage :type Float%20%28single-precision%29) (DamageType :type Damage%20Type%20Object%20Reference) (InstigatedBy :type Controller%20Object%20Reference) (DamageCauser :type Actor%20Object%20Reference))
  ;[0 0 0] When the Door takes any damage
  (if (Utilities|DoesObjectImplementInterface DamageCauser "/Script/TowerDefenceGame.EnemyInterface")
    (Class|HealthComponent|DeductHealth (Variables|Default|GetHealthComponent) Damage)))

(event Custom|OnObjectDamaged
  (params (CurrentHealth :type Float%20%28single-precision%29))
  (if (<= CurrentHealth 0.0)
    (Default|CallOnTargetDestroyed (Subsystems|GetGameSubsystem))))

(event Custom|HealthCompInitialised
  ;[0 0 0] Initialise the HealthComponent
  (bind _aswbp_object_health (Utilities|Casting|CastToWBP_ObjectHealth (UserInterface|GetWidget (Variables|Default|GetWidget))))
  (Class|ParentBar|Init _aswbp_object_health (Variables|Default|GetHealthComponent)))

(event Custom|OnPhaseComplete
  (params (Phase :type Integer))
  (Rendering|SetActorHiddenInGame true))

(event EventBeginPlay
  ;[0 0 0] When the Game Begins
  (CallFunction|HealthCompInitialised)
  (EventDispatchers|AssignOnTakeAnyDamage (delegate Custom|OnTakeDamage))
  (EventDispatchers|BindEventtoOnPhaseComplete (Subsystems|GetGameSubsystem) (EventDispatchers|CreateEvent :!event Custom|OnPhaseComplete))
  (EventDispatchers|BindEventtoOnHealthUpdated (Variables|Default|GetHealthComponent) (delegate Custom|OnObjectDamaged)))

(fn ConstructionScript)