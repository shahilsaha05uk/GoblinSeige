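; BP_Placement is an actor that switches its static mesh's look between a default and a selected state.
; BeginPlay runs the parent logic, then caches the mesh's slot 0 material as the default.
; The ToggleMaterial event takes a boolean and applies either the selected material or the cached default to that slot.
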(event EventToggleMaterial
  (params (Value :type Boolean))
  (bind _mstaticmesh (Variables|Default|GetmStaticMesh))
  ;[0 0 0] Changing Material
  (if Value
    (Rendering|Material|SetMaterial _mstaticmesh 0 (Variables|Default|GetSelectedMat))
    (else
      (Rendering|Material|SetMaterial _mstaticmesh 0 (Variables|Default|GetDefaultMat)))))

(event EventBeginPlay
  ;[0 0 0] Setting the Default Mat
  (|CallParentFunction)
  (Variables|Default|SetDefaultMat (Rendering|Material|GetMaterial (Variables|Default|GetmStaticMesh) 0)))

(fn ConstructionScript)