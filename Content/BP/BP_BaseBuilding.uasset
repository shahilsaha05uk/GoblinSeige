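; Base building Blueprint that flags whether the building can be placed while it is in placement mode.
; A box component's begin overlap switches the building to an invalid material and clears CanPlace.
; Any end overlap restores the normal material and CanPlace without checking for remaining overlaps, and both events print debug strings.
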(event OnComponentBeginOverlap(BoxComp)
  (params (OverlappedComponent :type Primitive%20Component%20Object%20Reference) (OtherActor :type Actor%20Object%20Reference) (OtherComp :type Primitive%20Component%20Object%20Reference) (OtherBodyIndex :type Integer) (bFromSweep :type Boolean) (SweepResult :type Hit%20Result%20Structure%20%28by%20ref%29))
  (if (Variables|Default|GetbInPlacementMode)
    (Class|BaseBuilding|ChangeBuildingMaterial "INVALID_MATERIAL")
    (Variables|Default|SetbCanPlace false)
    (Development|PrintString "Cant Place")))

(event OnComponentEndOverlap(BoxComp)
  (params (OverlappedComponent :type Primitive%20Component%20Object%20Reference) (OtherActor :type Actor%20Object%20Reference) (OtherComp :type Primitive%20Component%20Object%20Reference) (OtherBodyIndex :type Integer))
  (if (Variables|Default|GetbInPlacementMode)
    (Class|BaseBuilding|ChangeBuildingMaterial "VALID_MATERIAL")
    (Variables|Default|SetbCanPlace true)
    (Development|PrintString "Place")))

(fn ConstructionScript)