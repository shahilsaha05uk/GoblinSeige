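; BP_GameMode is a game mode Blueprint that handles phase transitions by swapping streamed levels.
; On phase load it runs the parent logic, unloads the Shahil1 level, blocking-loads Shahil2 as visible, then tells the game subsystem the current phase loaded.
; When a phase load succeeds, it asks the subsystem to show success feedback naming that phase.
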(event EventOnPhaseLoad
  (|CallParentFunction)
  (Class|GameplayStatics|UnloadStreamLevelbySoftObjectPtr "/Game/Assets/Stylized_Egypt/Maps/Shahil1.Shahil1" true)
  (Class|GameplayStatics|LoadStreamLevelbySoftObjectPtr "/Game/Assets/Stylized_Egypt/Maps/Shahil2.Shahil2" true true)
  (Default|CallOnPhaseLoadedSuccessfully (Subsystems|GetGameSubsystem) (Class|TowerDefenceGameGameModeBase|GetCurrentPhase)))

(event EventOnPhaseLoadedSuccess
  (params (LoadedPhase :type Integer))
  (Default|CallOnFeedbackEnabled (Subsystems|GetGameSubsystem) "Feed_Success" (Utilities|String|Append "Phase " (Utilities|String|ToString(Integer) LoadedPhase))))

(fn ConstructionScript)