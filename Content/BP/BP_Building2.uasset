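; BP_Building2 is a building Blueprint with an attack range shown by a decal.
; Its construction script calls IncreaseRange, which sizes the range collision sphere to MAttackRadius and scales the decal's Y and Z to match, at one unit per 100.
; The event graph holds only unconnected nodes that would toggle CanPlace and swap between valid and invalid materials, so that placement feedback never runs here.
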(fn ConstructionScript
  (CallFunction|IncreaseRange))

(fn IncreaseRange
  (bind _mattackradius (Variables|Default|GetmAttackRadius))
  (bind _returnvalue (/ _mattackradius 1e+02))
  (Components|Sphere|SetSphereRadius (Variables|Default|GetRangeCollisionComp) _mattackradius true)
  (Transformation|SetRelativeScale3D (Variables|Default|GetRangeDecalComp) (Math|Vector|MakeVector 1.0 _returnvalue _returnvalue)))