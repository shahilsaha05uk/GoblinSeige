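; Machine gun tower Blueprint that aims at a target and shoots projectiles at it.
; Fire aims through the parent's look-at logic, then spawns a projectile at the Arrow component's transform, passing it the current target.
; Without a valid target, it powers off, searches for a new one and fires immediately if found.
; An unconnected graph holds interpolated pitch and yaw aiming that never runs.
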(event EventStartCannonProjectile
  (bind _arrow (Variables|Default|GetArrow))
  (bind _returnvalue (Transformation|GetWorldTransform _arrow))
  (Class|Turret|SpawnProjectile (Variables|Default|GetmProjectileClass) (.location _returnvalue) (.rotation _returnvalue) (Variables|Default|GetCurrentTarget)))

(event EventLookatTarget
  (|CallParentFunction))

(event EventFire
  (Variables|Default|GetCurrentTarget
    (:then
      _)
    (:else
      (Class|Turret|PowerOff)
      (bind _returnvalue (Class|Turret|FindTarget))
      (bind _output_get (Variables|Default|SetCurrentTarget _returnvalue))
      (Utilities|IsValid _output_get
        (:Is%20Valid
          _))))
  (Class|Turret|LookatTarget)
  (CallFunction|StartCannonProjectile))

(fn ConstructionScript
  (|CallParentFunction))