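; BP_Tower_LaunchingPad is a tower weapon that launches BP_Missile projectiles at its current target.
; Its Fire event overrides the parent, spawning a missile at the Arrow component's transform with the target passed in, then calling parent Fire.
; If the target is invalid or reports dead through IsDeadMessage, it picks a new one with FindTarget and skips that shot.
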(event EventFire
  (bind _arrow (Variables|Default|GetArrow))
  (bind _returnvalue (Transformation|GetWorldTransform _arrow))
  ;[0 0 0] Fire
  (bind _currenttarget (Variables|Default|GetCurrentTarget)
    (:then
      (bind _returnvalue_2 (Class|EnemyInterface|IsDead(Message) _currenttarget))
      (if _returnvalue_2
        (bind _returnvalue_3 (Class|Turret|FindTarget :!label _label))
        (Variables|Default|SetCurrentTarget _returnvalue_3)
        (else
          (Class|Turret|SpawnProjectile "/Game/BP/Projectiles/BP_Missile.BP_Missile_C" (.location _returnvalue) (.rotation _returnvalue) _currenttarget)
          (|CallParentFunction))))
    (:else
      (goto _label))))

(fn ConstructionScript
  (|CallParentFunction))