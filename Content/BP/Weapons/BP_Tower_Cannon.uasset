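; BP_Tower_Cannon is a cannon tower weapon Blueprint that estimates how long it needs to aim at its current target.
; For a valid target, it takes the absolute yaw gap between MFort2's rotation and the look-at rotation from MFort3 to the target.
; It divides that gap by a fixed rate tied to FacingTarget's interpolation speed.
; Its construction script only runs the parent's.
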(fn ConstructionScript
  (|CallParentFunction))

(fn CalculatetheAimingTime
  (bind _currenttarget (Variables|Default|GetCurrentTarget)
    (:then
      (return (/ (Math|Float|Absolute(Float) (.yaw (Math|Rotator|Delta(Rotator) (Math|Rotator|FindLookatRotation (Transformation|GetWorldLocation (Variables|Default|GetM_Fort3)) (Transformation|GetActorLocation _currenttarget)) (Transformation|GetWorldRotation (Variables|Default|GetM_Fort2))))) 1.5e+02)))
    (:else)))