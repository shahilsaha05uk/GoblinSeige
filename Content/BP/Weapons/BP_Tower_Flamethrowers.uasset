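; Flamethrower tower Blueprint, apparently a variant of a parent tower that supplies the cannon projectile events and building stats.
; StartCannonProjectile is an empty event, while StopCannonProjectile switches off the FXFlame effect.
; Flame activation and stat-driven radial damage at the Arrow are left unwired, so neither runs here.
; Construction only calls the parent script, with range-based Box sizing also disconnected.
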(event EventStartCannonProjectile)

(event EventStopCannonProjectile
  (Components|Activation|SetActive (Variables|Default|GetFX_Flame) false false))

(fn ConstructionScript
  (|CallParentFunction))