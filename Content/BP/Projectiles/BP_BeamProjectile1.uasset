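; BP_BeamProjectile1 is a projectile Blueprint that homes on a target and takes speed changes from upgrades.
; ActivateProjectile stores the target and, if it is valid, points its BHP projectile movement component's homing at that actor and its current location.
; OnUpgrade, only for radial projectiles, overrides the movement's initial and max speed, skipping each value left at its sentinel default.
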(event EventOnUpgrade
  (params (ProjectileDetails :type Projectile%20Details%20Structure))
  (bind (_bisradialprojectile _initialspeed _maxspeed) (Utilities|Struct|BreakProjectileDetails ProjectileDetails))
  (bind _bhp_projectilemovement (Variables|Default|GetBHP_ProjectileMovement))
  (if _bisradialprojectile
    (Utilities|FlowControl|Sequence
      (:then_0
        (if (!= _initialspeed 0.0)
          (Variables|/Script/Engine.ProjectileMovementComponent|SetInitialSpeed _bhp_projectilemovement _initialspeed)))
      (:then_1
        (if (!= _maxspeed -1.0)
          (Variables|/Script/Engine.ProjectileMovementComponent|SetMaxSpeed _bhp_projectilemovement _maxspeed))))))

(event EventActivateProjectile
  (params (Target :type Actor%20Object%20Reference) (MinSpeed :type Float%20%28single-precision%29) (MaxSpeed :type Float%20%28single-precision%29))
  (bind _output_get (Variables|Default|SetmTarget Target))
  (Utilities|IsValid _output_get
    (:Is%20Valid
      (Class|BHPProjectileMovementComponent|SetHomingPointonActor (Variables|Default|GetBHP_ProjectileMovement) (Variables|Default|GetmTarget) (Transformation|GetActorLocation (Variables|Default|GetmTarget))))))

(fn ConstructionScript
  (|CallParentFunction))