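; Homing missile projectile that chases a target actor and explodes on hit, dealing full radial damage that visibility blockers can prevent.
; After a short launch delay it enables Tick for guidance, or destroys itself if the target is invalid.
; Tick interpolates ProjectileMovement velocity toward the target while raising speed by a fixed amount each frame, so acceleration depends on frame rate.
; Hit spawns a pooled Niagara explosion before destroying the missile.
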(event EventBeginPlay
  (Utilities|FlowControl|Delay 0.5)
  (Actor|Tick|SetActorTickEnabled true)
  (Utilities|IsValid (Variables|Default|GetmTarget)
    (:Is%20Not%20Valid
      (Actor|DestroyActor))))

(event EventTick
  (params (DeltaSeconds :type Float%20%28single-precision%29))
  (bind _mtarget (Variables|Default|GetmTarget))
  (Utilities|IsValid _mtarget
    (:Is%20Valid
      (Variables|Default|SetmTargetLocation (Transformation|GetActorLocation _mtarget))
      (Variables|/Script/Engine.MovementComponent|SetVelocity (Variables|Default|GetProjectileMovement) (Math|Interpolation|VInterpTo (Variables|/Script/Engine.MovementComponent|GetVelocity (Variables|Default|GetProjectileMovement)) (* (Math|Vector|GetUnitDirection(Vector) (Transformation|GetActorLocation) (Variables|Default|GetmTargetLocation)) (Variables|Default|GetmLaunchSpeed)) (Utilities|Time|GetWorldDeltaSeconds) 3.0))
      (Variables|Default|SetmLaunchSpeed (+ (Variables|Default|GetmLaunchSpeed) 5e+03)))))

(event Collision|EventHit
  (params (MyComp :type Primitive%20Component%20Object%20Reference) (Other :type Actor%20Object%20Reference) (OtherComp :type Primitive%20Component%20Object%20Reference) (bSelfMoved :type Boolean) (HitLocation :type Vector :default "0, 0, 0") (HitNormal :type Vector :default "0, 0, 0") (NormalImpulse :type Vector :default "0, 0, 0") (Hit :type Hit%20Result%20Structure%20%28by%20ref%29))
  (Niagara|SpawnSystematLocation "/Game/Particles/FX_Explode.FX_Explode" HitLocation "0, 0, 0" "5.000000,5.000000,5.000000" true true "AutoRelease")
  (Game|Damage|ApplyRadialDamage (Variables|Default|GetmBaseDamageValue) (Transformation|GetActorLocation) (Variables|Default|GetmDamageRadius) 0 0 0 0 true "ECC_Visibility") ; 可视性遮挡则无伤害
  (Actor|DestroyActor))

(fn ConstructionScript
  (Variables|/Script/Engine.ProjectileMovementComponent|SetInitialSpeed (Variables|Default|GetProjectileMovement) (Variables|Default|GetmLaunchSpeed)))