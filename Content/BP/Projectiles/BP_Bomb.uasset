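; BP_Bomb is a projectile that explodes and deals area damage when it hits.
; The construction script copies its launch speed variable into the ProjectileMovement initial speed.
; On Hit it spawns an enlarged explosion effect at the hit location, applies full radial damage from its own position, then destroys itself.
; Damage has no distance falloff and is prevented by occluders on the WorldStatic channel.
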(event Collision|EventHit
  (params (MyComp :type Primitive%20Component%20Object%20Reference) (Other :type Actor%20Object%20Reference) (OtherComp :type Primitive%20Component%20Object%20Reference) (bSelfMoved :type Boolean) (HitLocation :type Vector :default "0, 0, 0") (HitNormal :type Vector :default "0, 0, 0") (NormalImpulse :type Vector :default "0, 0, 0") (Hit :type Hit%20Result%20Structure%20%28by%20ref%29))
  (Niagara|SpawnSystematLocation "/Game/Particles/FX_Explode.FX_Explode" HitLocation "0, 0, 0" "5.000000,5.000000,5.000000")
  (Game|Damage|ApplyRadialDamage (Variables|Default|GetmBaseDamageValue) (Transformation|GetActorLocation) (Variables|Default|GetmDamageRadius) 0 0 self 0 true "ECC_WorldStatic") ; 可视性遮挡则无伤害
  (Actor|DestroyActor))

(fn ConstructionScript
  (Variables|/Script/Engine.ProjectileMovementComponent|SetInitialSpeed (Variables|Default|GetProjectileMovement) (Variables|Default|GetmLaunchSpeed)))