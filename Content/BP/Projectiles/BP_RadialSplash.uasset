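; Radial splash projectile Blueprint that applies area damage to enemies around its location when its DealDamage event is called.
; DealDamage runs a sphere overlap sized to the scaled radius of ProjectileCollider, filtered to one object type and ignoring itself.
; Each overlapped actor implementing EnemyInterface receives TakeRadiamDamageMessage with no damage value passed, keeping the splash decoupled from concrete enemy classes.
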(event EventDealDamage
  (params (DamagedActor :type Actor%20Object%20Reference) (BaseDamage :type Float%20%28single-precision%29) (EventInstigator :type Controller%20Object%20Reference) (DamageCauser :type Actor%20Object%20Reference))
  (bind _outactors (Collision|SphereOverlapActors (Transformation|GetActorLocation) (Components|Sphere|GetScaledSphereRadius (Variables|Default|GetProjectileCollider)) (Utilities|Array|MakeArray "ObjectTypeQuery11") 0 (Utilities|Array|MakeArray self)))
  (for _array_element _outactors
    (if (Utilities|DoesObjectImplementInterface _array_element "/Script/TowerDefenceGame.EnemyInterface")
      (Class|EnemyInterface|TakeRadiamDamage(Message) _array_element))))

(fn ConstructionScript)