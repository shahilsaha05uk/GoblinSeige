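; Homing projectile that flies at an assigned target and damages overlapped actors implementing EnemyInterface.
; ActivateProjectile unhides it, sets up muzzle and trail Niagara effects and starts a fast looping timer for target tracking.
; Tracking interpolates location toward the target, optionally rotating to face it.
; Any overlap or lost target stops the timer and signals job completion via dispatcher, rather than destroying the actor.
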(event OnComponentBeginOverlap(ProjectileCollider)
  (params (OverlappedComponent :type Primitive%20Component%20Object%20Reference) (OtherActor :type Actor%20Object%20Reference) (OtherComp :type Primitive%20Component%20Object%20Reference) (OtherBodyIndex :type Integer) (bFromSweep :type Boolean) (SweepResult :type Hit%20Result%20Structure%20%28by%20ref%29))
  (bind _hitniagara (Variables|Default|GetHitNiagara))
  (Components|Activation|Deactivate (Variables|Default|GetProjectileNiagara))
  (if (Utilities|DoesObjectImplementInterface OtherActor "/Script/TowerDefenceGame.EnemyInterface")
    (Class|NiagaraComponent|SetAsset (Variables|Default|GetHitNiagara) (Variables|Default|GetmProjectileHitAsset) true)
    (Components|Activation|SetActive _hitniagara true false)
    (Transformation|SetWorldLocation _hitniagara (Transformation|GetActorLocation OtherActor) false false)
    (CallFunction|DealDamage OtherActor (Variables|Default|GetmDamage) 0 (Components|GetOwner))
    (Class|Projectile|DeactivateProjectile)
    (Default|CallOnDamageDealt)
    (else
      (Class|Projectile|DeactivateProjectile))))

(event Custom|TrackTarget
  (bind _interp_speed (Variables|Default|GetInterp%20Speed))
  (bind (_rot _loc) (CallFunction|SetTarget _interp_speed))
  (if (Variables|Default|GetbShouldRotate)
    (Transformation|SetActorRotation _rot))
  (Transformation|SetActorLocation _loc false false)
  (Utilities|IsValid (Variables|Default|GetmTarget)
    (:Is%20Not%20Valid
      (Class|Projectile|DeactivateProjectile))))

(event Custom|DealDamage
  (params (DamagedActor :type Actor%20Object%20Reference) (BaseDamage :type Float%20%28single-precision%29) (EventInstigator :type Controller%20Object%20Reference) (DamageCauser :type Actor%20Object%20Reference))
  ;[1 1 1] Default damage
  (Game|Damage|ApplyDamage DamagedActor BaseDamage EventInstigator DamageCauser))

(event EventDeactivateProjectile
  (Default|CallOnProjectileJobComplete self)
  (Utilities|Time|ClearandInvalidateTimerbyHandle (Variables|TimerHandles|GetTargetTrackerTimerHandle)))

(event EventActivateProjectile
  (params (Target :type Actor%20Object%20Reference) (Details :type Projectile%20Details%20Structure))
  (bind _projectilemovement (Variables|Default|GetProjectileMovement))
  (bind _muzzleniagara (Variables|Default|GetMuzzleNiagara))
  (bind _projectileniagara (Variables|Default|GetProjectileNiagara))
  (bind _output_get (Variables|Default|SetmTarget Target))
  (Utilities|IsValid _output_get
    (:Is%20Valid
      (Rendering|SetActorHiddenInGame self false)
      (Transformation|SetActorRotation (.Rot (CallFunction|SetTarget (Variables|Default|GetInterp%20Speed))))
      (Niagara|ResetSystem _muzzleniagara)
      (Class|NiagaraComponent|SetAsset _muzzleniagara (Variables|Default|GetmProjectileMuzzleAsset) false)
      (Components|Activation|SetActive _muzzleniagara true false)
      (Transformation|SetWorldLocation _muzzleniagara (Transformation|GetActorLocation) false false)
      (Niagara|ResetSystem _projectileniagara)
      (Class|NiagaraComponent|SetAsset _projectileniagara (Variables|Default|GetmProjectileAsset) false)
      (bind _output_get_2 (Variables|/Script/Engine.ProjectileMovementComponent|SetMaxSpeed _projectilemovement (Variables|Default|GetmLaunchSpeed)))
      (Variables|/Script/Engine.ProjectileMovementComponent|SetInitialSpeed _projectilemovement _output_get_2)
      (bind _returnvalue (Utilities|Time|SetTimerbyEvent (EventDispatchers|CreateEvent :!event Custom|TrackTarget) 0.002 true))
      (Variables|TimerHandles|SetTargetTrackerTimerHandle _returnvalue))
    (:Is%20Not%20Valid
      (Class|Projectile|DeactivateProjectile))))

(fn ConstructionScript)

(fn SetTarget
  (params (InterpSpeed :type Float%20%28single-precision%29))
  (bind _returnvalue (Transformation|GetActorLocation))
  (bind _mtarget (Variables|Default|GetmTarget))
  (bind _returnvalue_2 (Transformation|GetActorLocation _mtarget))
  (Utilities|IsValid (Variables|Default|GetmTarget)
    (:Is%20Valid
      (return (Math|Rotator|FindLookatRotation _returnvalue _returnvalue_2) (Math|Interpolation|VInterpTo _returnvalue _returnvalue_2 (Utilities|Time|GetWorldDeltaSeconds) InterpSpeed)))))