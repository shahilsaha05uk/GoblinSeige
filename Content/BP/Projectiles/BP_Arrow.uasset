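; Homing arrow projectile that chases a target actor and damages what it hits.
; Each tick it interpolates its velocity toward a point slightly above the target, with launch speed growing every frame.
; On a valid hit it attaches to the struck component, applies damage, and disables collision and movement.
; If the hit actor is invalid, it destroys itself after a brief delay.
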(event EventTick
  (params (DeltaSeconds :type Float%20%28single-precision%29))
  (Variables|/Script/Engine.MovementComponent|SetVelocity (Variables|Default|GetProjectileMovement) (CallFunction|TracktheTarget))
  (Variables|Default|SetmLaunchSpeed (+ (Variables|Default|GetmLaunchSpeed) 1e+02)))

(event Collision|EventHit
  (params (MyComp :type Primitive%20Component%20Object%20Reference) (Other :type Actor%20Object%20Reference) (OtherComp :type Primitive%20Component%20Object%20Reference) (bSelfMoved :type Boolean) (HitLocation :type Vector :default "0, 0, 0") (HitNormal :type Vector :default "0, 0, 0") (NormalImpulse :type Vector :default "0, 0, 0") (Hit :type Hit%20Result%20Structure%20%28by%20ref%29))
  ;[1 1 1] Hit
  (Utilities|IsValid Other
    (:Is%20Valid
      (Variables|Default|SetHit true)
      (Transformation|AttachComponentToComponent OtherComp "None" "KeepWorld" "KeepWorld" "KeepRelative" false)
      (Game|Damage|ApplyDamage Other (Variables|Default|GetmDamageValue) 0 self)
      (Collision|SetCollisionEnabled (Variables|Default|GetSphere) "NoCollision")
      (Components|Activation|Deactivate (Variables|Default|GetProjectileMovement)))
    (:Is%20Not%20Valid
      (Utilities|FlowControl|Delay 0.01)
      (Actor|DestroyActor))))

(fn ConstructionScript
  (Variables|/Script/Engine.ProjectileMovementComponent|SetInitialSpeed (Variables|Default|GetProjectileMovement) (Variables|Default|GetmLaunchSpeed)))

(fn TracktheTarget
  (bind _mtarget (Variables|Default|GetmTarget)
    (:then
      (return (Math|Interpolation|VInterpTo (Variables|/Script/Engine.MovementComponent|GetVelocity (Variables|Default|GetProjectileMovement)) (* (Math|Vector|GetUnitDirection(Vector) (Transformation|GetActorLocation) (+ (Transformation|GetActorLocation _mtarget) "0.000000,0.000000,30.000000")) (Variables|Default|GetmLaunchSpeed)) (Utilities|Time|GetWorldDeltaSeconds) 15.0)))
    (:else)))