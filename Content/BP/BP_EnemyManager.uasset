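; BP_EnemyManager is a manager for spawning enemy controllers, which gathers every BP_EnemySpawnPoint in the level on BeginPlay.
; SpawnEnemies loops to spawn BP_EnemyController actors, handing each the given spawn point as its SpawnBox.
; GetRandomEnemyVal computes a random enemy total and a per-point share from the spawn point count.
; RequestEnemies is empty, and the logic distributing enemies across points is disconnected, so nothing here triggers spawning.
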(event Custom|RequestEnemies)

(event Custom|SpawnEnemies
  (params (LastIndex :type Integer) (spawnPoint :type BP%20Enemy%20Spawn%20Point%20Object%20Reference))
  (for _index (range 0 LastIndex)
    (Game|SpawnActorfromClass "/Game/BP/AI/BP_EnemyController.BP_EnemyController_C" (Variables|Default|GetControllerTransform) "Undefined" "MultiplyWithRoot" 0 spawnPoint 0)))

(event EventBeginPlay
  (bind _outactors (Actor|GetAllActorsOfClass "/Game/BP/BP_EnemySpawnPoint.BP_EnemySpawnPoint_C"))
  (Variables|Default|SetEnemySpawnPoints _outactors))

(fn ConstructionScript)

(fn GetRandomEnemyVal
  (bind _returnvalue (Math|Random|RandomFloatinRange 5.0 1e+01))
  (bind _returnvalue_2 (Math|Float|Ceil _returnvalue))
  (return _returnvalue_2 (/ _returnvalue_2 (Utilities|Array|Length (Variables|Default|GetEnemySpawnPoints)))))