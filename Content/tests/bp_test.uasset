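; Egyptian statue turret Blueprint with fire Niagara effects on its left and right sockets, meant to shoot projectiles at BaseEnemy actors.
; Sphere overlaps pick the nearest enemy, then start or stop a looping fire timer, which also starts on BeginPlay.
; SpawnerProjectile can spawn a projectile from each socket, but Fire is empty and the logic calling the spawner is disconnected, so nothing shoots.
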(event OnComponentBeginOverlap(Sphere)
  (params (OverlappedComponent :type Primitive%20Component%20Object%20Reference) (OtherActor :type Actor%20Object%20Reference) (OtherComp :type Primitive%20Component%20Object%20Reference) (OtherBodyIndex :type Integer) (bFromSweep :type Boolean) (SweepResult :type Hit%20Result%20Structure%20%28by%20ref%29))
  (CallFunction|FindTarget)
  (Variables|Default|GetTarget
    (:then
      (CallFunction|StartFiring))
    (:else
      (CallFunction|StopFiring))))

(event Custom|SetTarget
  (params (Target :type Actor%20Object%20Reference))
  (Variables|Default|SetTarget Target))

(event Custom|StartFiring
  (bind _returnvalue (Utilities|Time|SetTimerbyEvent (delegate Custom|Fire) (Variables|Default|GetfireRate) true))
  (Variables|Default|SetFiringTimerHandle _returnvalue))

(event Custom|Fire)

(event Custom|SpawnerProjectile
  (params (Class :type BP%20Projectile%20Class%20Reference) (Interp%20Speed :type Float%20%28single-precision%29) (InitialSpeed :type Float%20%28single-precision%29) (MaxSpeed :type Float%20%28single-precision%29) (mDamage :type Float%20%28single-precision%29) (mTargetLocation :type Vector) (mTarget :type Actor%20Object%20Reference))
  (bind (_left _right) (CallFunction|GetSocketTransforms))
  (Game|SpawnActorfromClass Class _left "Undefined" "MultiplyWithRoot" 0 Interp%20Speed true InitialSpeed MaxSpeed mDamage mTargetLocation mTarget 0)
  (Game|SpawnActorfromClass Class _right "Undefined" "MultiplyWithRoot" 0 Interp%20Speed true InitialSpeed MaxSpeed mDamage mTargetLocation mTarget 0))

(event Custom|StopFiring
  (Utilities|Time|ClearandInvalidateTimerbyHandle (Variables|Default|GetFiringTimerHandle))
  (Variables|Default|SetTarget 0))

(event Custom|FindTarget
  (CallFunction|SetTarget (.ReturnValue (Actor|FindNearestActor (Transformation|GetActorLocation) (Collision|GetOverlappingActors (Variables|Default|GetSphere) "/Script/TowerDefenceGame.BaseEnemy" :!class /Script/Engine.PrimitiveComponent)))))

(event EventBeginPlay
  (bind _sm_egyptian_statue_01 (Variables|Default|GetSM_egyptian_statue_01))
  (Niagara|SpawnSystemAttached (Variables|Default|GetFireNiagara) _sm_egyptian_statue_01 "left" "0, 0, 0" "0, 0, 0" "KeepWorldPosition" false)
  (Niagara|SpawnSystemAttached (Variables|Default|GetFireNiagara) _sm_egyptian_statue_01 "right" "0, 0, 0" "0, 0, 0" "KeepWorldPosition" false)
  (CallFunction|StartFiring))

(fn ConstructionScript)

(fn GetSocketTransforms
  (bind _sm_egyptian_statue_01 (Variables|Default|GetSM_egyptian_statue_01))
  (return (Transformation|GetSocketTransform _sm_egyptian_statue_01 "left" "RTS_World") (Transformation|GetSocketTransform _sm_egyptian_statue_01 "right" "RTS_World")))