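; Modular turret actor that assembles a base mesh and an upper weapon component from indexed part lists in its construction script.
; Fire and reload, from events or left mouse and R, are forwarded to the upper component.
; On begin play it either replaces itself with a substitute class for that upper, keeping the base mesh, or sets its activation state.
; Activation drives emissive materials and a looping timer that toggles rotation audio as the upper turns.
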(event Custom|HandleGunRotationSounds
  (bind _rotateaudio (Variables|Default|GetRotateAudio))
  (bind _upper (Variables|Default|GetUpper))
  (bind _returnvalue (Transformation|GetSocketRotation _upper "root"))
  ;[0.05 0.05 0.05] Activation / Deactivation
  ;;[0.05 0.05 0.05] Handling rotation sounds
  (if (Utilities|Operators|NotEqual(!=) (Variables|Turret|GetPreviousUpperRotation) _returnvalue 0.1)
    (Utilities|IsValid _rotateaudio
      (:Is%20Valid
        (Components|Activation|Activate _rotateaudio false))
      (:Is%20Not%20Valid
        _))
    (else
      (Utilities|IsValid _rotateaudio
        (:Is%20Valid
          (Components|Activation|Deactivate _rotateaudio))
        (:Is%20Not%20Valid
          _))))
  (Variables|Turret|SetPreviousUpperRotation _returnvalue))

(event Custom|OnTurretActivated
  ;[0.05 0.05 0.05] Activation / Deactivation
  (Rendering|Material|SetScalarParameterValueonMaterials (Variables|Default|GetBase) "Emissive_01" 5e+01)
  ;;[0.05 0.05 0.05] Handling rotation sounds
  (bind _returnvalue (Utilities|Time|SetTimerbyEvent (delegate Custom|HandleGunRotationSounds) 0.1 true))
  (Variables|Turret|SetRotationSoundTimerHandle _returnvalue))

(event Custom|Reload
  ;[0.05 0.05 0.05] Reload
  (bind _uppercomponent (Variables|Default|GetUpperComponent)
    (:then
      (Default|Reload _uppercomponent))
    (:else)))

(event Custom|Fire
  ;[0.05 0.05 0.05] Fire
  (bind _uppercomponent (Variables|Default|GetUpperComponent)
    (:then
      (Default|Fire _uppercomponent))
    (:else)))

(event Custom|Substitute
  (bind _substitutions (Variables|Turret|GetSubstitutions))
  (bind _upperindex (Variables|Turret|GetUpperIndex))
  (bind _baseaniminstances (Variables|Turret|GetBaseAnimInstances))
  (bind _baseindex (Variables|Turret|GetBaseIndex))
  (bind _output (Utilities|Array|Get(acopy) _substitutions _upperindex))
  (bind _output_2 (Utilities|Array|Get(acopy) _baseaniminstances _baseindex))
  ;[0.05 0.05 0.05] Substitute
  (if (Utilities|IsValidClass _output)
    (bind _returnvalue (Game|SpawnActorfromClass _output (Transformation|GetActorTransform) "AlwaysSpawn" "SelectDefaultAtRuntime" (Components|GetOwner) (Game|GetInstigator)))
    (Components|SkinnedMesh|SetSkinnedAssetandUpdate (Variables|/Game/Turrets_Pack_01/Blueprints/BP_Turret.BP_Turret_C|GetBase _returnvalue) (Components|SkeletalMesh|GetSkeletalMeshAsset (Variables|Default|GetBase)) true)
    (if (Utilities|IsValidClass _output_2)
      (Class|SkeletalMeshComponent|SetAnimClass (Variables|/Game/Turrets_Pack_01/Blueprints/BP_Turret.BP_Turret_C|GetBase _returnvalue) _output_2))
    (Actor|DestroyActor)))

(event Custom|OnTurretDeactivated
  ;[0.05 0.05 0.05] Activation / Deactivation
  (Rendering|Material|SetScalarParameterValueonMaterials (Variables|Default|GetBase) "Emissive_01" 0.0)
  (Utilities|Time|ClearandInvalidateTimerbyHandle (Variables|Turret|GetRotationSoundTimerHandle)))

(event Custom|UpdateParts
  ;[0.05 0.05 0.05] Update parts
  (if (Variables|Turret|GetIsModular)
    (Components|SkinnedMesh|SetSkinnedAssetandUpdate (Variables|Default|GetBase) (Utilities|Array|Get(acopy) (Variables|Turret|GetBaseList) (Variables|Turret|GetBaseIndex)) true)
    (bind _uppercomponent (Variables|Default|GetUpperComponent)
      (:then
        (Components|DestroyComponent _uppercomponent))
      (:else
        _))
    (bind _returnvalue (Game|AddComponentbyClass (Utilities|Array|Get(acopy) (Variables|Turret|GetUpperList) (Variables|Turret|GetUpperIndex))))
    (Variables|Default|SetUpperComponent _returnvalue)
    (bind _uppercomponent_2 (Variables|Default|GetUpperComponent)
      (:then
        (Components|SkinnedMesh|SetSkinnedAssetandUpdate (Variables|Default|GetUpper) (Variables|/Game/tests/BP_Turret_Upper.BP_Turret_Upper_C|GetUpperMesh _uppercomponent_2) true))
      (:else
        (Components|SkinnedMesh|SetSkinnedAssetandUpdate (Variables|Default|GetUpper) 0 true)))
    (else
      (Variables|Default|SetUpperComponent (Actor|GetComponentbyClass "/Game/tests/BP_Turret_Upper.BP_Turret_Upper_C")))))

(event EventBeginPlay
  ;[0.05 0.05 0.05] Begin play
  (if (Variables|Turret|GetSubstituteOnBeginPlay)
    (CallFunction|Substitute)
    (else
      (Utilities|FlowControl|DelayUntilNextTick)
      (if (Variables|Turret|GetStartActivated)
        (CallFunction|OnTurretActivated)
        (else
          (CallFunction|OnTurretDeactivated))))))

(event Input|MouseEvents|LeftMouseButton
  (params (Key :type Key%20Structure))
  ;[0.05 0.05 0.05] Fire
  (:Pressed
    (bind _uppercomponent (Variables|Default|GetUpperComponent)
      (:then
        (Default|Fire _uppercomponent))
      (:else))))

(event Input|KeyboardEvents|R
  (params (Key :type Key%20Structure))
  ;[0.05 0.05 0.05] Reload
  (:Pressed
    (bind _uppercomponent (Variables|Default|GetUpperComponent)
      (:then
        (Default|Reload _uppercomponent))
      (:else))))

(fn ConstructionScript
  (CallFunction|UpdateParts))