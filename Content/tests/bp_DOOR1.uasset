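; Breakable door that only enemies can damage, with a widget showing its health.
; On begin play it initialises the widget from its HealthComponent and binds to damage and health updates.
; Damage deducts health only when the causer implements EnemyInterface.
; At zero health it notifies the game subsystem that the door broke and raises a warning feedback with the failure message.
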(event Custom|OnTakeDamage
  (params (DamagedActor :type Actor%20Object%20Reference) (Damage :type Float%20%28single-precision%29) (DamageType :type Damage%20Type%20Object%20Reference) (InstigatedBy :type Controller%20Object%20Reference) (DamageCauser :type Actor%20Object%20Reference))
  ;[0 0 0] When the Door takes any damage
  (if (Utilities|DoesObjectImplementInterface DamageCauser "/Script/TowerDefenceGame.EnemyInterface")
    (Class|HealthComponent|DeductHealth (Variables|Default|GetHealthComponent) Damage)))

(event Custom|OnObjectDamaged
  (params (CurrentHealth :type Float%20%28single-precision%29))
  (bind _returnvalue (Subsystems|GetGameSubsystem))
  (if (<= CurrentHealth 0.0)
    (Default|CallOnDoorBroken _returnvalue)
    (Default|CallOnFeedbackEnabled _returnvalue "Feed_Warning" (.Value (Utilities|Map|Find (Variables|Default|GetFeedbackString) "Feed_Failed")))))

(event Custom|HealthCompInitialised
  ;[0 0 0] Initialise the HealthComponent
  (bind _aswbp_object_health (Utilities|Casting|CastToWBP_ObjectHealth (UserInterface|GetWidget (Variables|Default|GetWidget))))
  (Class|ParentBar|Init _aswbp_object_health (Variables|Default|GetHealthComponent)))

(event EventBeginPlay
  ;[0 0 0] When the Game Begins
  (CallFunction|HealthCompInitialised)
  (EventDispatchers|AssignOnTakeAnyDamage (delegate Custom|OnTakeDamage))
  (EventDispatchers|BindEventtoOnHealthUpdated (Variables|Default|GetHealthComponent) (delegate Custom|OnObjectDamaged)))

(fn ConstructionScript)