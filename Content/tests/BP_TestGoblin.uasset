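; BP_TestGoblin is a test goblin actor with health that removes itself from the world when killed.
; Its OnHealthUpdated event destroys the actor once current health drops to zero or below.
; IsDead is a stub that always returns false, and GetTarget is empty.
; A SetHealth call on MHealthComponent is left unconnected, so it never runs.
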(event EventOnHealthUpdated
  (params (CurrentHealth :type Float%20%28single-precision%29))
  (if (<= CurrentHealth 0.0)
    (Actor|DestroyActor)))

(fn ConstructionScript
  (|CallParentFunction))

(fn IsDead
  (return false))

(fn GetTarget
  (return 0))