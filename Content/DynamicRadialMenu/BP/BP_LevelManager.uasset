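; Level manager that saves and restores the player's transform and inventory through a BP_Savedata save slot.
; On BeginPlay it registers itself with each checkpoint, then, if a save exists, moves the player to the saved transform and restores inventory items and selected indices.
; Its SaveGame event creates the save object if needed, captures the player's current state and writes it to the slot, without using the passed Checkpoint.
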(event Custom|Save%20Game
  (params (checkpoint :type BP%20Checkpoint%20Object%20Reference))
  (Utilities|IsValid (Variables|Default|Getsavedata)
    (:Is%20Valid
      _)
    (:Is%20Not%20Valid
      (bind _returnvalue (SaveGame|CreateSaveGameObject "/Game/DynamicRadialMenu/BP/BP_Savedata.BP_Savedata_C"))
      (Variables|Default|Setsavedata _returnvalue)))
  (|SetSaveVariables)
  (SaveGame|SaveGametoSlot (Variables|Default|Getsavedata) (Variables|Default|GetSlot%20Name)))

(event EventBeginPlay
  (|InitCheckpoints
    (:Completed
      (bind _returnvalue (SaveGame|DoesSaveGameExist (Variables|Default|GetSlot%20Name)))
      (if _returnvalue
        (bind _returnvalue_2 (SaveGame|LoadGamefromSlot (Variables|Default|GetSlot%20Name)))
        (bind _asbp_savedata (Utilities|Casting|CastToBP_Savedata _returnvalue_2))
        (bind _output_get (Variables|Default|Setsavedata _asbp_savedata))
        (Transformation|SetActorLocationAndRotation (Game|GetPlayerCharacter 0) (.location (Variables|/Game/DynamicRadialMenu/BP/BP_Savedata.BP_Savedata_C|Getplayer%20transform _output_get)) (.rotation (Variables|/Game/DynamicRadialMenu/BP/BP_Savedata.BP_Savedata_C|Getplayer%20transform _output_get)))
        (|LoadInventory)))))

(fn ConstructionScript)