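; Health pack interactable that a character picks up, inspects in hand and collects into the inventory.
; StartInteraction plays a take montage, turns the character with hand IK on, then on the montage notify starts the inspect montage and eases the attached pack into the hand socket.
; Collect requires the item in hand; it and Unequipped add the item and expire the actor.
; ShowTip displays key prompts on the HUD, while Use defers to the parent.
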(event EventBeginPlay
  (|CallParentFunction) ; This node is disabled and will not be called.\nDrag off pins to build functionality.
)

(event Collision|EventActorBeginOverlap
  (params (OtherActor :type Actor%20Object%20Reference))
  (|CallParentFunction OtherActor) ; This node is disabled and will not be called.\nDrag off pins to build functionality.
)

(event EventTick
  (params (DeltaSeconds :type Float%20%28single-precision%29))
  (|CallParentFunction DeltaSeconds) ; This node is disabled and will not be called.\nDrag off pins to build functionality.
)

(event EventStartInteraction
  (params (interacting%20character :type Character%20Object%20Reference))
  (if (not (Variables|Default|GetItemInHand))
    (Utilities|FlowControl|DoOnce false :!label _label
      (:Completed
        (Variables|Default|SetInteracting%20Character interacting%20character)
        (Animation|Montage|PlayMontage (Variables|/Script/Engine.Character|GetMesh (Variables|Default|GetInteracting%20Character)) "/Game/DynamicRadialMenu/DemoContent/Mannequin/Animations/AM_ThirdPersonInspectTake.AM_ThirdPersonInspectTake" 2.0
          (:then
            (Class|BPICharacter|Turnto(Message) (Variables|Default|GetInteracting%20Character) (Transformation|GetWorldLocation (Variables|Default|Getobject%20mesh)))
            (Class|BPICharacter|ToggleHandIK(Message) (Variables|Default|GetInteracting%20Character) true))
          (:OnInterrupted
            (goto _label Reset))
          (:OnNotifyBegin
            (Animation|Montage|PlayMontage (Variables|/Script/Engine.Character|GetMesh (Variables|Default|GetInteracting%20Character)) "/Game/DynamicRadialMenu/DemoContent/Mannequin/Animations/AM_ThirdPersonInspect.AM_ThirdPersonInspect"
              (:then
                (Transformation|AttachComponentToComponent (Variables|/Script/Engine.Character|GetMesh (Variables|Default|GetInteracting%20Character)) "hand_r_socket" "KeepWorld" "KeepWorld" "KeepWorld" true)
                (Components|MoveComponentTo (Variables|Default|GetDefaultSceneRoot) "0, 0, 0" "0, 0, 0" true true 0.3 true)
                (Variables|Default|SetItemInHand true)))))))))

(event EventUse
  (params (used%20by :type Character%20Object%20Reference))
  (|CallParentFunction used%20by))

(event EventCollect
  (params (inventory :type BP%20Inventory%20Object%20Reference))
  (bind _interacting_character (Variables|Default|GetInteracting%20Character))
  (if (Variables|Default|GetItemInHand)
    (bind _inventory (Class|BPICharacter|GetInventory(Message) (Variables|Default|GetInteracting%20Character)))
    (Default|AddItem _inventory (Variables|Default|Getinventory%20item))
    (Actor|SetLifeSpan 0.1)
    (Class|BPICharacter|ToggleHandIK(Message) _interacting_character false)
    (Animation|StopAnimMontage _interacting_character "/Game/DynamicRadialMenu/DemoContent/Mannequin/Animations/AM_ThirdPersonInspect.AM_ThirdPersonInspect")
    (|CallParentFunction inventory)
    (else
      (Development|PrintString "Collect the Item in Hand First!"))))

(event EventUnequipped
  (params (Inventory :type BP%20Inventory%20Object%20Reference) (Interacting%20Character :type Character%20Object%20Reference))
  (Variables|Default|SetInteracting%20Character Interacting%20Character)
  (bind _inventory (Class|BPICharacter|GetInventory(Message) (Variables|Default|GetInteracting%20Character)))
  (Default|AddItem _inventory (Variables|Default|Getinventory%20item))
  (Actor|SetLifeSpan 0.1)
  (Class|BPICharacter|ToggleHandIK(Message) (Variables|Default|GetInteracting%20Character) true)
  (Animation|StopAnimMontage (Variables|Default|GetInteracting%20Character) "/Game/DynamicRadialMenu/DemoContent/Mannequin/Animations/AM_ThirdPersonInspect.AM_ThirdPersonInspect"))

(fn ConstructionScript
  (|CallParentFunction))

(fn ShowTip
  (bind _returnvalue (Game|GetPlayerController 0))
  (bind _keys (Class|BPIPlayerController|GetInputKeys(Message) _returnvalue "Interact"))
  (bind _keys_2 (Class|BPIPlayerController|GetInputKeys(Message) _returnvalue "Collect"))
  (Class|BPIHud|ShowTip(Message) (HUD|GetHUD _returnvalue) (Utilities|String|Append "Press " _keys " to Interact. " "Press " _keys_2 " to Collect " (Utilities|String|ToString(Text) (.name (Variables|Default|Getinventory%20item))) ".") 5.0))