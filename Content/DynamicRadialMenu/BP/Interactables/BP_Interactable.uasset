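; Base interactable pickup that players can inspect in hand, put back, collect into inventory or use.
; A sphere overlap registers it with the overlapping actor, highlighting the mesh and showing a key tip for players.
; StartInteraction toggles taking and leaving, using montage notifies to attach or detach it and glide it between hand socket and original transform.
; Collect and Unequipped add its item struct to inventory; Use plays a heal montage, and all three expire the actor.
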(event OnComponentBeginOverlap(Sphere)
  (params (OverlappedComponent :type Primitive%20Component%20Object%20Reference) (OtherActor :type Actor%20Object%20Reference) (OtherComp :type Primitive%20Component%20Object%20Reference) (OtherBodyIndex :type Integer) (bFromSweep :type Boolean) (SweepResult :type Hit%20Result%20Structure%20%28by%20ref%29))
  (Class|BPICharacter|SetInteractable(Message) OtherActor self)
  (bind _yes_no (Class|BPICharacter|IsPlayer(Message) OtherActor))
  (if _yes_no
    (CallFunction|ShowTip)
    (Rendering|Material|SetScalarParameterValueonMaterials (Variables|Default|Getobject%20mesh) "highlight" 1.0)))

(event OnComponentEndOverlap(Sphere)
  (params (OverlappedComponent :type Primitive%20Component%20Object%20Reference) (OtherActor :type Actor%20Object%20Reference) (OtherComp :type Primitive%20Component%20Object%20Reference) (OtherBodyIndex :type Integer))
  (Class|BPICharacter|SetInteractable(Message) OtherActor)
  (Rendering|Material|SetScalarParameterValueonMaterials (Variables|Default|Getobject%20mesh) "highlight" 0.0))

(event EventBeginPlay
  (Variables|Default|Setinitial%20transform (Transformation|GetActorTransform)))

(event EventUnequipped
  (params (Inventory :type BP%20Inventory%20Object%20Reference) (Interacting%20Character :type Character%20Object%20Reference))
  (Variables|Default|SetInteracting%20Character Interacting%20Character)
  (Animation|StopAnimMontage (Variables|Default|GetInteracting%20Character) "/Game/DynamicRadialMenu/DemoContent/Mannequin/Animations/AM_ThirdPersonInspect.AM_ThirdPersonInspect")
  (Class|BPICharacter|ToggleInspectView(Message) (Variables|Default|GetInteracting%20Character) true)
  (Actor|SetLifeSpan 0.1)
  (Class|BPICharacter|ToggleInspectView(Message) (Variables|Default|GetInteracting%20Character) false)
  (bind _inventory (Class|BPICharacter|GetInventory(Message) (Variables|Default|GetInteracting%20Character)))
  (Default|AddItem _inventory (Variables|Default|Getinventory%20item)))

(event EventStartInteraction
  (params (interacting%20character :type Character%20Object%20Reference))
  (Utilities|FlowControl|DoOnce false :!label _label
    (:Completed
      (Variables|Default|SetInteracting%20Character interacting%20character)
      (if (Variables|Default|Getinteracting)
        (|LeaveObject)
        (goto _label Reset)
        (else
          (|TakeObject)
          (goto _label Reset))))))

(event EventCollect
  (params (inventory :type BP%20Inventory%20Object%20Reference))
  (bind _interacting_character (Variables|Default|GetInteracting%20Character))
  (if (Variables|Default|Getinteracting)
    (Animation|StopAnimMontage _interacting_character "/Game/DynamicRadialMenu/DemoContent/Mannequin/Animations/AM_ThirdPersonInspect.AM_ThirdPersonInspect")
    (Class|BPICharacter|ToggleInspectView(Message) _interacting_character true)
    (Actor|SetLifeSpan 0.1)
    (Class|BPICharacter|ToggleInspectView(Message) _interacting_character false)
    (bind _inventory (Class|BPICharacter|GetInventory(Message) _interacting_character))
    (Default|AddItem _inventory (Variables|Default|Getinventory%20item))))

(event EventUse
  (params (used%20by :type Character%20Object%20Reference))
  (Class|BPICharacter|GetInventory(Message) used%20by)
  (Actor|SetLifeSpan 0.1)
  (Animation|Montage|PlayMontage (Variables|/Script/Engine.Character|GetMesh used%20by) "/Game/DynamicRadialMenu/DemoContent/Mannequin/Animations/AM_Heal.AM_Heal"))

(fn ConstructionScript
  (Utilities|Struct|SetmembersinSTRUCT_inventory_item (Variables|Default|Getinventory%20item) (Utilities|GetClass self))
  (Variables|/Script/Engine.PrimitiveComponent|SetbGenerateOverlapEvents (Variables|Default|GetSphere) (Variables|Default|Getcan%20interact)))

(fn ShowTip
  (bind _returnvalue (Game|GetPlayerController 0))
  (bind _keys (Class|BPIPlayerController|GetInputKeys(Message) _returnvalue "Interact"))
  (Class|BPIHud|ShowTip(Message) (HUD|GetHUD _returnvalue) (Utilities|String|Append "Use " _keys " to Inspect " (Utilities|String|ToString(Text) (.name (Variables|Default|Getinventory%20item)))) 5.0))

(fn GetItemData
  (return (Variables|Default|Getinventory%20item)))

(fn IsThrowable
  (return false))