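; BP_stone is a throwable stone interactable for the dynamic radial menu system.
; It reports itself as throwable through IsThrowable, which always returns true.
; Its Throw event turns on query and physics collision and physics simulation on ObjectMesh, then replaces the mesh's linear velocity with the supplied launch velocity.
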(event EventBeginPlay
  (|CallParentFunction) ; This node is disabled and will not be called.\nDrag off pins to build functionality.
)

(event Collision|EventActorBeginOverlap
  (params (OtherActor :type Actor%20Object%20Reference))
  (|CallParentFunction OtherActor) ; This node is disabled and will not be called.\nDrag off pins to build functionality.
)

(event EventTick
  (params (DeltaSeconds :type Float%20%28single-precision%29))
  (|CallParentFunction DeltaSeconds) ; This node is disabled and will not be called.\nDrag off pins to build functionality.
)

(event EventThrow
  (params (Launch%20velocity :type Vector :default "0, 0, 0"))
  (bind _object_mesh (Variables|Default|Getobject%20mesh))
  (Collision|SetCollisionEnabled _object_mesh "QueryAndPhysics")
  (Physics|SetSimulatePhysics _object_mesh true)
  (Class|PrimitiveComponent|SetAllPhysicsLinearVelocity _object_mesh Launch%20velocity false))

(fn ConstructionScript
  (|CallParentFunction))

(fn IsThrowable
  (return true))