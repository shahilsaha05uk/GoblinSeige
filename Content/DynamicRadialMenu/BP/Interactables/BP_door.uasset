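; Interactable sliding door for the radial menu project that opens when a character interacts with it and closes itself after a short wait.
; StartInteraction eases the object mesh sideways with MoveComponentTo, delays, then eases it back to its zero relative location.
; A DoOnce blocks repeat interactions until the cycle resets.
; ShowTip displays a timed HUD prompt built from the keys bound to Interact.
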(event EventBeginPlay
  (|CallParentFunction) ; This node is disabled and will not be called.\nDrag off pins to build functionality.
)

(event Collision|EventActorBeginOverlap
  (params (OtherActor :type Actor%20Object%20Reference))
  (|CallParentFunction OtherActor) ; This node is disabled and will not be called.\nDrag off pins to build functionality.
)

(event EventTick
  (params (DeltaSeconds :type Float%20%28single-precision%29))
  (|CallParentFunction DeltaSeconds) ; This node is disabled and will not be called.\nDrag off pins to build functionality.
)

(event EventStartInteraction
  (params (interacting%20character :type Character%20Object%20Reference))
  (Utilities|FlowControl|DoOnce false :!label _label
    (:Completed
      (Variables|Default|SetInteracting%20Character interacting%20character)
      (Components|MoveComponentTo (Variables|Default|Getobject%20mesh) "0,-170.000000, 0" "0, 0, 0" true true 0.8 true)
      (Utilities|FlowControl|Delay 5.0)
      (Components|MoveComponentTo (Variables|Default|Getobject%20mesh) "0, 0, 0" "0, 0, 0" true true 0.8 true)
      (goto _label Reset))))

(fn ConstructionScript
  (|CallParentFunction))

(fn ShowTip
  (bind _returnvalue (Game|GetPlayerController 0))
  (bind _keys (Class|BPIPlayerController|GetInputKeys(Message) _returnvalue "Interact"))
  (Class|BPIHud|ShowTip(Message) (HUD|GetHUD _returnvalue) (Utilities|String|Append "Press" _keys " to open") 3.0))