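; Inventory Blueprint for the dynamic radial menu system, storing item structs with name, usage and quantity.
; AddItem stacks quantities by matching name, while RemoveItem decrements by one and drops emptied entries.
; GetItemsByUsage filters items by usage and remembers a selected index per usage, optionally advancing it and wrapping to the first.
; It also stores the active interactable, and GetItemData only clears the player's interactable status message.
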(event Custom|SetActiveInteractable
  (params (Interactable :type BP%20Interactable%20Object%20Reference))
  (Variables|Default|SetInteractable Interactable))

(fn AddItem
  (params (item :type STRUCT%20Inventory%20Item%20Structure))
  (bind (_name _quantity) (Utilities|Struct|BreakSTRUCT_inventory_item item))
  (bind _items (Variables|Default|Getitems))
  (for (_array_element _array_index) _items
    (if (Utilities|Enum|Equal(Enum) (.name (Utilities|Struct|BreakSTRUCT_inventory_item _array_element)) _name)
      (Utilities|Struct|SetmembersinSTRUCT_inventory_item (Utilities|Array|Get(acopy) _items _array_index) (+ (.Quantity (Utilities|Struct|BreakSTRUCT_inventory_item _array_element)) _quantity))
      (LocalVariables|Setitem%20found true)
      (Variables|Default|SetAdded true)))
  (if (not (LocalVariables|Getitem%20found))
    (Utilities|Array|Add _items item)))

(fn GetItemsbyUsage
  (params (usage :type ENUM_ItemSkills%20Enum :default "NewEnumerator0") (getNext :type Boolean) (NewParam :type STRUCT%20Inventory%20Item%20Structure))
  (bind _usage (Utilities|Struct|BreakSTRUCT_inventory_item NewParam))
  (bind _items_by_usage (LocalVariables|Getitems%20by%20usage))
  (bind _selected_index_map (Variables|Default|Getselected%20index%20map))
  (bind _returnvalue (Utilities|Array|Length _items_by_usage))
  (bind _returnvalue_2 (> _returnvalue 0))
  (LocalVariables|Setselected%20index (+ (.Value (Utilities|Map|Find (Variables|Default|Getselected%20index%20map) _usage)) (Math|Conversions|ToInteger(Boolean) getNext)))
  (for _array_element (Variables|Default|Getitems)
    (if (Utilities|Enum|Equal(Enum) (.usage (Utilities|Struct|BreakSTRUCT_inventory_item _array_element)) _usage)
      (Utilities|Array|Add (LocalVariables|Getitems%20by%20usage) _array_element)))
  (if (> (Utilities|Array|Length _items_by_usage) (LocalVariables|Getselected%20index))
    (Utilities|Map|Add _selected_index_map _usage (LocalVariables|Getselected%20index))
    (return (Utilities|Array|Get(acopy) _items_by_usage (LocalVariables|Getselected%20index)) true)
    (else
      (Utilities|Map|Add _selected_index_map _usage (Class|KismetSystemLibrary|MakeLiteralInteger))
      (if _returnvalue_2
        (return (Utilities|Array|Get(acopy) _items_by_usage) _returnvalue_2)))))

(fn RemoveItem
  (params (item%20data :type STRUCT%20Inventory%20Item%20Structure))
  (bind _items (Variables|Default|Getitems))
  (bind (_array_element _array_index) (Utilities|Array|ForEachLoopwithBreak _items :!label _label)
    (:LoopBody
      (if (Utilities|Enum|Equal(Enum) (.name (Utilities|Struct|BreakSTRUCT_inventory_item _array_element)) (.name (Utilities|Struct|BreakSTRUCT_inventory_item item%20data)))
        (if (< (- (.Quantity (Utilities|Struct|BreakSTRUCT_inventory_item _array_element)) 1) 1)
          (LocalVariables|Setremove%20index _array_index))
        (Utilities|Struct|SetmembersinSTRUCT_inventory_item (Utilities|Array|Get(acopy) _items _array_index) (- (.Quantity (Utilities|Struct|BreakSTRUCT_inventory_item _array_element)) 1))
        (goto _label Break)))
    (:Completed
      (if (> (LocalVariables|Getremove%20index) -1)
        (Utilities|Array|RemoveIndex (Variables|Default|Getitems) (LocalVariables|Getremove%20index))))))

(fn GetItemData
  (Class|BPICharacter|SetInteractableStatus(Message) (Game|GetPlayerCharacter 0) false))