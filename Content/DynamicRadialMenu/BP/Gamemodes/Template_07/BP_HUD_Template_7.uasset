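; HUD for radial menu Template 7 that manages the quick-access pie menu, inventory, timed tips and controls guide.
; The pie menu is created on BeginPlay, while tip and inventory widgets are created lazily and reused.
; Opening menus switches to game-and-UI input with a cursor; closing restores game-only input, after a delay for the pie menu.
; The guide queries the PlayerController for the active device's key bindings through message calls.
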(event Custom|Set%20Game%20Input%20Mode
  (bind _returnvalue (Game|GetPlayerController 0))
  ;[0 0 0] Game Input Mode
  (Input|SetInputModeGameOnly _returnvalue false)
  (Variables|/Script/Engine.PlayerController|SetbShowMouseCursor _returnvalue false))

(event Custom|Set%20UI%20InputMode
  (bind _returnvalue (Game|GetPlayerController 0))
  ;[0 0 0] UI input mode
  (Input|SetInputModeGameandUI _returnvalue 0 "DoNotLock" true false)
  (Variables|/Script/Engine.PlayerController|SetbShowMouseCursor _returnvalue true))

(event Custom|CreateQuickAccess
  ;[0 0 0] Create Quick Menu
  (bind _returnvalue (UserInterface|CreateWidget "/Game/DynamicRadialMenu/BP/Widgets/WDG_PieMenu_07.WDG_PieMenu_07_C"))
  (Variables|Default|SetWDG_QuickMenu _returnvalue))

(event EventCloseQuickAccess
  ;[0 0 0] Close Quick Menu
  (Utilities|FlowControl|Delay 2.0)
  (Default|CloseQuickAccess (Variables|Default|GetWDG_QuickMenu))
  (CallFunction|SetGameInputMode))

(event EventBeginPlay
  (CallFunction|CreateQuickAccess)
  (|GuideHUD_2))

(event EventShowTip
  (params (tip :type String) (timeout :type Float%20%28double-precision%29))
  ;[0 0 0] Show Tip
  (Utilities|IsValid (Variables|Default|GetWDG_Tip)
    (:Is%20Valid
      _)
    (:Is%20Not%20Valid
      (bind _returnvalue (UserInterface|CreateWidget "/Game/DynamicRadialMenu/BP/Widgets/BaseWidgets/WDG_Tips.WDG_Tips_C"))
      (Variables|Default|SetWDG_Tip _returnvalue)))
  (Default|ShowTip (Variables|Default|GetWDG_Tip) tip timeout)
  (if (UserInterface|Viewport|IsinViewport (Variables|Default|GetWDG_Tip))
    _
    (else
      (UserInterface|Viewport|AddtoViewport (Variables|Default|GetWDG_Tip) 0)))
  (Utilities|FlowControl|RetriggerableDelay timeout)
  (Widget|RemovefromParent (Variables|Default|GetWDG_Tip)))

(event EventQuickAccess
  (bind _wdg_quickmenu (Variables|Default|GetWDG_QuickMenu))
  ;[0 0 0] Toggle Quick Menu
  (Utilities|IsValid (Variables|Default|GetWDG_QuickMenu)
    (:Is%20Valid
      (UserInterface|Viewport|AddtoViewport _wdg_quickmenu 0)
      (Default|InitQuickAccess _wdg_quickmenu)
      (CallFunction|SetUIInputMode))))

(event EventToggleInventory
  (params (show/hide :type Boolean))
  ;[0 0 0] Toggle Inventory
  (if show/hide
    (Utilities|IsValid (Variables|Default|GetWDG_Inventory)
      (:Is%20Valid
        _)
      (:Is%20Not%20Valid
        (bind _returnvalue (UserInterface|CreateWidget "/Game/DynamicRadialMenu/BP/Widgets/WDG_Inventory_7.WDG_Inventory_7_C"))
        (Variables|Default|SetWDG_Inventory _returnvalue)))
    (if (UserInterface|Viewport|IsinViewport (Variables|Default|GetWDG_Inventory))
      _
      (else
        (UserInterface|Viewport|AddtoViewport (Variables|Default|GetWDG_Inventory) 0)))
    (CallFunction|SetUIInputMode)
    (Default|InitItems (Variables|Default|GetWDG_Inventory))
    (else
      (Utilities|IsValid (Variables|Default|GetWDG_Inventory)
        (:Is%20Valid
          (Widget|RemovefromParent (Variables|Default|GetWDG_Inventory))
          (CallFunction|SetGameInputMode))))))

(event EventShowGuide
  (params (QuickMenu%20 :type String) (Inventory%20%20 :type String) (Interact%20%20 :type String) (Collect%20Item :type String) (Use%20Item :type String))
  (Default|ShowGuide (Variables|Default|GetWDG_GuideHUD) QuickMenu%20 Inventory%20%20 Interact%20%20 Collect%20Item Use%20Item))

(fn ConstructionScript)