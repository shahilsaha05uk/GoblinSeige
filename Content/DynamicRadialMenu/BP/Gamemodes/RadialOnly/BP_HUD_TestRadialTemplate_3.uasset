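; HUD Blueprint for a radial menu test setup, managing the pie menu, timed tips and a control-guide overlay.
; Opening the menu locks look input and slows time to 0.1; closing restores both and writes any valid selection to the player's SelectedItem.
; BeginPlay adds the guide and sends it Quick Menu and Inventory key prompts obtained from the player controller.
; Tips reuse one widget, removed after a retriggerable delay.
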(event EventShowGuide
  (params (QuickMenu%20%20 :type String) (Inventory :type String))
  (Default|ShowGuide (Variables|Default|GetWDG_GuideHUD) QuickMenu%20%20 Inventory))

(event EventInitRadialMenu
  (bind _returnvalue (UserInterface|CreateWidget "/Game/DynamicRadialMenu/BP/Widgets/RadialOnly/WDG_TestPieMenu_03.WDG_TestPieMenu_03_C"))
  (bind _output_get (Variables|Default|SetWDG_QuickMenu _returnvalue))
  (UserInterface|Viewport|AddtoViewport _output_get 0)
  (Input|SetInputModeGameandUI (Game|GetPlayerController 0) (Variables|Default|GetWDG_QuickMenu) "LockAlways" true false)
  (Input|SetIgnoreLookInput (Game|GetPlayerController 0) true)
  (Utilities|Time|SetGlobalTimeDilation 0.1))

(event EventShowTip
  (params (tip%20 :type String) (timeout :type Float%20%28double-precision%29))
  ;[0 0 0] Show Tip
  (Utilities|IsValid (Variables|Default|GetWDG_Tip)
    (:Is%20Valid
      _)
    (:Is%20Not%20Valid
      (bind _returnvalue (UserInterface|CreateWidget "/Game/DynamicRadialMenu/BP/Widgets/BaseWidgets/WDG_Tips.WDG_Tips_C"))
      (Variables|Default|SetWDG_Tip _returnvalue)))
  (Default|ShowTip (Variables|Default|GetWDG_Tip) tip%20 timeout)
  (if (UserInterface|Viewport|IsinViewport (Variables|Default|GetWDG_Tip))
    _
    (else
      (UserInterface|Viewport|AddtoViewport (Variables|Default|GetWDG_Tip) 0)))
  (Utilities|FlowControl|RetriggerableDelay timeout)
  (Widget|RemovefromParent (Variables|Default|GetWDG_Tip)))

(event EventBeginPlay
  (|GuideHUD_2_2))

(event EventCloseRadialMenu
  (Utilities|IsValid (Variables|Default|GetWDG_QuickMenu)
    (:Is%20Valid
      (Widget|RemovefromParent (Variables|Default|GetWDG_QuickMenu))
      (Utilities|Time|SetGlobalTimeDilation 1.0)
      (Input|SetInputModeGameOnly (Game|GetPlayerController 0) false)
      (Input|SetIgnoreLookInput (Game|GetPlayerController 0) false)
      (if (.Valid (Default|GetSelectedOption (Variables|Default|GetWDG_QuickMenu)))
        (bind _returnvalue (Actor|GetActorOfClass "/Game/DynamicRadialMenu/BP/BP_CodeLikeMeTestPlayer.BP_CodeLikeMeTestPlayer_C"))
        (Variables|/Game/DynamicRadialMenu/BP/BP_CodeLikeMeTestPlayer.BP_CodeLikeMeTestPlayer_C|SetSelectedItem _returnvalue (.OutIndex (Default|GetSelectedOption (Variables|Default|GetWDG_QuickMenu)))))
      (Variables|Default|SetWDG_QuickMenu 0))))

(fn ConstructionScript)