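; Player controller for the dynamic radial menu that routes UI navigation and tracks the active input device.
; Backspace, Q and E send back, previous and next messages to the registered in-viewport widget, and an event toggles character input.
; Any key press switches between keyboard/mouse and gamepad, which filters action or axis mappings into tagged key labels, using an Xbox name map for gamepads.
; A helper exposes stick directions as vectors.
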(event EventSetActiveWidget
  (params (widget :type User%20Widget%20Object%20Reference))
  (Variables|Default|Setactive%20widget widget))

(event EventTogglePlayerCharacterInput
  (params (enable :type Boolean))
  (bind _returnvalue (Game|GetPlayerCharacter 0))
  (bind _returnvalue_2 (Game|GetPlayerController 0))
  (if enable
    (Input|EnableInput _returnvalue _returnvalue_2)
    (else
      (Input|DisableInput _returnvalue _returnvalue_2))))

(event Input|KeyboardEvents|Backspace
  (params (Key :type Key%20Structure))
  (:Pressed
    (bind _active_widget (Utilities|GetActiveWidget))
    (Class|BPIWidget|Back(Message) _active_widget)))

(event Input|KeyboardEvents|Q
  (params (Key :type Key%20Structure))
  (:Pressed
    (bind _active_widget (Utilities|GetActiveWidget))
    (Class|BPIWidget|Prev(Message) _active_widget)))

(event Input|KeyboardEvents|E
  (params (Key :type Key%20Structure))
  (:Pressed
    (bind _active_widget (Utilities|GetActiveWidget))
    (Class|BPIWidget|Next(Message) _active_widget)))

(event Input|KeyboardEvents|AnyKey
  (params (Key :type Key%20Structure))
  (:Pressed
    (if (or (Class|KismetInputLibrary|KeyIsKeyboardKey Key) (Class|KismetInputLibrary|KeyIsMouseButton Key))
      (Variables|Default|Setactive%20input%20device "NewEnumerator0")
      (elif (Class|KismetInputLibrary|KeyIsGamepadKey Key)
        (Variables|Default|Setactive%20input%20device "NewEnumerator1")))))

(fn ConstructionScript)

(fn IsActiveInputDevice
  (params (key :type Key%20Structure :default "None"))
  (if (or (Class|KismetInputLibrary|KeyIsKeyboardKey key) (Class|KismetInputLibrary|KeyIsMouseButton key))
    (LocalVariables|Setkey%20device "NewEnumerator0")
    (elif (Class|KismetInputLibrary|KeyIsGamepadKey key)
      (LocalVariables|Setkey%20device "NewEnumerator1")))
  (return (Utilities|Enum|Equal(Enum) (LocalVariables|Getkey%20device) (Variables|Default|Getactive%20input%20device))))

(fn GetKeyLabel
  (params (input%20key :type Key%20Structure :default "None") (key%20device :type ENUM_InputDevices%20Enum :default "NewEnumerator0"))
  (bind _returnvalue (Class|KismetInputLibrary|KeyGetDisplayName input%20key true))
  (bind _xbox_map (LocalVariables|Getxbox%20map))
  (bind _returnvalue_2 (Utilities|String|ToString(Text) _returnvalue))
  (bind (_value _returnvalue_3) (Utilities|Map|Find _xbox_map _returnvalue_2))
  (switch Utilities|FlowControl|Switch|SwitchonENUM_InputDevices key%20device
    (:NewEnumerator0
      _)
    (:NewEnumerator1
      (if _returnvalue_3
        (return _value)
        (else
          _))))
  (return _returnvalue_2))

(fn GetActiveInputDevice
  (return (Variables|Default|Getactive%20input%20device)))

(fn GetInputKeys
  (params (input%20name :type String))
  (bind _returnvalue (Class|InputSettings|GetInputSettings))
  (bind _returnvalue_2 (Utilities|String|StringToName input%20name))
  (bind _active_input_device (Variables|Default|Getactive%20input%20device))
  (bind _outmappings (Class|InputSettings|GetActionMappingbyName _returnvalue _returnvalue_2))
  (bind _outmappings_2 (Class|InputSettings|GetAxisMappingbyName _returnvalue _returnvalue_2))
  (if (> (Utilities|Array|Length _outmappings) 0)
    (for _array_element _outmappings
      (if (CallFunction|IsActiveInputDevice (.Key (Utilities|Struct|BreakInputActionKeyMapping _array_element)))
        (if (not (Utilities|Enum|Equal(Enum) (CallFunction|GetKeyLabel (.Key (Utilities|Struct|BreakInputActionKeyMapping _array_element)) (Variables|Default|Getactive%20input%20device)) (LocalVariables|Getinput%20keys%20)))
          (LocalVariables|Setinput%20keys%20 (Utilities|String|Append (CallFunction|GetKeyLabel (.Key (Utilities|Struct|BreakInputActionKeyMapping _array_element)) (Variables|Default|Getactive%20input%20device)) (LocalVariables|Getinput%20keys%20))))))
    (return (Utilities|String|Append (Utilities|Select :Index _active_input_device :NewEnumerator0 "<input>" :NewEnumerator1 "<gamepad>") (LocalVariables|Getinput%20keys%20) "</>") _active_input_device)
    (elif (> (Utilities|Array|Length _outmappings_2) 0)
      (for _array_element_2 _outmappings_2
        (if (CallFunction|IsActiveInputDevice (.Key (Utilities|Struct|BreakInputAxisKeyMapping _array_element_2)))
          (if (not (Utilities|Enum|Equal(Enum) (CallFunction|GetKeyLabel (.Key (Utilities|Struct|BreakInputAxisKeyMapping _array_element_2)) (Variables|Default|Getactive%20input%20device)) (LocalVariables|Getinput%20keys%20)))
            (LocalVariables|Setinput%20keys%20 (Utilities|String|Append (CallFunction|GetKeyLabel (.Key (Utilities|Struct|BreakInputAxisKeyMapping _array_element_2)) (Variables|Default|Getactive%20input%20device)) (LocalVariables|Getinput%20keys%20))))))
      (return (Utilities|String|Append (Utilities|Select :Index _active_input_device :NewEnumerator0 "<input>" :NewEnumerator1 "<gamepad>") (LocalVariables|Getinput%20keys%20) "</>") _active_input_device))))

(fn GetJoystickDirection
  (params (Stick :type ENUM_JoystickTypes%20Enum :default "NewEnumerator0"))
  (switch Utilities|FlowControl|Switch|SwitchonENUM_JoystickTypes Stick
    (:NewEnumerator0
      (return (Math|Vector2D|MakeVector2D (Class|Actor|GetInputAxisKeyValue) (* (Class|Actor|GetInputAxisKeyValue) -1.0))))
    (:NewEnumerator1
      (return (Math|Vector2D|MakeVector2D (Class|Actor|GetInputAxisKeyValue) (Class|Actor|GetInputAxisKeyValue))))))