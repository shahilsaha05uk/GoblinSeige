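; Turret projectile actor that plays impact feedback when it hits something, then retires itself.
; On hit it spawns a pooled effect aligned to the surface normal, feeding that normal into its Direction parameter, and plays a sound.
; An optional decal attaches to the hit component and fades out at the end of its lifespan.
; The mesh is then hidden and a short configurable lifespan delays the actor's destruction.
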(event Collision|EventHit
  (params (MyComp :type Primitive%20Component%20Object%20Reference) (Other :type Actor%20Object%20Reference) (OtherComp :type Primitive%20Component%20Object%20Reference) (bSelfMoved :type Boolean) (HitLocation :type Vector :default "0, 0, 0") (HitNormal :type Vector :default "0, 0, 0") (NormalImpulse :type Vector :default "0, 0, 0") (Hit :type Hit%20Result%20Structure%20%28by%20ref%29))
  (bind _returnvalue (Niagara|SpawnSystematLocation (Variables|Default|GetOnHitVFX) HitLocation (Math|Conversions|RotationFromXVector HitNormal) "1.000000,1.000000,1.000000" true true "AutoRelease"))
  (Niagara|SetNiagaraVariable(Vector3) _returnvalue "Direction" HitNormal)
  (Audio|PlaySoundatLocation (Variables|Default|GetOnHitSound) HitLocation "0, 0, 0" 1.0 1.0 0.0 0 0 0 0)
  (bind _onimpactdecal (Variables|Default|GetOnImpactDecal)
    (:then
      (bind _returnvalue_2 (Class|GameplayStatics|SpawnDecalAttached _onimpactdecal "64.000000,64.000000,64.000000" OtherComp "None" HitLocation (Math|Conversions|RotationFromXVector HitNormal) "KeepWorldPosition" (Variables|Default|GetOnImpactDecalLifespan)))
      (Rendering|Components|Decal|SetFadeOut _returnvalue_2 (- (Variables|Default|GetOnImpactDecalLifespan) (Variables|Default|GetOnImpactDelayFadeOutDuration)) (Variables|Default|GetOnImpactDelayFadeOutDuration) false))
    (:else
      _))
  (Development|SetHiddeninGame (Variables|Default|GetStaticMesh) true false)
  (Actor|SetLifeSpan (Variables|Default|GetOnImpactLifespan)))

(fn ConstructionScript)