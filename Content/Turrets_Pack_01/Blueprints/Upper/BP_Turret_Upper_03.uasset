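; BP_Turret_Upper_03 is the Blueprint for an upper turret part that handles firing and reloading.
; Its Fire event calls the parent Fire, then sets Firing only when one round of ammo is available and the target is reachable from the FirePoint tag within a fixed range.
; When ammo runs out and no reload is in progress, it starts a reload.
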(event EventFire
  (bind _result (CallFunction|HasAmmo 1))
  (|CallParentFunction)
  (Variables|Default|SetFiring (and _result (CallFunction|IsTargetReachable 1e+04 "FirePoint")))
  (if (and (not _result) (not (Variables|Default|GetReloading)))
    (CallFunction|Reload)))